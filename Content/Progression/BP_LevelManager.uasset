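; Level manager that runs the game's progression through levels and enemy waves loaded from DT_Levels.
; Each wave spawns AI ships that jump to random overlap-tested spots around the celestial target, with enemy marks and boss health UI, and advances once all are destroyed.
; Finished levels re-enable player jumps, optionally flagging an editor stop, and count arrivals before starting the next level.
; Completing all levels plays a victory overlay, saves first-time completion and returns to menu.
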(event `self.ReceiveBeginPlay`
  (bind _outrownames (`DataTableFunctionLibrary.GetDataTableRowNames` "/Game/Progression/DT_Levels.DT_Levels"))
  (for _array_element _outrownames
    (bind _returnvalue (`|GetDataTableRow` "/Game/Progression/DT_Levels.DT_Levels" _array_element)
      (:`then`
        (`KismetArrayLibrary.Array_Add` (`self.Levels`) _returnvalue))))
  (`KismetSystemLibrary.DelayUntilNextTick`)
  (bind _returnvalue_2 (`|CreateWidget` "/Game/Ships/Player/UI/WBP_LevelWaveData.WBP_LevelWaveData_C"))
  (bind _output_get (set `self.Level Progress UI` _returnvalue_2))
  (`UserWidget.AddToViewport` _output_get 0)
  (`self.Next Wave`))

(event `Next Wave`
  (bind (_level_waves _level_spawneditoratend _level_spawnactoronlevelstart) (break `/Game/Progression/BPS_Level` (`self.Get Current Level`)))
  (bind (_level_waves_2 _level_spawneditoratend_2) (break `/Game/Progression/BPS_Level` (`self.Get Current Level`)))
  (bind _current_wave_index (`self.Current Wave Index`))
  (bind _jumps_before_level_start (`self.Jumps Before Level Start`))
  (bind _result (`/Engine/EditorBlueprintResources/StandardMacros.IncrementInt` _current_wave_index)
    (:`  `
      (`/Game/Ships/Player/UI/WBP_LevelWaveData.Show Progress Info` (`self.Level Progress UI`) _current_wave_index (`self.Get Wave Count`) (`self.Current Level Index`))
      (if (== _result 0)
        (if (`KismetSystemLibrary.IsValidClass` _level_spawnactoronlevelstart)
          (`|SpawnActorFromClass` _level_spawnactoronlevelstart (`KismetMathLibrary.MakeTransform` (0.0 0.0 0.0)) "AlwaysSpawn" "MultiplyWithRoot" null null)))
      ;[1 1 1] Check if Level Completed
      (if (== _result (`self.Get Wave Count`))
        ;[1 1 1] Allow Jumping and Jump to Editor if Needed
        (`self.On Level End`)
        (add `/Game/CelestialSystem/Blueprints/BP_CelestialSystem.On Jump End` (`self.Celestial System`) (delegate `On Jump End`))
        (`/Game/CelestialSystem/Blueprints/BP_CelestialSystem.Set Can Jump` (`self.Celestial System`) true)
        (if _level_spawneditoratend_2
          (bind _output_get (set `self.Jumps Before Level Start` (+ _jumps_before_level_start 2)))
          (set `/Game/CelestialSystem/Blueprints/BP_CelestialSystem.Next Jump Is Editor` (== _output_get 2) (`self.Celestial System`))
          (else
            (set `self.Jumps Before Level Start` (+ _jumps_before_level_start 1))))
        (else
          (`self.Spawn Ships`))))))

(event `On Jump End`
  (bind _celestial_system (`self.Celestial System`))
  (bind _ship_editor (`/Game/CelestialSystem/Blueprints/BP_CelestialSystem.Ship Editor` _celestial_system))
  ;[1 1 1] Start Next Level When Arrived
  (bind _result (`/Engine/EditorBlueprintResources/StandardMacros.DecrementInt` (`self.Jumps Before Level Start`))
    (:`  `
      (if (== _result 0)
        (remove `/Game/CelestialSystem/Blueprints/BP_CelestialSystem.On Jump End` _celestial_system (delegate `On Jump End`))
        (`/Game/CelestialSystem/Blueprints/BP_CelestialSystem.Set Can Jump` (`self.Celestial System`) false)
        (`self.Next Level`)
        (`/Engine/EditorBlueprintResources/StandardMacros.IsValid` _ship_editor
          (:`Is Valid`
            (`self.K2_DestroyActor` _ship_editor)))))))

(event `Next Level`
  (set `self.Current Wave Index` -1)
  (bind _result (`/Engine/EditorBlueprintResources/StandardMacros.IncrementInt` (`self.Current Level Index`))
    (:`  `
      (if (== _result (`KismetArrayLibrary.Array_Length` (`self.Levels`)))
        (bind _returnvalue (`|CreateWidget` "/Game/Blueprints/WBP_VictoryOverlay.WBP_VictoryOverlay_C"))
        (`UserWidget.AddToViewport` _returnvalue 0)
        (bind _returnvalue_2 (`GameplayStatics.DoesSaveGameExist` "completion"))
        (if _returnvalue_2
          (bind _turnon (`/Game/Blueprints/WBP_VictoryOverlay.TurnOn` _returnvalue))
          (`UserWidget.PlayAnimation` _returnvalue _turnon 0.0 1 "Forward" 1.0 false)
          (`KismetSystemLibrary.Delay` (`WidgetAnimation.GetEndTime` _turnon))
          (else
            (bind _returnvalue_3 (`GameplayStatics.CreateSaveGameObject` "/Game/Progression/BP_SaveGame_Completion.BP_SaveGame_Completion_C"))
            (set `/Game/Progression/BP_SaveGame_Completion.Completed` true _returnvalue_3)
            (`GameplayStatics.SaveGameToSlot` _returnvalue_3 "completion")
            (bind _turnonfirst (`/Game/Blueprints/WBP_VictoryOverlay.TurnOnFirst` _returnvalue))
            (`UserWidget.PlayAnimation` _returnvalue _turnonfirst 0.0 1 "Forward" 1.0 false)
            (`KismetSystemLibrary.Delay` (`WidgetAnimation.GetEndTime` _turnonfirst))))
        (`GameplayStatics.OpenLevelBySoftObjectPtr` "/Game/L_Menu.L_Menu")
        (else
          (`self.Next Wave`))))))

(event `Spawn Ships`
  (bind _wave_shipnames (break `/Game/Progression/BPS_Wave` (`self.Get Current Wave`)))
  (bind (_wave_shipnames_2 _wave_isboss) (break `/Game/Progression/BPS_Wave` (`self.Get Current Wave`)))
  (set `self.Ships Left` (`KismetArrayLibrary.Array_Length` _wave_shipnames))
  (for (_array_element _array_index) _wave_shipnames
    (bind _returnvalue (`|GetDataTableRow` "/Game/Ships/DT_ShipData.DT_ShipData" _array_element)
      (:`then`
        (bind (_jump_location _spawn_location) (`self.Get Spawn and Jump Location` (`.BoxCollisionExtent_9_EDAE709B44B4082725E7D0B79EF0565B` (break `/Game/Ships/ShipEditor/Structures/BPS_ShipData_World` _returnvalue)) (`self.K2_GetActorLocation` (`ActorComponent.GetOwner` (`/Game/CelestialSystem/Blueprints/BP_CelestialSystem.Target Body` (`self.Celestial System`)))))) ; 1. посчитай откуда спавнить корабли\n2. посчитай куда корабли должны прыгать\n3. сократи время прыжка вражеских кораблей до минимума
        (bind _returnvalue_2 (`|SpawnActorFromClass` "/Game/Ships/AI/BP_Ship_AI.BP_Ship_AI_C" (`KismetMathLibrary.MakeTransform` _spawn_location) "AdjustIfPossibleButAlwaysSpawn" "MultiplyWithRoot" null 1.0 0.5 1.0 0.7 _array_element null))
        (set `/Game/Ships/BP_Ship.Look At Time` 0.1 _returnvalue_2)
        (set `/Game/Ships/BP_Ship.Stop Time` 0.1 _returnvalue_2)
        (bind (_returnvalue_x _returnvalue_y) (`KismetMathLibrary.BreakVector` (`self.K2_GetActorLocation` _returnvalue_2)))
        (`self.K2_SetActorLocation` (`KismetMathLibrary.MakeVector` _returnvalue_x _returnvalue_y (`self.Ship Plane Height`)) false true)
        (`/Game/Ships/BP_Ship.Jump` _returnvalue_2 _jump_location 0.5)
        (add `/Game/Ships/BP_Ship.On Ship Destroyed` _returnvalue_2 (delegate `On Ship Destroyed`))
        (bind _returnvalue_3 (`|CreateWidget` "/Game/Ships/Player/UI/WBP_EnemyMark.WBP_EnemyMark_C" null _returnvalue_2))
        (`UserWidget.AddToViewport` _returnvalue_3 0)
        (`BlueprintMapLibrary.Map_Add` (`self.Ship Marks Map`) _returnvalue_2 _returnvalue_3)
        (if (and _wave_isboss (== _array_index 0))
          (bind _returnvalue_4 (`|CreateWidget` "/Game/Blueprints/WBP_BossHealth.WBP_BossHealth_C" null _returnvalue_2))
          (`UserWidget.AddToViewport` _returnvalue_4 0))))))

(event `On Ship Destroyed`
  (params (Ship :type "/Game/Ships/BP_Ship Object Reference"))
  (bind _ship_marks_map (`self.Ship Marks Map`))
  (bind (_value _returnvalue) (`BlueprintMapLibrary.Map_Find` _ship_marks_map Ship))
  (`self.On Enemy Ship Destroyed` Ship)
  (if _returnvalue
    (`Widget.RemoveFromParent` _value)
    (`BlueprintMapLibrary.Map_Remove` _ship_marks_map Ship))
  (bind _result (`/Engine/EditorBlueprintResources/StandardMacros.DecrementInt` (`self.Ships Left`))
    (:`  `
      (if (== _result 0)
        (`self.Next Wave`)))))

(fn `Get Current Level`
  (returns (Level :type "/Game/Progression/BPS_Level Structure"))
  (return (`|GetArrayItem` (`self.Levels`) (`self.Current Level Index`))))

(fn `Get Current Wave`
  (returns (Wave :type "/Game/Progression/BPS_Wave Structure"))
  (return (`|GetArrayItem` (`.Waves_3_EA127D5E43A08BD93CDBBA94BEFFC3B3` (break `/Game/Progression/BPS_Level` (`self.Get Current Level`))) (`self.Current Wave Index`))))

(fn `Get Half Diagonal Length`
  (params (`Bounds Extent` :type "Vector Structure"))
  (returns (`Half Diagonal` :type "Float (double-precision)"))
  (bind _x (.x `Bounds Extent`))
  (bind _y (.y `Bounds Extent`))
  (bind _z (.z `Bounds Extent`))
  (return (* (`KismetMathLibrary.Sqrt` (+ (* _x _x) (* _y _y) (* _z _z))) 0.5)))

(fn `Get Random Location`
  (params (Offset :type "Vector Structure"))
  (returns (`Jump Location` :type "Vector Structure") (`Spawn Location` :type "Vector Structure"))
  (locals (`Random Direction` :type "Vector Structure") (NewLocalVar :type "Float (double-precision)"))
  (bind (_returnvalue_x _returnvalue_y) (`KismetMathLibrary.BreakVector` (`KismetMathLibrary.RandomUnitVector`)))
  (bind _output_get (set `local.Random Direction` (`KismetMathLibrary.Normal` (`KismetMathLibrary.MakeVector` _returnvalue_x _returnvalue_y))))
  (return (+ Offset (* _output_get (`KismetMathLibrary.RandomFloatInRange` (`self.Min Spawn Radius`) (`self.Max Spawn Radius`)))) (+ Offset (* _output_get (`self.Max Spawn Radius`) 2.0))))

(fn `Get Spawn and Jump Location`
  (params (`Box Extent` :type "Vector Structure") (`Spawn Offset` :type "Vector Structure"))
  (returns (`Jump Location` :type "Vector Structure") (`Spawn Location` :type "Vector Structure"))
  (locals (`Is Correct` :type Boolean))
  (bind _half_diagonal (`self.Get Half Diagonal Length` `Box Extent`)) ; For simplicity circumspheres will be compared instead
  (while (not (`local.Is Correct`))
    (bind (_jump_location _spawn_location) (`self.Get Random Location` `Spawn Offset`))
    (set `local.Is Correct` true)
    (bind (_outactors _returnvalue) (`KismetSystemLibrary.SphereOverlapActors` _jump_location _half_diagonal (`|MakeArray` "ObjectTypeQuery2" "ObjectTypeQuery3" "ObjectTypeQuery1" :!type "EObjectTypeQuery Enum") null (`self.Ignore to Ignore Overlapping`))) ; check to not intersect existing actors
    (if (not _returnvalue)
      (bind _keys (`BlueprintMapLibrary.Map_Keys` (`self.Jumping Ships`))) ; check to not intersect not yet spawned ships
      (for _array_element _keys
        (bind (_location _boundingboxextent) (break `/Game/Ships/Structures/BPS_SpawnJump` (`BlueprintMapLibrary.Map_Find` (`self.Jumping Ships`) _array_element)))
        (bind _half_diagonal_2 (`self.Get Half Diagonal Length` _boundingboxextent))
        (bind _returnvalue_2 (- _jump_location _location))
        (if (< (`KismetMathLibrary.Vector_Distance` _returnvalue_2 _returnvalue_2) (+ _half_diagonal _half_diagonal_2))
          (set `local.Is Correct` false)
          (break)))
      (else
        (set `local.Is Correct` false))))
  (return _jump_location _spawn_location))

(fn `Get Wave Count`
  (returns (`Wave Count` :type Integer))
  (return (`KismetArrayLibrary.Array_Length` (`.Waves_3_EA127D5E43A08BD93CDBBA94BEFFC3B3` (break `/Game/Progression/BPS_Level` (`|GetArrayItem` (`self.Levels`) (`self.Current Level Index`)))))))

(fn `UserConstructionScript`)