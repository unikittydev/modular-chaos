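; Item manager that rolls heal and ship module drops at the location of each enemy ship the LevelManager reports destroyed.
; Heal and module drops roll independently against their own spawn chances.
; For modules, it filters each loot table to rows valid for the current level in DT_ShipModuleData, caching non-empty results in LootMap.
; A probability-weighted roll over LootMap keys yields an index into LootTable, configuring the spawned BP_Item_Module.
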(event `self.ReceiveBeginPlay`
  (add `/Game/Progression/BP_LevelManager.On Enemy Ship Destroyed` (`self.Level Manager`) (delegate `On Ship Destroyed`)))

(event `On Ship Destroyed`
  (params (Ship :type "/Game/Ships/BP_Ship Object Reference"))
  (bind _returnvalue (`self.K2_GetActorLocation` Ship))
  (bind _level_manager (`self.Level Manager`))
  (if (> (`self.Heal Spawn Chance`) (`KismetMathLibrary.RandomFloat`))
    (`|SpawnActorFromClass` "/Game/Items/Heal/Blueprints/BP_Item_Heal.BP_Item_Heal_C" (`KismetMathLibrary.MakeTransform` _returnvalue) "Undefined" "MultiplyWithRoot" null null))
  (if (> (`self.Item Spawn Chance`) (`KismetMathLibrary.RandomFloat`))
    (for _array_element (`self.Loot Table`)
      (bind _module_names (`self.Get Available Loot` _array_element))
      (bind _returnvalue_2 (`KismetArrayLibrary.Array_Length` _module_names))
      (`KismetSystemLibrary.PrintString` (`KismetStringLibrary.Concat_StrStr` (`KismetSystemLibrary.GetDisplayName` (`.DataTable_11_4608EA364E8AB3BF3E28478AB78C1DA0` (break `/Game/Progression/BPS_ItemSpawner` _array_element))) " " (`KismetStringLibrary.Conv_IntToString` _returnvalue_2)) true true (struct :`R` 1.0 :`G` 0.151155 :`A` 1.0))
      (if (> _returnvalue_2 0)
        (`BlueprintMapLibrary.Map_Add` (`self.Loot Map`) _array_element (make `/Game/Progression/BPS_ModuleList` _module_names))))
    (bind _index (`self.Get Weight Index`))
    (bind _output (`|GetArrayItem` (`self.Loot Table`) _index))
    (bind (_probability _datatable _minpoints _maxpoints) (break `/Game/Progression/BPS_ItemSpawner` _output))
    (`|SpawnActorFromClass` "/Game/Items/Modules/BP_Item_Module.BP_Item_Module_C" (`KismetMathLibrary.MakeTransform` _returnvalue) "Undefined" "MultiplyWithRoot" null (`/Game/Progression/BP_LevelManager.Current Level Index` _level_manager) (`/Game/Progression/BP_LevelManager.Current Wave Index` _level_manager) _minpoints _maxpoints (break `/Game/Progression/BPS_ModuleList` (`BlueprintMapLibrary.Map_Find` (`self.Loot Map`) _output)) null)))

(fn `Get Available Loot`
  (params (`Loot Type` :type "/Game/Progression/BPS_ItemSpawner Structure"))
  (returns (`Module Names` :type "Array of Name"))
  (locals (Modules :type "Array of Name"))
  (bind _current_level_index (`/Game/Progression/BP_LevelManager.Current Level Index` (`self.Level Manager`)))
  (bind _outrownames (`DataTableFunctionLibrary.GetDataTableRowNames` (`.DataTable_11_4608EA364E8AB3BF3E28478AB78C1DA0` (break `/Game/Progression/BPS_ItemSpawner` `Loot Type`))))
  (bind _outrownames_2 (`DataTableFunctionLibrary.GetDataTableRowNames` "/Game/Ships/Modules/Base/DT_ShipModuleData.DT_ShipModuleData"))
  (for _array_element _outrownames_2
    (if (`KismetArrayLibrary.Array_Contains` _outrownames _array_element)
      (bind _returnvalue (`|GetDataTableRow` "/Game/Ships/Modules/Base/DT_ShipModuleData.DT_ShipModuleData" _array_element)
        (:`then`
          (bind (_classreference _size _defaulthp _powerpoints _basemesh _flippedmesh _level _minlevel _maxlevel) (break `/Game/Ships/Modules/Base/Structures/BPS_ShipModuleData` _returnvalue))
          (if (and (>= _current_level_index _minlevel) (<= _current_level_index _maxlevel))
            (`KismetArrayLibrary.Array_Add` (`local.Modules`) _array_element))))))
  (return (`local.Modules`)))

(fn `Get Weight Index`
  (returns (Index :type Integer))
  (locals (Sum :type "Float (double-precision)") (Points :type "Float (double-precision)"))
  (bind _keys (`BlueprintMapLibrary.Map_Keys` (`self.Loot Map`)))
  (for _array_element _keys
    (set `local.Sum` (+ (`.Probability_5_10F8286741DAA6DB81564095CB38467C` (break `/Game/Progression/BPS_ItemSpawner` _array_element)) (`local.Sum`))))
  (set `local.Points` (`KismetMathLibrary.RandomFloatInRange` 0.0 (`local.Sum`)))
  (set `local.Sum` 0.0)
  (for (_array_element_2 _array_index) _keys
    (bind _output_get (set `local.Sum` (+ (`.Probability_5_10F8286741DAA6DB81564095CB38467C` (break `/Game/Progression/BPS_ItemSpawner` _array_element_2)) (`local.Sum`))))
    (if (> _output_get (`local.Points`))
      (return _array_index))))

(fn `UserConstructionScript`)