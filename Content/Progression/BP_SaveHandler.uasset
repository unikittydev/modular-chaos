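; BP_SaveHandler persists player progress to a single save slot.
; On BeginPlay it creates a save with starter ship and items for a new game, otherwise loads or creates one, then applies it.
; Loading restores inventory (or a cheat inventory), level and wave indices, player transform, and respawns any saved ship-editor activator.
; It saves this state whenever BP_LevelManager signals level end, storing the wave index minus one.
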(event `self.ReceiveBeginPlay`
  (bind _returnvalue (`GameplayStatics.GetActorOfClass` "/Game/Ships/Player/BP_Ship_Player.BP_Ship_Player_C"))
  (bind _output_get (set `self.Ship` _returnvalue))
  (set `self.Inventory` (`/Game/Ships/Player/BP_Ship_Player.Inventory` _output_get))
  (bind _returnvalue_2 (`GameplayStatics.GetActorOfClass` "/Game/Progression/BP_LevelManager.BP_LevelManager_C"))
  (bind _output_get_2 (set `self.Level Manager` _returnvalue_2))
  (add `/Game/Progression/BP_LevelManager.On Level End` _output_get_2 (delegate `On Next Level`))
  (bind _asbp_game_instance (cast `/Game/Menu/BP_GameInstance` (`GameplayStatics.GetGameInstance`)))
  (if (`/Game/Menu/BP_GameInstance.New Game` _asbp_game_instance)
    (`self.Create Save`)
    (else
      (`self.Load or Create Save`)))
  (`self.Load Game`))

(event `On Next Level`
  (`self.Save Game`))

(fn `Create Save`
  (bind _returnvalue (`GameplayStatics.CreateSaveGameObject` "/Game/Progression/BP_SaveGame_Player.BP_SaveGame_Player_C"))
  (bind _output_get (set `self.Save` _returnvalue))
  (bind _returnvalue_2 (`|GetDataTableRow` "/Game/Ships/DT_ShipData.DT_ShipData" "Ship.0")
    (:`then`
      (set `/Game/Progression/BP_SaveGame_Player.Ship` _returnvalue_2 _output_get)
      (set `/Game/Progression/BP_SaveGame_Player.Items` (`|MakeArray` "weapon_1x1_1_L1" "weapon_1x1_1_L1" "hull_1x1_0_L1" :!type "Name") _output_get))))

(fn `Load Game`
  (bind _inventory (`self.Inventory`))
  (bind _save (`self.Save`))
  (bind _save_2 (`self.Save`))
  (bind _level_manager (`self.Level Manager`))
  (bind _level_manager_2 (`self.Level Manager`))
  (bind _asbp_game_instance (cast `/Game/Menu/BP_GameInstance` (`GameplayStatics.GetGameInstance`)))
  (if (`/Game/Menu/BP_GameInstance.Cheat Inventory` _asbp_game_instance)
    (`/Game/Ships/Player/BPC_Inventory.Set Cheat Inventory` _inventory true)
    (else
      (`/Game/Ships/Player/BPC_Inventory.Set Items` _inventory (`/Game/Progression/BP_SaveGame_Player.Items` _save))))
  (set `/Game/Progression/BP_LevelManager.Current Level Index` (`/Game/Progression/BP_SaveGame_Player.Level Index` _save) _level_manager_2)
  (set `/Game/Progression/BP_LevelManager.Current Wave Index` (`/Game/Progression/BP_SaveGame_Player.Wave Index` _save) _level_manager_2)
  (`SceneComponent.K2_SetWorldTransform` (`/Game/Ships/BP_Ship.BoxCollision` (`self.Ship`)) (`/Game/Progression/BP_SaveGame_Player.Player Transform` (`self.Save`)) false true)
  (if (`/Game/Progression/BP_SaveGame_Player.Spawn Editor Activator` _save_2)
    (bind _returnvalue (`|SpawnActorFromClass` "/Game/Ships/ShipEditor/Grid/BP_ShipEditorActivator.BP_ShipEditorActivator_C" (`/Game/Progression/BP_SaveGame_Player.Editor Activator Transform` _save_2) "AlwaysSpawn" "MultiplyWithRoot" null false null))
    (set `/Game/Progression/BP_LevelManager.Jumps Before Level Start` -1 _level_manager)
    (set `/Game/CelestialSystem/Blueprints/BP_CelestialSystem.Ship Editor` _returnvalue (`/Game/Progression/BP_LevelManager.Celestial System` _level_manager))))

(fn `Load or Create Save`
  (bind _returnvalue (`GameplayStatics.LoadGameFromSlot` "player"))
  (bind _asbp_save_game_player (cast `/Game/Progression/BP_SaveGame_Player` _returnvalue)
    (:`then`
      (set `self.Save` _asbp_save_game_player))
    (:`CastFailed`
      (`self.Create Save`)))
  (return))

(fn `Save Game`
  (bind _level_manager (`self.Level Manager`))
  (bind _save (`self.Save`))
  (bind _save_2 (`self.Save`))
  (bind _items (`/Game/Ships/Player/BPC_Inventory.Get All Items` (`self.Inventory`)))
  (set `/Game/Progression/BP_SaveGame_Player.Items` _items (`self.Save`))
  (set `/Game/Progression/BP_SaveGame_Player.Level Index` (- (`/Game/Progression/BP_LevelManager.Current Level Index` _level_manager) 0) _save)
  (set `/Game/Progression/BP_SaveGame_Player.Wave Index` (- (`/Game/Progression/BP_LevelManager.Current Wave Index` _level_manager) 1) _save)
  (`/Engine/EditorBlueprintResources/StandardMacros.IsValid` (`self.Ship Editor Activator`)
    (:`Is Valid`
      (set `/Game/Progression/BP_SaveGame_Player.Spawn Editor Activator` true _save_2)
      (set `/Game/Progression/BP_SaveGame_Player.Editor Activator Transform` (`self.GetTransform` (`self.Ship Editor Activator`)) _save_2))
    (:`Is Not Valid`
      _))
  (set `/Game/Progression/BP_SaveGame_Player.Player Transform` (`self.GetTransform` (`self.Ship`)) (`self.Save`))
  (`GameplayStatics.SaveGameToSlot` (`self.Save`) "player"))

(fn `UserConstructionScript`)