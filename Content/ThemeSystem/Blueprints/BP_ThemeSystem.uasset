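; BP_ThemeSystem plays background music themes in rotation, each with a default and a chiptuned version.
; It starts at a random ThemeList entry, loads both sounds from DT_Themes, shows a WBP_NowPlaying widget, then advances after the chiptuned track's length plus a random wait.
; SwitchTheme crossfades between versions, using playback-percent callbacks to start the incoming one at the outgoing one's position.
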(event `self.ReceiveBeginPlay`
  (add `AudioComponent.OnAudioPlaybackPercent` (`self.Default Theme`) (delegate `Default Playback`))
  (add `AudioComponent.OnAudioPlaybackPercent` (`self.Chiptuned Theme`) (delegate `Chiptuned Playback`))
  (set `self.Current Theme Index` (`KismetMathLibrary.RandomIntegerInRange` 0 (`KismetArrayLibrary.Array_LastIndex` (`self.Theme List`))))
  (`self.Next Theme`))

(event `Default Playback`
  (params (PlayingSoundWave :type "SoundWave Object Reference") (PlaybackPercent :type "Float (single-precision)"))
  (set `self.Default Time` (* (`SoundBase.Duration` PlayingSoundWave) PlaybackPercent)))

(event `Chiptuned Playback`
  (params (PlayingSoundWave :type "SoundWave Object Reference") (PlaybackPercent :type "Float (single-precision)"))
  (set `self.Chiptune Time` (* (`SoundBase.Duration` PlayingSoundWave) PlaybackPercent)))

(event `Next Theme`
  (bind _theme (`self.Play Theme By Index` (`self.Current Theme Index`)))
  (bind _returnvalue (`|CreateWidget` "/Game/Menu/WBP_NowPlaying.WBP_NowPlaying_C" null (`.Name_7_D38C2285459B3590D4E55BA1C3270A28` (break `/Game/ThemeSystem/Blueprints/BPS_Theme` _theme))))
  (`UserWidget.AddToViewport` _returnvalue 0)
  (`KismetSystemLibrary.Delay` (+ (`SoundBase.Duration` (`AudioComponent.Sound` (`self.Chiptuned Theme`))) (`KismetMathLibrary.RandomFloatInRange` (`self.Wait Delay Min`) (`self.Wait Delay Max`))))
  (set `self.Current Theme Index` (mod (+ (`self.Current Theme Index`) 1) (`KismetArrayLibrary.Array_Length` (`self.Theme List`))))
  (`self.Next Theme`))

(event `Switch Theme`
  (params (Chiptuned :type Boolean))
  (bind _fade_time (`self.Fade Time`))
  (bind _fade_time_2 (`self.Fade Time`))
  (bind _output_get (set `self.Chiptuned` Chiptuned))
  (if _output_get
    (`AudioComponent.FadeIn` (`self.Chiptuned Theme`) _fade_time 1.0 (`self.Default Time`) "Linear")
    (`AudioComponent.FadeOut` (`self.Default Theme`) _fade_time 0.0 "Linear")
    (else
      (`AudioComponent.FadeIn` (`self.Default Theme`) _fade_time_2 1.0 (`self.Chiptune Time`) "Linear")
      (`AudioComponent.FadeOut` (`self.Chiptuned Theme`) _fade_time_2 0.0 "Linear"))))

(fn `Play Theme By Index`
  (params (Index :type Integer))
  (returns (Theme :type "/Game/ThemeSystem/Blueprints/BPS_Theme Structure"))
  (bind _returnvalue (`|GetDataTableRow` "/Game/ThemeSystem/DT_Themes.DT_Themes" (`|GetArrayItem` (`self.Theme List`) Index))
    (:`then`
      (bind (_default _chiptuned) (break `/Game/ThemeSystem/Blueprints/BPS_Theme` _returnvalue))
      (`AudioComponent.SetSound` (`self.Default Theme`) _default)
      (`AudioComponent.SetSound` (`self.Chiptuned Theme`) _chiptuned)
      (`AudioComponent.FadeIn` (select `bool` (`self.Chiptuned`) :`false` (`self.Default Theme`) :`true` (`self.Chiptuned Theme`)) (`self.Fade Time`) 1.0 0.0 "Linear")
      (return _returnvalue))))

(fn `UserConstructionScript`)