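; Pickup item that grants a random batch of modules to the collecting player's inventory.
; The batch size is a random roll, at least one, whose upper bound grows with Wave and Level.
; Items are drawn at random from ModuleNames and debug-printed via a second, separate random pick.
; GetAvailableModules filters a data table by level range against DT_ShipModuleData, but nothing in this file calls it.
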(event `self.On Item Collected`
  (params (Player :type "/Game/Ships/Player/BP_Ship_Player Object Reference"))
  (bind _modules (`self.Get Random Modules`))
  (for _array_element _modules
    (`/Game/Ships/Player/BPC_Inventory.Add Item` (`/Game/Ships/Player/BP_Ship_Player.Inventory` Player) _array_element)))

(fn `Calculate Points`
  (returns (Points :type Integer))
  (return (`KismetMathLibrary.Max` (`KismetMathLibrary.RandomIntegerInRange` (`self.Min Count`) (+ (+ (/ (`self.Wave`) 2) (/ (`self.Level`) 3)) (`self.Max Count`))) 1)))

(fn `Get Available Modules`
  (returns (`Module Names` :type "Array of Name"))
  (locals (Modules :type "Array of Name"))
  (`KismetArrayLibrary.Array_Clear` (`local.Modules`))
  (bind _returnvalue (`KismetSystemLibrary.LoadAsset_Blocking` (`self.Target Data Table`)))
  (bind _asdata_table (cast `DataTable` _returnvalue))
  (bind _returnvalue_2 (`DataTableFunctionLibrary.GetDataTableColumnAsString` "/Game/Ships/Modules/Base/DT_ShipModuleData.DT_ShipModuleData" "MinLevel"))
  (bind _returnvalue_3 (`DataTableFunctionLibrary.GetDataTableColumnAsString` "/Game/Ships/Modules/Base/DT_ShipModuleData.DT_ShipModuleData" "MaxLevel"))
  (bind _outrownames (`DataTableFunctionLibrary.GetDataTableRowNames` "/Game/Ships/Modules/Base/DT_ShipModuleData.DT_ShipModuleData"))
  (bind _outrownames_2 (`DataTableFunctionLibrary.GetDataTableRowNames` _asdata_table))
  (for _array_element _outrownames_2
    (bind _returnvalue_4 (`KismetArrayLibrary.Array_Find` _outrownames _array_element))
    (if (and (>= (`self.Level`) (`KismetStringLibrary.Conv_StringToInt` (`|GetArrayItem` _returnvalue_2 _returnvalue_4))) (<= (`self.Level`) (`KismetStringLibrary.Conv_StringToInt` (`|GetArrayItem` _returnvalue_3 _returnvalue_4))))
      (`KismetArrayLibrary.Array_Add` (`local.Modules`) _array_element)))
  (return (`local.Modules`)))

(fn `Get Random Modules`
  (returns (Modules :type "Array of Name"))
  (locals (Items :type "Array of Name"))
  (bind _outitem (`KismetArrayLibrary.Array_Random` (`self.Module Names`)))
  (bind _points (`self.Calculate Points`))
  (for _ (range 1 (+ _points 1))
    (`KismetArrayLibrary.Array_Add` (`local.Items`) _outitem)
    (`KismetSystemLibrary.PrintString` (`KismetStringLibrary.Conv_NameToString` _outitem) true true (struct :`R` 0.312544 :`G` 1.0 :`A` 1.0)))
  (return (`local.Items`)))

(fn `UserConstructionScript`
  (`parent.UserConstructionScript`))