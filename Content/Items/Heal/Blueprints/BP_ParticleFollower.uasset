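; BP_ParticleFollower is a heal item effect actor that keeps a Niagara particle system at the location of a Target actor.
; Tick moves the actor to the Target's location every frame, without sweep or attachment.
; The Deactivate event stops the Niagara system and plays a timeline whose inverted track drives its OpacityFactor parameter.
; In parallel, a DestroyTimer delay destroys the actor.
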(event `Deactivate`
  (`ActorComponent.Deactivate` (`self.NS`))
  (`|ExecutionSequence`
    (:`then_0`
      (bind (_direction _track) (`Timeline|Timeline`)
        (:`Update`
          (`NiagaraComponent.SetVariableFloat` (`self.NS`) "OpacityFactor" (- 1.0 _track)))))
    (:`then_1`
      (`KismetSystemLibrary.Delay` (`self.Destroy Timer`))
      (`self.K2_DestroyActor`))))

(event `self.ReceiveTick`
  (params (DeltaSeconds :type "Float (single-precision)"))
  (`self.K2_SetActorLocation` (`self.K2_GetActorLocation` (`self.Target`))))

(fn `UserConstructionScript`)