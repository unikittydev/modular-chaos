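; Timed heal zone that heals overlapping actors with a BPC_DamageableManager component, then destroys itself.
; A timeline grows the sphere from zero to full scale, then a second drives material opacity through a curve until expiry.
; Overlaps maintain the target list and a particle follower per target.
; Tick sends each target whole-number healing scaled by delta time, keeping the fractional remainder in Error.
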(event `self.ReceiveBeginPlay`
  (bind _heal_sphere (`self.Heal Sphere`))
  (bind _returnvalue (`KismetMaterialLibrary.CreateDynamicMaterialInstance` (`PrimitiveComponent.GetMaterial` _heal_sphere 0)))
  (`PrimitiveComponent.SetMaterial` _heal_sphere 0 _returnvalue)
  (set `self.MID` _returnvalue)
  (set `self.Target Scale` (`SceneComponent.K2_GetComponentScale` (`self.Heal Sphere`)))
  (`TimelineComponent.SetPlayRate` (`self.Fade In Timeline`) (/ 1.0 (`self.Fade In Duration`)))
  (bind (_direction _track) (`Timeline|Fade In Timeline` :!via `PlayFromStart`)
    (:`Update`
      (`SceneComponent.SetWorldScale3D` (`self.Heal Sphere`) (`KismetMathLibrary.VLerp` (0.0 0.0 0.0) (`self.Target Scale`) _track)))
    (:`Finished`
      (`TimelineComponent.SetPlayRate` (`self.Heal Timeline`) (/ 1.0 (`self.Heal Duration`)))
      (bind (_direction_2 _track_2) (`Timeline|Heal Timeline` :!via `PlayFromStart`)
        (:`Update`
          (`MaterialInstanceDynamic.SetScalarParameterValue` (`self.MID`) "OpacityFactor" (`CurveFloat.GetFloatValue` (`self.Opacity Curve`) _track_2)))
        (:`Finished`
          (`self.K2_DestroyActor`))))))

(event `self.ReceiveActorBeginOverlap`
  (params (OtherActor :type "Actor Object Reference"))
  (bind _returnvalue (`self.GetComponentByClass` OtherActor "/Game/DamageSystem/Blueprints/BPC_DamageableManager.BPC_DamageableManager_C"))
  (`/Engine/EditorBlueprintResources/StandardMacros.IsValid` _returnvalue
    (:`Is Valid`
      (`KismetArrayLibrary.Array_Add` (`self.Targets`) _returnvalue)
      (bind _returnvalue_2 (`|SpawnActorFromClass` "/Game/Items/Heal/Blueprints/BP_ParticleFollower.BP_ParticleFollower_C" (`self.GetTransform` OtherActor) "Undefined" "MultiplyWithRoot" null (`ActorComponent.GetOwner` _returnvalue) null))
      (`KismetArrayLibrary.Array_Add` (`self.Heal Particles`) _returnvalue_2))))

(event `self.ReceiveActorEndOverlap`
  (params (OtherActor :type "Actor Object Reference"))
  (bind _returnvalue (`self.GetComponentByClass` OtherActor "/Game/DamageSystem/Blueprints/BPC_DamageableManager.BPC_DamageableManager_C"))
  (bind _output (`|GetArrayItem` (`self.Heal Particles`) (`KismetArrayLibrary.Array_Find` (`self.Targets`) _returnvalue)))
  (`/Engine/EditorBlueprintResources/StandardMacros.IsValid` _returnvalue
    (:`Is Valid`
      (`/Game/Items/Heal/Blueprints/BP_ParticleFollower.Deactivate` _output)
      (`KismetArrayLibrary.Array_RemoveItem` (`self.Heal Particles`) _output)
      (`KismetArrayLibrary.Array_RemoveItem` (`self.Targets`) _returnvalue))))

(event `self.ReceiveTick`
  (params (DeltaSeconds :type "Float (single-precision)"))
  (bind _returnvalue (+ (* DeltaSeconds (`self.Heal`)) (`self.Error`)))
  (bind _returnvalue_2 (`KismetMathLibrary.FTrunc` _returnvalue))
  (set `self.Error` (- _returnvalue _returnvalue_2))
  (for _array_element (`self.Targets`)
    (`/Game/DamageSystem/Blueprints/BPC_DamageableManager.On Take Heal` _array_element _returnvalue_2)))

(fn `UserConstructionScript`)