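; Screen utility function library that finds where a player's mouse cursor lands on a horizontal game plane at a given height.
; The mouse viewport position is multiplied by viewport scale, deprojected to a world ray and passed to ProjectMouseOnPlane, with a zero vector returned if deprojection fails.
; The Project Mouse on Plane graph holds dot-product ray-plane intersection math, shown as unconnected to any output.
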(fn `Project Mouse Location on Game Plane`
  (params (Player :type "PlayerController Object Reference") (`Plane Height` :type "Float (double-precision)"))
  (returns (Location :type "Vector Structure"))
  (bind _returnvalue (`WidgetLayoutLibrary.GetMousePositionOnViewport` Player))
  (bind (_worldposition _worlddirection _returnvalue_2) (`GameplayStatics.DeprojectScreenToWorld` Player (* _returnvalue (`WidgetLayoutLibrary.GetViewportScale` Player))))
  (bind _returnvalue_3 (- (`KismetMathLibrary.MakeVector` (.x _worldposition) (.y _worldposition) `Plane Height`) _worldposition))
  (return (`KismetMathLibrary.SelectVector` (+ _worldposition (* (/ (`KismetMathLibrary.VSize` _returnvalue_3) (`KismetMathLibrary.Dot_VectorVector` (`KismetMathLibrary.Normal` _returnvalue_3) _worlddirection)) _worlddirection)) (0.0 0.0 0.0) (and _returnvalue_2 true))))