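; Spawner actor that creates an AI ship (BP_Ship_AI) at its own transform, chosen to match a target power value.
; SpawnSingleShip reads the Power column of DT_ShipPower, and GetClosestIndex linearly scans it for the value nearest TargetPower.
; The matching row name is passed to the spawned ship as ShipName.
; SpawnShipWave is an empty stub.
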(fn `Spawn Ship Wave`)

(fn `Spawn Single Ship`
  (params (`Target Power` :type Integer))
  (locals (`Closest Index` :type Integer) (`Closest Power` :type Integer :default -2147483648))
  (bind _target_power (`local.Target Power`))
  (bind _returnvalue (`DataTableFunctionLibrary.GetDataTableColumnAsString` "/Game/Ships/DT_ShipPower.DT_ShipPower" "Power"))
  (for (_array_element _array_index) _returnvalue
    (bind _returnvalue_2 (`KismetStringLibrary.Conv_StringToInt` _array_element))
    (if (< (`KismetMathLibrary.Abs_Int` (- _returnvalue_2 _target_power)) (`KismetMathLibrary.Abs_Int` (- _target_power (`local.Closest Power`))))
      (set `local.Closest Power` _returnvalue_2)
      (set `local.Closest Index` _array_index)))
  (bind _outrownames (`DataTableFunctionLibrary.GetDataTableRowNames` "/Game/Ships/DT_ShipPower.DT_ShipPower"))
  (`|SpawnActorFromClass` "/Game/Ships/AI/BP_Ship_AI.BP_Ship_AI_C" (`self.GetTransform`) "Undefined" "MultiplyWithRoot" null 1.0 0.5 1.0 0.7 (`|GetArrayItem` _outrownames (`local.Closest Index`)) null))

(fn `UserConstructionScript`)