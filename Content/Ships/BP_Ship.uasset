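; BP_Ship is a modular spaceship actor assembled at BeginPlay from data tables, with modules spawned as child actor components under Model.
; Hull HP is the sum of module HP, and a damageable manager layers a regenerating shield over the hull.
; Zero hull HP disables and resets the ship, shockwaves nearby ships and optionally destroys it.
; Jump uses timelines to damp physics, turn toward the target and lerp there with Niagara and sound effects.
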(event Custom|On%20HP%20Zero
  (CallFunction|SetShipEnabled false)
  (CallFunction|SetShipReset true)
  (bind _outactors (Collision|SphereOverlapActors (Transformation|GetWorldLocation (Variables|Components|GetBoxCollision)) (Variables|Default|GetShock%20Wave%20Radius) (Utilities|Array|MakeArray "ObjectTypeQuery3" "ObjectTypeQuery2") 0))
  (for _array_element _outactors
    (bind _asbp_ship (Utilities|Casting|CastToBP_Ship _array_element))
    (Default|CallOnGetShipinShockWave _asbp_ship))
  (Default|CallOnShipDestroyed self)
  (if (Variables|Default|GetDestroy%20Actor)
    (Utilities|FlowControl|Delay (Variables|Default|GetCleanup%20Time))
    (Actor|DestroyActor)))

(event Custom|Ship%20Modules%20Changed
  (params (Module :type BP%20Ship%20Module%20Object%20Reference))
  (CallFunction|UpdateShipHP))

(event Custom|Look%20At%20Smooth
  (params (Direction :type Vector) (Time :type Float%20%28double-precision%29))
  (bind _boxcollision (Variables|Components|GetBoxCollision))
  (bind _returnvalue (Transformation|GetWorldLocation _boxcollision))
  (Components|Timeline|SetPlayRate (Variables|Default|GetLook%20At%20Timeline) (/ 1.0 Time))
  (Variables|Default|SetOld%20Rotation (Transformation|GetWorldRotation (Variables|Components|GetBoxCollision)))
  (bind _track (Timeline|Look%20At%20Timeline PlayFromStart)
    (:Update
      (Transformation|SetWorldRotation (Variables|Components|GetBoxCollision) (Math|Rotator|Lerp(Rotator) (Variables|Default|GetOld%20Rotation) (Math|Rotator|FindLookatRotation _returnvalue (+ _returnvalue Direction)) _track true) false false))))

(event Custom|Jump
  (params (Target%20Location :type Vector) (Jump%20Time :type Float%20%28double-precision%29))
  (bind _look_at_time (Variables|Jump|GetLook%20At%20Time))
  (bind _boxcollision (Variables|Components|GetBoxCollision))
  (bind _boxcollision_2 (Variables|Components|GetBoxCollision))
  (bind _returnvalue (Transformation|GetWorldLocation _boxcollision))
  ;[1 1 1] Stop Ship
  (Default|CallOnShipMove 1.0 0.0 0.0) ; To make engines emit fire while jumping
  (Utilities|FlowControl|DelayUntilNextTick)
  (bind _returnvalue_2 (Physics|GetPhysicsLinearVelocity _boxcollision_2 "None"))
  (Variables|Jump|SetAngular%20Velocity (Class|PrimitiveComponent|GetPhysicsAngularVelocityinRadians _boxcollision_2 "None"))
  (CallFunction|SetShipEnabled false)
  (Collision|SetCollisionEnabled (Variables|Components|GetBoxCollision) "PhysicsOnly")
  (Physics|SetSimulatePhysics (Variables|Components|GetBoxCollision) true)
  (Components|Timeline|SetPlayRate (Variables|Default|GetStop%20Physics%20Timeline) (/ 1.0 (Variables|Jump|GetStop%20Time)))
  (Audio|PlaySoundatLocation "/Game/Audio/Jump/SW_Jump_Rotate.SW_Jump_Rotate" (Transformation|GetWorldLocation (Variables|Components|GetBoxCollision)) "0, 0, 0" 1.0 1.0 0.0 0 0 0 0)
  (bind _track (Timeline|Stop%20Physics%20Timeline PlayFromStart)
    (:Update
      (|DampShip _track _returnvalue_2))
    (:Finished
      (Physics|SetSimulatePhysics (Variables|Components|GetBoxCollision) false)
      (Collision|SetCollisionEnabled (Variables|Components|GetBoxCollision) "NoCollision")
      ;[1 1 1] Rotate Ship
      (CallFunction|LookatSmooth (Math|Vector|Normalize (- Target%20Location (Transformation|GetWorldLocation (Variables|Components|GetBoxCollision)))) _look_at_time)
      (Utilities|FlowControl|Delay _look_at_time)
      ;[1 1 1] Move Ship
      (Class|NiagaraComponent|SetVariableBool (Variables|Default|GetNS_Jump) "Spawn" true)
      (Audio|PlaySoundatLocation "/Game/Audio/Jump/SW_Jump_Perform.SW_Jump_Perform" _returnvalue "0, 0, 0" 1.0 1.0 0.0 0 0 0 0)
      (CallFunction|LerpLocation _returnvalue Target%20Location Jump%20Time)
      (Utilities|FlowControl|Delay Jump%20Time)
      (Class|NiagaraComponent|SetVariableBool (Variables|Default|GetNS_Jump) "Spawn" false)
      ;[1 1 1] Complete Jump
      (Audio|PlaySoundatLocation "/Game/Audio/Jump/SW_Jump_End.SW_Jump_End" _returnvalue "0, 0, 0" 1.0 1.0 0.0 0 0 0 0)
      (CallFunction|SetShipEnabled true))))

(event Custom|Lerp%20Location
  (params (From%20Location :type Vector) (To%20Location :type Vector) (Time :type Float%20%28double-precision%29))
  (Components|Timeline|SetPlayRate (Variables|Default|GetLerp%20Location%20Timeline) (/ 1.0 Time))
  (bind _returnvalue (Audio|SpawnSoundAttached "/Game/Audio/Jump/SW_Jump_Ambient.SW_Jump_Ambient" (Variables|Components|GetBoxCollision) "None" "0, 0, 0" "0, 0, 0" "KeepRelativeOffset" false 1.0 1.0 0.0 0 0 false))
  (bind (_direction _track _ambient_volume) (Timeline|Lerp%20Location%20Timeline PlayFromStart)
    (:Update
      (Transformation|SetWorldLocation (Variables|Components|GetBoxCollision) (Math|Vector|Lerp(Vector) From%20Location To%20Location _track) false false)
      (Default|CallOnShipMove 1.0 0.0 0.0)
      (Audio|Components|Audio|SetVolumeMultiplier _returnvalue _ambient_volume :!class /Script/Engine.AudioComponent))
    (:Finished
      (Components|DestroyComponent _returnvalue))))

(event EventBeginPlay
  ;[1 1 1] Bindings
  (EventDispatchers|AssignOnHPZero (Variables|Default|GetShip%20Hull) (delegate Custom|On%20HP%20Zero))
  (EventDispatchers|BindEventtoOnModuleAdded (delegate Custom|Ship%20Modules%20Changed))
  (EventDispatchers|BindEventtoOnModuleRemoved (delegate Custom|Ship%20Modules%20Changed))
  (CallFunction|TryLoadShip)
  ;[1 1 1] Init
  (|InitShield)
  (|InitDamageManager
    (:_
      (CallFunction|UpdateShipHP))))

(fn ConstructionScript)

(fn UpdateShipHP
  (bind _ship_hull (Variables|Default|GetShip%20Hull))
  (bind _ship_hull_2 (Variables|Default|GetShip%20Hull))
  (Variables|/Game/DamageSystem/Blueprints/BPC_DamageableLayer.BPC_DamageableLayer_C|SetMax%20HP _ship_hull_2 0)
  (Variables|/Game/DamageSystem/Blueprints/BPC_DamageableLayer.BPC_DamageableLayer_C|SetCurrent%20HP _ship_hull_2 0)
  (for _array_element (Components|GetChildrenComponents (Variables|Default|GetModel) false)
    (bind _aschild_actor_component (Utilities|Casting|CastToChildActorComponent _array_element))
    (bind _asbp_ship_module (Utilities|Casting|CastToBP_ShipModule (Variables|/Script/Engine.ChildActorComponent|GetChildActor _aschild_actor_component)))
    (bind _output_get (Variables|/Game/DamageSystem/Blueprints/BPC_DamageableLayer.BPC_DamageableLayer_C|SetMax%20HP _ship_hull (+ (Variables|/Game/DamageSystem/Blueprints/BPC_DamageableLayer.BPC_DamageableLayer_C|GetMax%20HP _ship_hull) (Variables|/Game/Ships/Modules/Base/Blueprints/BP_ShipModule.BP_ShipModule_C|GetDefault%20HP _asbp_ship_module))))
    (Variables|/Game/DamageSystem/Blueprints/BPC_DamageableLayer.BPC_DamageableLayer_C|SetCurrent%20HP _ship_hull _output_get)))

(fn LoadModule
  (params (Module%20Data :type BPS%20Ship%20Module%20Data%20World%20Structure))
  (bind (_modulename _position _rotation _flipped) (Utilities|Struct|BreakBPS_ShipModuleData_World Module%20Data))
  (bind _component (|SpawnChildActorComponent _modulename (Math|Transform|MakeTransform _position _rotation "1.000000,1.000000,1.000000")))
  (bind _asbp_ship_module (Utilities|Casting|CastToBP_ShipModule (Variables|/Script/Engine.ChildActorComponent|GetChildActor _component)))
  (Default|Initialize _asbp_ship_module self _modulename)
  (Default|InitializeMesh _asbp_ship_module _flipped)
  (Variables|/Game/Ships/Modules/Base/Blueprints/BP_ShipModule.BP_ShipModule_C|SetCleanup%20Time _asbp_ship_module (Variables|Default|GetCleanup%20Time))
  (Default|CallOnModuleAdded _asbp_ship_module)
  (return _asbp_ship_module))

(fn RemoveModule
  (params (Module :type BP%20Ship%20Module%20Object%20Reference))
  (for _array_element (Components|GetChildrenComponents (Variables|Default|GetModel) false)
    (bind _aschild_actor_component (Utilities|Casting|CastToChildActorComponent _array_element))
    (if (== (Variables|/Script/Engine.ChildActorComponent|GetChildActor _aschild_actor_component) Module)
      (Actor|DestroyActor (Variables|/Script/Engine.ChildActorComponent|GetChildActor _aschild_actor_component))
      (Components|DestroyComponent _aschild_actor_component)
      (Default|CallOnModuleRemoved Module)
      (return))))

(fn SetShipEnabled
  (params (Enable :type Boolean))
  (Variables|Default|SetIs%20Enabled Enable)
  (for _array_element (Components|GetChildrenComponents (Variables|Default|GetModel) false)
    (|SetModulesEnabled _array_element))
  (|SetCollisionandPhysics)
  (Actor|Tick|SetActorTickEnabled Enable)
  (Default|CallOnSetEnabled Enable))

(fn AddNewModule
  (params (Module%20Name :type Name))
  (bind _returnvalue (Utilities|GetDataTableRow "/Game/Ships/Modules/Base/DT_ShipModuleData.DT_ShipModuleData" Module%20Name)
    (:then
      (bind _module (CallFunction|LoadModule (Utilities|Struct|MakeBPS_ShipModuleData_World Module%20Name "0.000000,0.000000,0.000000" "0.000000,0.000000,0.000000" false)))
      (return _module _returnvalue))))

(fn LoadShipData
  (bind _returnvalue (Utilities|GetDataTableRow "/Game/Ships/DT_ShipData.DT_ShipData" (Variables|Default|GetShip%20Name))
    (:then
      (CallFunction|LoadShipfromData _returnvalue))))

(fn GetMaxFireRange
  (for _array_element (Components|GetChildrenComponents (Variables|Default|GetModel) false)
    (bind _aschild_actor_component (Utilities|Casting|CastToChildActorComponent _array_element))
    (bind _asbp_ship_weapon_particle (Utilities|Casting|CastToBP_ShipWeapon_Particle (Variables|/Script/Engine.ChildActorComponent|GetChildActor _aschild_actor_component)))
    (if (> (.ProjectileDistance (Utilities|Struct|BreakBPS_Weapon_Functional (.Functional (Utilities|Struct|BreakBPS_Weapon (Variables|/Game/Ships/Modules/Weapons/Blueprints/BP_ShipWeapon_Particle.BP_ShipWeapon_Particle_C|GetData _asbp_ship_weapon_particle))))) (LocalVariables|GetMax%20Distance))
      (LocalVariables|SetMax%20Distance (.ProjectileDistance (Utilities|Struct|BreakBPS_Weapon_Functional (.Functional (Utilities|Struct|BreakBPS_Weapon (Variables|/Game/Ships/Modules/Weapons/Blueprints/BP_ShipWeapon_Particle.BP_ShipWeapon_Particle_C|GetData _asbp_ship_weapon_particle))))))))
  (return (LocalVariables|GetMax%20Distance)))

(fn GetTotalShipPower
  (for _array_element (Components|GetChildrenComponents (Variables|Default|GetModel) false)
    (bind _aschild_actor_component (Utilities|Casting|CastToChildActorComponent _array_element))
    (bind _asbp_ship_module (Utilities|Casting|CastToBP_ShipModule (Variables|/Script/Engine.ChildActorComponent|GetChildActor _aschild_actor_component)))
    (LocalVariables|SetPower (+ (Default|GetPowerPoints _asbp_ship_module) (LocalVariables|GetPower))))
  (return (LocalVariables|GetPower)))

(fn SetShipReset
  (params (Reset :type Boolean))
  (Components|Activation|SetActive (Variables|Default|GetBPC_ShipSmoke) (not Reset) false)
  (Components|Activation|SetActive (Variables|Default|GetBPC_ShipFire) (not Reset) false)
  (Variables|/Game/Ships/BPC_ShieldDepletionIndicator.BPC_ShieldDepletionIndicator_C|SetDepleted (Variables|Default|GetBPC_ShieldDepletionIndicator) false)
  (for _array_element (Components|GetChildrenComponents (Variables|Default|GetModel) false)
    (|ResetModules _array_element)))

(fn HealShip
  (bind _ship_hull (Variables|Default|GetShip%20Hull))
  (bind _ship_shield (Variables|Default|GetShip%20Shield))
  (Default|TakeHeal _ship_hull (Variables|/Game/DamageSystem/Blueprints/BPC_DamageableLayer.BPC_DamageableLayer_C|GetMax%20HP _ship_hull))
  (Default|TakeHeal _ship_shield (Variables|/Game/DamageSystem/Blueprints/BPC_DamageableLayer.BPC_DamageableLayer_C|GetMax%20HP _ship_shield))
  (Components|Tick|SetComponentTickEnabled (Variables|Default|GetShield%20Regen) true))

(fn LoadShipfromData
  (params (Data :type BPS%20Ship%20Data%20World%20Structure))
  (bind (_modules _boxcollisioncenter _boxcollisionextent) (Utilities|Struct|BreakBPS_ShipData_World Data))
  (Variables|Default|SetGrid%20Offset _boxcollisioncenter)
  (Components|Box|SetBoxExtent (Variables|Components|GetBoxCollision) _boxcollisionextent true)
  (for _array_element _modules
    (CallFunction|LoadModule _array_element)))

(fn TryLoadShip
  (CallFunction|LoadShipData))