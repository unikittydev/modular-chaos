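; Component on BP_Grid that repositions the ship's camera while the ship grid editor is active.
; On editor start it caches the camera rotation, shifts the spring arm's TargetOffset along X by the arm length and sets a fixed camera rotation.
; When the grid ends play it restores that rotation and zeroes TargetOffset.
; The spring arm's SocketOffset is also saved but never used.
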(event `self.ReceiveBeginPlay`
  (bind _asbp_grid (cast `/Game/Ships/ShipEditor/Grid/BP_Grid` (`self.GetOwner`)))
  (bind _output_get (set `self.Grid` _asbp_grid))
  (add `/Game/Ships/ShipEditor/Grid/BP_Grid.On Editor Start` _output_get (delegate `Editor Start`))
  (add `Actor.OnEndPlay` _output_get (delegate `Editor End`)))

(event `self.ReceiveEndPlay`
  (params (EndPlayReason :type "EEndPlayReason Enum" :default "Destroyed"))
  (bind _grid (`self.Grid`))
  (remove `/Game/Ships/ShipEditor/Grid/BP_Grid.On Editor Start` _grid (delegate `Editor Start`))
  (remove `Actor.OnEndPlay` _grid (delegate `Editor End`)))

(event `Editor Start`
  (bind _ship (`self.Ship`))
  (bind _ship_2 (`self.Ship`))
  (bind _springarm (`/Game/Ships/Player/BP_Ship_Player.SpringArm` _ship_2))
  (set `self.Ship` (`/Game/Ships/ShipEditor/Grid/BP_Grid.Ship` (`self.Grid`)))
  (set `self.SpringArmOffset` (`SpringArmComponent.SocketOffset` _springarm))
  (set `self.CameraRotation` (`SceneComponent.RelativeRotation` (`/Game/Ships/Player/BP_Ship_Player.Camera` _ship_2)))
  (set `SpringArmComponent.TargetOffset` (`KismetMathLibrary.MakeVector` (`SpringArmComponent.TargetArmLength` _springarm)) (`/Game/Ships/Player/BP_Ship_Player.SpringArm` _ship))
  (`SceneComponent.K2_SetRelativeRotation` (`/Game/Ships/Player/BP_Ship_Player.Camera` _ship) (struct :`Pitch` -90.0) false false))

(event `Editor End`
  (params (Actor :type "Actor Object Reference") (EndPlayReason :type "EEndPlayReason Enum" :default "Destroyed"))
  (bind _ship (`self.Ship`))
  (`SceneComponent.K2_SetRelativeRotation` (`/Game/Ships/Player/BP_Ship_Player.Camera` _ship) (`self.CameraRotation`) false false)
  (set `SpringArmComponent.TargetOffset` (0.0 0.0 0.0) (`/Game/Ships/Player/BP_Ship_Player.SpringArm` _ship)))