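; Draggable proxy actor for the ship editor grid that lets the mouse move a target actor.
; A press becomes a drag past a pixel threshold, then the cursor is projected onto the game plane, keeping the grab offset.
; Drag events and position requests go out through Call hooks, and the target copies the proxy's transform.
; Helpers scale the cube to grid element size, swap correct/incorrect/default materials and draw a debug box.
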(event `self.ReceiveBeginPlay`
  (bind _output_get (set `self.Target Actor Meshes` (`self.K2_GetComponentsByClass` (`self.Target Actor`) "/Script/Engine.StaticMeshComponent")))
  (for _array_element _output_get
    (`KismetArrayLibrary.Array_Append` (`self.Default Materials`) (`MeshComponent.GetMaterials` _array_element))))

(event `self.ReceiveActorOnReleased`
  (params (ButtonReleased :type "Key Structure"))
  (set `self.isPressed` false)
  (`self.On Mouse Up`))

(event `self.ReceiveActorOnClicked`
  (params (ButtonPressed :type "Key Structure"))
  (bind _returnvalue (`WidgetLayoutLibrary.GetMousePositionOnViewport`))
  (set `self.Mouse Location` _returnvalue)
  (set `self.isPressed` (== ButtonPressed "LeftMouseButton"))
  (`self.On Mouse Down`))

(event `self.ReceiveTick`
  (params (DeltaSeconds :type "Float (single-precision)"))
  (bind _bpc_gridelement (`self.BPC_GridElement`))
  (bind (_returnvalue_x _returnvalue_y) (`KismetMathLibrary.BreakVector` (`KismetMathLibrary.Conv_IntVectorToVector` (`/Game/Ships/ShipEditor/Grid/BPC_GridElement.Size` _bpc_gridelement))))
  (if (`/Game/Ships/ShipEditor/Grid/BP_Grid.Draw Gizmos` (`/Game/Ships/ShipEditor/Grid/BPC_GridElement.Grid` (`self.BPC_GridElement`)))
    (`KismetSystemLibrary.DrawDebugBox` (`self.K2_GetActorLocation`) (* (`/Game/Ships/ShipEditor/Grid/BP_Grid.Cell Size` (`/Game/Ships/ShipEditor/Grid/BPC_GridElement.Grid` _bpc_gridelement)) 0.5 (`KismetMathLibrary.MakeVector` _returnvalue_x _returnvalue_y 1.0)) (`KismetMathLibrary.SelectColor` (struct :`G` 0.068148 :`B` 1.0 :`A` 1.0) (struct :`R` 1.0 :`G` 1.0 :`B` 1.0 :`A` 1.0) (`self.isDragged`))))
  (`|ExecutionSequence`
    (:`then_0`
      (if (`self.isPressed`)
        (bind _returnvalue (`WidgetLayoutLibrary.GetMousePositionOnViewport`))
        (if (> (`KismetMathLibrary.DistanceSquared2D` _returnvalue (`self.Mouse Location`)) (`KismetMathLibrary.Square` (`self.Drag Distance`)))
          (`self.BeginDrag`))))
    (:`then_1`
      (if (and (`PlayerController.WasInputKeyJustReleased` (`GameplayStatics.GetPlayerController` 0) "LeftMouseButton") (`self.isDragged`))
        (`self.EndDrag`)))
    (:`then_2`
      (if (`self.isDragged`)
        (`self.DragTick`)))))

(event `BeginDrag`
  (set `self.isPressed` false)
  (set `self.isDragged` true)
  (bind _location (`/Game/Blueprints/BPL_ScreenUtils.Project Mouse Location on Game Plane` (`GameplayStatics.GetPlayerController` 0)))
  (set `self.Position Offset` (- (`self.K2_GetActorLocation`) _location))
  (`self.On Drag Begin`))

(event `DragTick`
  (bind _location (`/Game/Blueprints/BPL_ScreenUtils.Project Mouse Location on Game Plane` (`GameplayStatics.GetPlayerController` 0)))
  (`self.Try Update Position` (+ _location (`self.Position Offset`)))
  (`self.Update Target Actor Transform`))

(event `EndDrag`
  (if (or (`self.isDragged`) (`self.isPressed`))
    (set `self.isPressed` false)
    (set `self.isDragged` false)
    (`self.On Drag End`)))

(event `self.ReceiveActorBeginCursorOver`
  (`self.On Cursor Over`))

(fn `Update Materials`
  (params (`Is Moving` :type Boolean) (`Is Correct` :type Boolean))
  (locals (`Material Index` :type Integer))
  (bind _returnvalue (select `bool` (`local.Is Correct`) :`false` (`self.Incorrect Material`) :`true` (select `bool` (`local.Is Moving`) :`true` (`self.Correct Material`) :!type "MaterialInterface Object Reference") :!type "MaterialInterface Object Reference"))
  (for _array_element (`self.Target Actor Meshes`)
    (for _index (range 1 (+ (`PrimitiveComponent.GetNumMaterials` _array_element) 1))
      (`PrimitiveComponent.SetMaterial` _array_element (- _index 1) (select `bool` (`KismetSystemLibrary.IsValid` _returnvalue) :`false` (`|GetArrayItem` (`self.Default Materials`) (`local.Material Index`)) :`true` _returnvalue))
      (`/Engine/EditorBlueprintResources/StandardMacros.IncrementInt` (`local.Material Index`)))))

(fn `Update Size`
  (bind (_size_x _size_y) (break `IntVector` (`/Game/Ships/ShipEditor/Grid/BPC_GridElement.Size` (`self.BPC_GridElement`))))
  (`SceneComponent.SetWorldScale3D` (`self.Cube`) (`KismetMathLibrary.MakeVector` (`KismetMathLibrary.Conv_IntToDouble` _size_x) (`KismetMathLibrary.Conv_IntToDouble` _size_y) 1.0)))

(fn `Update Target Actor Transform`
  (bind (_returnvalue_location _returnvalue_rotation) (`KismetMathLibrary.BreakTransform` (`self.GetTransform`)))
  (bind _target_actor (`self.Target Actor`))
  (`/Engine/EditorBlueprintResources/StandardMacros.IsValid` _target_actor
    (:`Is Valid`
      (`self.K2_SetActorLocationAndRotation` _target_actor _returnvalue_location _returnvalue_rotation false false)
      (return))))

(fn `UserConstructionScript`)