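; World trigger that opens the grid-based ship editor when the player's ship is in range and F is pressed.
; Sphere overlap drives an interact overlay and a color-coded status material; the radius expands a tick after BeginPlay.
; Loading spawns a centered BP_Grid, snaps, disables and heals the ship, registers its modules, and shows a one-time tutorial tracked by a save slot.
; Completing an edit saves the ship through BP_SaveHandler.
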(event `self.ReceiveBeginPlay`
  (bind _sphere (`self.Sphere`))
  (bind _returnvalue (`PrimitiveComponent.CreateDynamicMaterialInstance` (`self.Status Mesh`) 0 "/Game/Ships/ShipEditor/Materials/M_Grid_Status.M_Grid_Status" "None"))
  (bind _output_get (set `self.Status Material` _returnvalue))
  (`PrimitiveComponent.SetMaterial` (`self.Status Mesh`) 0 _output_get)
  (`SphereComponent.SetSphereRadius` _sphere 0.0 false)
  (`KismetSystemLibrary.DelayUntilNextTick`)
  (`SphereComponent.SetSphereRadius` _sphere 500.0 true))

(event `self.ReceiveActorBeginOverlap`
  (params (OtherActor :type "Actor Object Reference"))
  (bind _asbp_ship_player (cast `/Game/Ships/Player/BP_Ship_Player` OtherActor))
  (set `self.Ship` _asbp_ship_player)
  (`self.Update Status` "NewEnumerator1")
  (bind _returnvalue (`|CreateWidget` "/Game/Ships/ShipEditor/UI/WBP_InteractOverlay.WBP_InteractOverlay_C"))
  (bind _output_get (set `self.Overlay` _returnvalue))
  (`UserWidget.AddToViewport` _output_get 0))

(event `self.ReceiveActorEndOverlap`
  (params (OtherActor :type "Actor Object Reference"))
  (cast `/Game/Ships/Player/BP_Ship_Player` OtherActor)
  (set `self.Ship` null)
  (`self.Update Status` "NewEnumerator0")
  (`Widget.RemoveFromParent` (`self.Overlay`)))

(event `Update Status`
  (params (Status :type "/Game/Ships/ShipEditor/Grid/BPE_GridStatus Enum" :default "NewEnumerator0"))
  (bind _output_get (set `self.Grid Status` Status))
  (`self.SetActorTickEnabled` (`|EnumEquality` _output_get "NewEnumerator1"))
  (`MaterialInstanceDynamic.SetVectorParameterValue` (`self.Status Material`) "EmissionColor" (select `/Game/Ships/ShipEditor/Grid/BPE_GridStatus` (`self.Grid Status`) :`NewEnumerator0` (struct :`A` 1.0) :`NewEnumerator1` (struct :`G` 1.0 :`B` 0.856848 :`A` 1.0) :`NewEnumerator2` (struct :`R` 0.025951 :`B` 1.0 :`A` 1.0) :`NewEnumerator3` (struct :`R` 1.0 :`G` 0.052632 :`A` 1.0) :!type "LinearColor Structure")))

(event `Key|F`
  (params (Key :type "Key Structure"))
  (:`Pressed`
    (if (== (`self.Grid Status`) 1)
      (`self.Load Ship Editor` (`self.Ship`))
      (`self.Update Status` "NewEnumerator2")
      (add `/Game/Ships/ShipEditor/Grid/BP_Grid.On Edit Completed` (`self.Grid`) (delegate `Edit Completed`)))))

(event `Edit Completed`
  (params (`Ship Data` :type "/Game/Ships/ShipEditor/Structures/BPS_ShipData_World Structure"))
  (`self.Update Status` "NewEnumerator1")
  (bind _returnvalue (`GameplayStatics.GetActorOfClass` "/Game/Progression/BP_SaveHandler.BP_SaveHandler_C"))
  (`/Engine/EditorBlueprintResources/StandardMacros.IsValid` _returnvalue
    (:`Is Valid`
      (set `/Game/Progression/BP_SaveHandler.Ship Editor Activator` self _returnvalue)
      (set `/Game/Progression/BP_SaveGame_Player.Ship` `Ship Data` (`/Game/Progression/BP_SaveHandler.Save` _returnvalue))
      (`/Game/Progression/BP_SaveHandler.Save Game` _returnvalue))))

(fn `Load Ship Editor`
  (params (`Loaded Ship` :type "/Game/Ships/BP_Ship Object Reference"))
  (bind _intvector (make `IntVector` 5 5))
  (bind _loaded_ship (`local.Loaded Ship`))
  (bind _loaded_ship_2 (`local.Loaded Ship`))
  (bind _grid (`self.Grid`))
  (bind (_x _y) (break `IntVector` _intvector))
  (bind _returnvalue (`SceneComponent.K2_GetComponentToWorld` (`self.Cube`)))
  (bind (_returnvalue_x _returnvalue_y) (`KismetMathLibrary.BreakVector` (* (`KismetMathLibrary.MakeVector` (`KismetMathLibrary.Conv_IntToDouble` (- _x 1)) (`KismetMathLibrary.Conv_IntToDouble` (- _y 1))) 0.5 (`self.Test Cell Size`))))
  (bind _returnvalue_2 (`|SpawnActorFromClass` "/Game/Ships/ShipEditor/Grid/BP_Grid.BP_Grid_C" (`KismetMathLibrary.MakeTransform` (- (`KismetMathLibrary.MakeVector` (.x (.location _returnvalue)) (.y (.location _returnvalue))) (`KismetMathLibrary.MakeVector` _returnvalue_x _returnvalue_y)) (.rotation _returnvalue)) "AlwaysSpawn" "MultiplyWithRoot" null _intvector (`self.Test Cell Size`) (`local.Loaded Ship`) false (`self.Save to Table`) null))
  (bind _output_get (set `self.Grid` _returnvalue_2))
  (bind (_returnvalue_location _returnvalue_rotation) (`KismetMathLibrary.BreakTransform` (`self.GetTransform` _output_get)))
  (bind _returnvalue_3 (- _returnvalue_location (`/Game/Ships/BP_Ship.Grid Offset` (`local.Loaded Ship`))))
  (`self.K2_SetActorTransform` _loaded_ship (`KismetMathLibrary.MakeTransform` _returnvalue_3 _returnvalue_rotation) false true)
  (`SceneComponent.K2_SetWorldTransform` (`/Game/Ships/BP_Ship.BoxCollision` _loaded_ship) (`KismetMathLibrary.MakeTransform` _returnvalue_3 _returnvalue_rotation) false true)
  (`SceneComponent.K2_SetRelativeRotation` :`self` (`/Game/Ships/BP_Ship.Model` (`local.Loaded Ship`)))
  (`/Game/Ships/BP_Ship.Set Ship Enabled` _loaded_ship_2 false)
  (`/Game/Ships/BP_Ship.Set Ship Reset` _loaded_ship_2 true)
  (`/Game/Ships/BP_Ship.Heal Ship` _loaded_ship_2)
  (for _array_element (`SceneComponent.GetChildrenComponents` (`/Game/Ships/BP_Ship.Model` (`local.Loaded Ship`)) false)
    (bind _aschild_actor_component (cast `ChildActorComponent` _array_element))
    (bind _asbp_ship_module (cast `/Game/Ships/Modules/Base/Blueprints/BP_ShipModule` (`ChildActorComponent.ChildActor` _aschild_actor_component)))
    (bind (_position _rotation) (`/Game/Ships/ShipEditor/Grid/BP_Grid.Module Transform To Grid Position And Rotation` _grid _asbp_ship_module))
    (`/Game/Ships/ShipEditor/Grid/BP_Grid.Add Module To Grid` _grid _asbp_ship_module _position _rotation))
  (bind _returnvalue_4 (`GameplayStatics.DoesSaveGameExist` "tutorial"))
  (if (not _returnvalue_4)
    (bind _returnvalue_5 (`GameplayStatics.CreateSaveGameObject` "/Game/Ships/ShipEditor/Grid/BP_SaveGame_Tutorial.BP_SaveGame_Tutorial_C"))
    (set `/Game/Ships/ShipEditor/Grid/BP_SaveGame_Tutorial.Completed` true _returnvalue_5)
    (`GameplayStatics.SaveGameToSlot` _returnvalue_5 "tutorial")
    (`|SpawnActorFromClass` "/Game/Blueprints/BP_Tutorial.BP_Tutorial_C" (`KismetMathLibrary.MakeTransform` (0.0 0.0 0.0)) "AlwaysSpawn" "MultiplyWithRoot" null (`|MakeArray` "<normal>Перед тобой редактор кораблей</>" "<normal>Детали выставляются на сетку перетаскиванием с верхней панели. Убрать детали можно, перетащив их с сетки в свободное пространство</>" "<normal>Их можно двигать, вращать и отражать</>" "<normal>Если деталь пересекается с другой, или она задевает границы сетки, она подсветится красным, показывая, что она поставлена некорректно</>" "<normal>Для сохранения корабля все детали должны быть поставлены правильно. Также ему нужно хотя бы одно </><highlight>орудие</><normal> и один </><highlight>двигатель</>" "<normal>Ищите детали, укрепляйте корабль, и побеждайте всё более сильных противников!</>" :!type "Text") null)))

(fn `UserConstructionScript`)