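; Actor component that makes a draggable ship module an element of the ship editor grid, tracking its cell position, size, rotation and flip state.
; It binds to the owner's BP_DragDrop events, snapping the actor to cells and notifying the Grid as it moves.
; Drags set the grid's selection and play sounds, dropping outside removes the module, and hovering updates the module info UI.
; Quarter-turn rotation swaps size on odd turns, shifts position and re-snaps.
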(event `self.ReceiveBeginPlay`
  (bind _asbp_drag_drop (cast `/Game/Ships/ShipEditor/Grid/BP_DragDrop` (`self.GetOwner`)))
  (bind _output_get (set `self.Drag Drop` _asbp_drag_drop))
  (add `/Game/Ships/ShipEditor/Grid/BP_DragDrop.Try Update Position` _output_get (delegate `Update Position`))
  (add `/Game/Ships/ShipEditor/Grid/BP_DragDrop.On Drag End` _output_get (delegate `On Drag End`))
  (add `/Game/Ships/ShipEditor/Grid/BP_DragDrop.On Drag Begin` _output_get (delegate `On Drag Begin`))
  (add `/Game/Ships/ShipEditor/Grid/BP_DragDrop.On Cursor Over` _output_get (delegate `On Cursor Over`))
  (add `/Game/Ships/ShipEditor/Grid/BP_DragDrop.On Mouse Down` _output_get (delegate `On Mouse Down`))
  (add `/Game/Ships/ShipEditor/Grid/BP_DragDrop.On Mouse Up` _output_get (delegate `On Mouse Up`)))

(event `Update Position`
  (params (Position :type "Vector Structure"))
  (bind (_size_x _size_y) (break `IntVector` (`self.Size`)))
  (bind (_x _y _z) (break `IntVector` (`self.Position`)))
  (bind _cell_size (`/Game/Ships/ShipEditor/Grid/BP_Grid.Cell Size` (`self.Grid`)))
  (bind _returnvalue (`KismetMathLibrary.Vector_SnappedToGrid` (`KismetMathLibrary.InverseTransformLocation` (`Actor.GetTransform` (`self.Grid`)) Position) _cell_size))
  (bind _returnvalue_2 (`KismetMathLibrary.FTruncVector` (/ _returnvalue _cell_size)))
  (bind (_x_2 _y_2 _z_2) (break `IntVector` _returnvalue_2))
  (if (or (!= _x_2 _x) (!= _y_2 _y) (!= _z_2 _z))
    (bind _output_get (set `self.Position` _returnvalue_2))
    (`self.Grid Position Changed` _output_get true)
    (`Actor.K2_SetActorLocation` (`self.GetOwner`) (+ (`KismetMathLibrary.TransformLocation` (`Actor.GetTransform` (`self.Grid`)) _returnvalue) (* (`KismetMathLibrary.Conv_IntVectorToVector` (make `IntVector` (- 1 (mod _size_x 2)) (- 1 (mod _size_y 2)))) 0.5 (`/Game/Ships/ShipEditor/Grid/BP_Grid.Cell Size` (`self.Grid`)))) false false)))

(event `Grid Position Changed`
  (params (`New Position` :type "IntVector Structure") (`Is Moving` :type Boolean))
  (`/Game/Ships/ShipEditor/Grid/BP_Grid.Update Element` (`self.Grid`) self `Is Moving`))

(event `On Drag End`
  (bind _grid (`self.Grid`))
  (`GameplayStatics.PlaySound2D` "/Game/Audio/ShipEditor/SW_ShipEditor_Place.SW_ShipEditor_Place" 1.0 1.0 0.0 null null)
  (set `/Game/Ships/ShipEditor/Grid/BP_Grid.Selected Element` null (`self.Grid`))
  (bind __ (`/Game/Ships/ShipEditor/Grid/BP_Grid.Is Element Outside Grid` (`self.Grid`) self))
  (if __
    (`/Game/Ships/ShipEditor/Grid/BP_Grid.Remove Ship Module` _grid self)
    (`/Game/Ships/ShipEditor/Grid/BP_Grid.Remove` _grid self))
  (`/Game/Ships/ShipEditor/Grid/BP_Grid.Update Elements` (`self.Grid`) false))

(event `On Drag Begin`
  (`GameplayStatics.PlaySound2D` "/Game/Audio/ShipEditor/SW_ShipEditor_Take.SW_ShipEditor_Take" 1.0 1.0 0.0 null null)
  (set `/Game/Ships/ShipEditor/Grid/BP_Grid.Selected Element` self (`self.Grid`))
  (`/Game/Ships/ShipEditor/Grid/BP_Grid.Update Elements` (`self.Grid`) false)
  (`/Game/Ships/ShipEditor/Grid/BP_Grid.Update Element` (`self.Grid`) self true))

(event `On Cursor Over`
  (bind _grid (`self.Grid`))
  (`/Game/Ships/ShipEditor/UI/WBP_ModuleInfoList.Update Module Info` (`/Game/Ships/ShipEditor/UI/WBP_ShipEditor.ModuleInfo` (`/Game/Ships/ShipEditor/Grid/BP_Grid.UI` _grid)) (`/Game/Ships/Modules/Base/Blueprints/BP_ShipModule.Module Name` (`BlueprintMapLibrary.Map_Find` (`/Game/Ships/ShipEditor/Grid/BP_Grid.ModuleMap` _grid) self))))

(event `On Mouse Down`)

(event `On Mouse Up`)

(fn `Contains Position`
  (params (Position :type "IntVector Structure"))
  (returns (_ :type Boolean))
  (bind (_size_x _size_y) (break `IntVector` (`self.Size`)))
  (bind (_position_x _position_y) (break `IntVector` (`self.Position`)))
  (return (and (>= Position_X _position_x) (>= Position_Y _position_y) (< Position_X (+ _position_x _size_x)) (< Position_Y (+ _position_y _size_y)))))

(fn `Flip`
  (set `self.Flipped` (not (`self.Flipped`))))

(fn `Get Max Position`
  (returns (Min :type "IntVector Structure"))
  (bind (_size_x _size_y) (break `IntVector` (`self.Size`)))
  (bind (_position_x _position_y) (break `IntVector` (`self.Position`)))
  (return (make `IntVector` (+ _position_x (- _size_x 1)) (+ _position_y (- _size_y 1)))))

(fn `Get Min Position`
  (returns (Min :type "IntVector Structure"))
  (return (`self.Position`)))

(fn `Rotate 90 Degrees`
  (params (Times :type Integer))
  (bind _returnvalue (`self.GetOwner`))
  (bind (_size_x _size_y) (break `IntVector` (`self.Size`)))
  (bind (_size_x_2 _size_y_2) (break `IntVector` (`self.Size`)))
  (bind (_position_x _position_y) (break `IntVector` (`self.Position`)))
  (bind _returnvalue_2 (/ (- _size_x_2 _size_y_2) 2))
  (set `self.Rotation` (mod (+ Times (`self.Rotation`)) 4))
  (if (!= (mod Times 2) 0)
    (set `self.Size` (make `IntVector` _size_y _size_x)))
  (set `self.Position` (make `IntVector` (+ _position_x _returnvalue_2) (- _position_y _returnvalue_2)))
  (`Actor.K2_SetActorRotation` _returnvalue (`KismetMathLibrary.ComposeRotators` (`Actor.K2_GetActorRotation` _returnvalue) (`KismetMathLibrary.MakeRotator` 0.0 0.0 (* Times 90.0))) false)
  (`self.Update Position` (`Actor.K2_GetActorLocation` (`self.GetOwner`))))