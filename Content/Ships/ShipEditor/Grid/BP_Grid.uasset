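; Grid actor for the ship editor, where the player places, rotates and flips modules on a cell grid.
; Each module gets a BP_DragDrop proxy whose grid element is mapped to it, with materials showing whether placement is valid.
; Adding or removing modules updates the ship's inventory.
; Saving requires valid placement, a thruster and a weapon, then recenters the ship's box collision and modules, emits ship data and destroys the grid.
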(event `Module Added` :!signature `self.On Module Added`
  (params (`Module Name` :type Name))
  (`/Game/Ships/Player/BPC_Inventory.Remove Item` (`/Game/Ships/Player/BP_Ship_Player.Inventory` (`self.Ship`)) `Module Name`))

(event `Module Removed` :!signature `self.On Module Removed`
  (params (`Module Name` :type Name))
  (`/Game/Ships/Player/BPC_Inventory.Add Item` (`/Game/Ships/Player/BP_Ship_Player.Inventory` (`self.Ship`)) `Module Name`))

(event `self.ReceiveBeginPlay`
  (bind _returnvalue (`GameplayStatics.GetPlayerController` 0))
  (bind (_resolution_x _resolution_y) (break `IntVector` (`self.Resolution`)))
  (for _index (range (* _resolution_x _resolution_y))
    (bind _returnvalue_2 (`|SpawnActorFromClass` "/Game/Ships/ShipEditor/Grid/BP_GridCell.BP_GridCell_C" (`KismetMathLibrary.MakeTransform` (* (`self.Get Position From Index` _index) (`self.Cell Size`))) "AlwaysSpawn" "MultiplyWithRoot" self null))
    (`self.K2_AttachToActor` _returnvalue_2 self "None" "KeepRelative" "KeepRelative" "KeepRelative" true)
    (`KismetArrayLibrary.Array_Add` (`self.Cells`) _returnvalue_2))
  (`/Engine/EditorBlueprintResources/StandardMacros.IsValid` (`self.Ship`)
    (:`Is Valid`
      _)
    (:`Is Not Valid`
      (bind _returnvalue_3 (`GameplayStatics.GetActorOfClass` "/Game/Ships/Player/BP_Ship_Player.BP_Ship_Player_C"))
      (set `self.Ship` _returnvalue_3)
      (`self.Load Ship` (make `/Game/Ships/ShipEditor/Structures/BPS_ShipData_Grid` (make `/Game/Ships/ShipEditor/Structures/BPS_GridData` (make `IntVector` 5 5) 100.0) (`|MakeArray` (make `/Game/Ships/ShipEditor/Structures/BPS_ShipModuleData_Grid` "Thruster" (make `IntVector` 2 3)) (make `/Game/Ships/ShipEditor/Structures/BPS_ShipModuleData_Grid` "Thruster" (make `IntVector` 2 2)) (make `/Game/Ships/ShipEditor/Structures/BPS_ShipModuleData_Grid` "Test" (make `IntVector` 3 1) 3) (make `/Game/Ships/ShipEditor/Structures/BPS_ShipModuleData_Grid` "Test" (make `IntVector` 3 3) 1))))))
  (add `self.On Module Added` (delegate `Module Added`))
  (add `self.On Module Removed` (delegate `Module Removed`))
  (if (`self.Save On BeginPlay`)
    (`KismetSystemLibrary.DelayUntilNextTick`)
    (`self.Save`)
    (else
      (bind _returnvalue_4 (`|CreateWidget` "/Game/Ships/ShipEditor/UI/WBP_ShipEditor.WBP_ShipEditor_C" (`GameplayStatics.GetPlayerController` 0) self))
      (bind _output_get (set `self.UI` _returnvalue_4))
      (`UserWidget.AddToViewport` _returnvalue_4 0)
      (`UserWidget.AddToViewport` _output_get 0)
      (set `PlayerController.bShowMouseCursor` true _returnvalue)
      (`WidgetBlueprintLibrary.SetInputMode_GameAndUIEx` _returnvalue _output_get "DoNotLock" false)
      (for _array_element (`self.Elements`)
        (`self.Update Element` _array_element))
      (`self.On Editor Start`))))

(event `self.ReceiveTick`
  (params (DeltaSeconds :type "Float (single-precision)"))
  (if (`self.Draw Gizmos`)
    (bind (_center _extent) (`self.Get Ship Bounds`))
    (`KismetSystemLibrary.DrawDebugBox` _center _extent (struct :`R` 0.971142 :`G` 1.0 :`A` 1.0))))

(event `Key|Q`
  (params (Key :type "Key Structure"))
  (bind _selected_element (`self.Selected Element`))
  (:`Pressed`
    (`/Engine/EditorBlueprintResources/StandardMacros.IsValid` _selected_element
      (:`Is Valid`
        (`/Game/Ships/ShipEditor/Grid/BPC_GridElement.Rotate 90 Degrees` _selected_element -1)))))

(event `Key|E`
  (params (Key :type "Key Structure"))
  (bind _selected_element (`self.Selected Element`))
  (:`Pressed`
    (`/Engine/EditorBlueprintResources/StandardMacros.IsValid` _selected_element
      (:`Is Valid`
        (`/Game/Ships/ShipEditor/Grid/BPC_GridElement.Rotate 90 Degrees` _selected_element 1)))))

(event `Key|Z`
  (params (Key :type "Key Structure"))
  (bind _selected_element (`self.Selected Element`))
  (:`Pressed`
    (`/Engine/EditorBlueprintResources/StandardMacros.IsValid` _selected_element
      (:`Is Valid`
        (`/Game/Ships/ShipEditor/Grid/BPC_GridElement.Flip` _selected_element)
        (`/Game/Ships/Modules/Base/Blueprints/BP_ShipModule.Initialize Mesh` (`BlueprintMapLibrary.Map_Find` (`self.ModuleMap`) _selected_element) (`/Game/Ships/ShipEditor/Grid/BPC_GridElement.Flipped` _selected_element))
        (`self.Update Element` (`self.Selected Element`) true)))))

(event `Key|Enter`
  (params (Key :type "Key Structure"))
  (:`Pressed`
    (if (not (`KismetSystemLibrary.IsValid` (`self.Selected Element`)))
      (`self.Save`))))

(event `Save`
  (bind _returnvalue (`GameplayStatics.GetPlayerController` 0))
  (bind _ui (`self.UI`))
  (bind (__ _error_message) (`self.Can Save`))
  (if __
    (`self.Correct Ship Module Locations`)
    (if (`self.Save To Table`)
      (`self.On Ship Save`))
    (bind _data (`self.Get Ship Data`))
    (`/Engine/EditorBlueprintResources/StandardMacros.IsValid` _ui
      (:`Is Valid`
        (`Widget.RemoveFromParent` _ui)
        (set `PlayerController.bShowMouseCursor` false _returnvalue)
        (`WidgetBlueprintLibrary.SetInputMode_GameOnly` _returnvalue))
      (:`Is Not Valid`
        _))
    (for _array_element (`self.Elements`)
      (`self.K2_DestroyActor` (`ActorComponent.GetOwner` _array_element)))
    (for _array_element_2 (`self.Cells`)
      (`self.K2_DestroyActor` _array_element_2))
    (`self.K2_DestroyActor`)
    (`/Game/Ships/BP_Ship.Set Ship Enabled` (`self.Ship`) true)
    (`self.On Edit Completed` _data)
    (else
      (`/Game/Ships/ShipEditor/UI/WBP_ShipEditor.On Save Error` (`self.UI`) _error_message))))

(fn `Add`
  (params (Element :type "/Game/Ships/ShipEditor/Grid/BPC_GridElement Object Reference"))
  (if (not (`KismetArrayLibrary.Array_Contains` (`self.Elements`) Element))
    (`KismetArrayLibrary.Array_Add` (`self.Elements`) Element)
    (`self.On Element Add` Element))
  (`self.Update Element` (`local.Element`)))

(fn `Add Module To Grid`
  (params (Module :type "/Game/Ships/Modules/Base/Blueprints/BP_ShipModule Object Reference (by ref)") (`Grid Position` :type "IntVector Structure") (`Grid Rotation` :type Integer))
  (bind _drag_drop_actor (`self.Create Drag Drop Actor` (`.Size_6_486419E04BAEE024BCD892A2D43727DB` (break `/Game/Ships/Modules/Base/Structures/BPS_ShipModuleData` (`/Game/Ships/Modules/Base/Blueprints/BP_ShipModule.Module Data` Module))) false Module))
  (set `/Game/Ships/ShipEditor/Grid/BP_DragDrop.Target Actor` Module _drag_drop_actor)
  (bind _bpc_gridelement (`/Game/Ships/ShipEditor/Grid/BP_DragDrop.BPC_GridElement` _drag_drop_actor))
  (`BlueprintMapLibrary.Map_Add` (`self.ModuleMap`) _bpc_gridelement Module)
  (`/Game/Ships/ShipEditor/Grid/BPC_GridElement.Rotate 90 Degrees` _bpc_gridelement `Grid Rotation`)
  (`/Game/Ships/ShipEditor/Grid/BPC_GridElement.Update Position` _bpc_gridelement (`KismetMathLibrary.TransformLocation` (`self.GetTransform`) (`self.Grid to Relative Location` `Grid Position`)))
  (`/Game/Ships/ShipEditor/Grid/BPC_GridElement.Grid Position Changed` _bpc_gridelement `Grid Position` false)
  (`/Game/Ships/ShipEditor/Grid/BP_DragDrop.Update Target Actor Transform` _drag_drop_actor)
  (set `/Game/Ships/ShipEditor/Grid/BPC_GridElement.Flipped` (`/Game/Ships/Modules/Base/Blueprints/BP_ShipModule.Is Flipped` (`local.Module`)) _bpc_gridelement)
  (`self.Add` _bpc_gridelement))

(fn `Add Ship Module`
  (params (`Module Name` :type Name))
  (returns (`Drag Drop Actor` :type "/Game/Ships/ShipEditor/Grid/BP_DragDrop Object Reference"))
  (bind (_module _module_data) (`/Game/Ships/BP_Ship.Add New Module` (`self.Ship`) `Module Name`))
  (`/Game/Ships/Modules/Base/Blueprints/BP_ShipModule.On Disable` _module)
  (bind _drag_drop_actor (`self.Create Drag Drop Actor` (`.Size_6_486419E04BAEE024BCD892A2D43727DB` (break `/Game/Ships/Modules/Base/Structures/BPS_ShipModuleData` _module_data)) true _module))
  (set `/Game/Ships/ShipEditor/Grid/BP_DragDrop.Target Actor` _module _drag_drop_actor)
  (bind _bpc_gridelement (`/Game/Ships/ShipEditor/Grid/BP_DragDrop.BPC_GridElement` _drag_drop_actor))
  (`BlueprintMapLibrary.Map_Add` (`self.ModuleMap`) _bpc_gridelement _module)
  (`/Game/Ships/ShipEditor/Grid/BPC_GridElement.On Drag Begin` _bpc_gridelement)
  (`self.On Module Added` `Module Name`)
  (return _drag_drop_actor))

(fn `Can Place Element`
  (params (Element :type "/Game/Ships/ShipEditor/Grid/BPC_GridElement Object Reference"))
  (returns (_ :type Boolean))
  (bind (_position_x _position_y) (break `IntVector` (`/Game/Ships/ShipEditor/Grid/BPC_GridElement.Position` Element)))
  (bind (_size_x _size_y) (break `IntVector` (`/Game/Ships/ShipEditor/Grid/BPC_GridElement.Size` Element)))
  (for _index (range _size_y)
    (for _index_2 (range _size_x)
      (bind _intvector (make `IntVector` (+ _index_2 _position_x) (+ _index _position_y)))
      (bind __ (`self.Contains Position` _intvector))
      (if __
        (bind _count (`self.Get Modules Count at Position` _intvector))
        (if (> _count 1)
          (return false))
        (else
          (return false)))))
  (return true))

(fn `Can Save`
  (returns (_ :type Boolean) (`Error Message` :type Text))
  (locals (hasThruster :type Boolean) (hasWeapon :type Boolean))
  (for _array_element (`self.Elements`)
    (bind __ (`self.Can Place Element` _array_element))
    (if (not __)
      (return false "Ошибка: детали поставлены некорректно")))
  (set `local.hasThruster` false)
  (set `local.hasWeapon` false)
  (bind _values (`BlueprintMapLibrary.Map_Values` (`self.ModuleMap`)))
  (for _array_element_2 _values
    (cast `/Game/Ships/Modules/Thruster/BP_ShipThruster` _array_element_2
      (:`then`
        (set `local.hasThruster` true))
      (:`CastFailed`
        (cast `/Game/Ships/Modules/Weapons/Blueprints/BP_ShipWeapon_Particle` _array_element_2
          (:`then`
            (set `local.hasWeapon` true))
          (:`CastFailed`
            (cast `/Game/Ships/Modules/Squadron/BP_ShipWeapon_Squadron` _array_element_2)
            (set `local.hasWeapon` true))))))
  (return (and (`local.hasThruster`) (`local.hasWeapon`)) (select `bool` (`local.hasThruster`) :`false` "Ошибка: отсутствует двигатель" :`true` "Ошибка: отсутствует вооружение" :!type "Text")))

(fn `Contains Position`
  (params (Position :type "IntVector Structure"))
  (returns (_ :type Boolean))
  (bind (_resolution_x _resolution_y) (break `IntVector` (`self.Resolution`)))
  (return (and (>= Position_X 0) (>= Position_Y 0) (< Position_X _resolution_x) (< Position_Y _resolution_y))))

(fn `Correct Ship Module Locations`
  (locals (`Camera Offset` :type "Vector Structure") (`Old Location` :type "Vector Structure"))
  (bind _boxcollision (`/Game/Ships/BP_Ship.BoxCollision` (`self.Ship`)))
  (set `local.Old Location` (`self.K2_GetActorLocation` (`self.Ship`)))
  (bind (_center _extent) (`self.Get Ship Bounds`))
  (`BoxComponent.SetBoxExtent` _boxcollision _extent false)
  (bind _returnvalue (- (`local.Old Location`) _center))
  (`SceneComponent.K2_SetWorldLocation` _boxcollision (- (`SceneComponent.K2_GetComponentLocation` _boxcollision) _returnvalue) false true)
  (for _array_element (`SceneComponent.GetChildrenComponents` (`/Game/Ships/BP_Ship.Model` (`self.Ship`)) false)
    (bind _aschild_actor_component (cast `ChildActorComponent` _array_element))
    (`SceneComponent.K2_SetRelativeLocation` _aschild_actor_component (+ (`SceneComponent.RelativeLocation` _aschild_actor_component) _returnvalue) false true))
  (set `/Game/Ships/BP_Ship.Grid Offset` (- (`self.K2_GetActorLocation`) _center) (`self.Ship`))
  (return))

(fn `Create Drag Drop Actor`
  (params (Size :type "IntVector Structure") (`Is Dragged` :type Boolean) (Module :type "/Game/Ships/Modules/Base/Blueprints/BP_ShipModule Object Reference"))
  (returns (`Drag Drop Actor` :type "/Game/Ships/ShipEditor/Grid/BP_DragDrop Object Reference"))
  (bind _returnvalue (`|SpawnActorFromClass` "/Game/Ships/ShipEditor/Grid/BP_DragDrop.BP_DragDrop_C" (`KismetMathLibrary.MakeTransform` (0.0 0.0 0.0)) "AlwaysSpawn" "MultiplyWithRoot" null `Is Dragged` Module null))
  (bind _bpc_gridelement (`/Game/Ships/ShipEditor/Grid/BP_DragDrop.BPC_GridElement` _returnvalue))
  (set `/Game/Ships/ShipEditor/Grid/BPC_GridElement.Size` Size _bpc_gridelement)
  (set `/Game/Ships/ShipEditor/Grid/BPC_GridElement.Grid` self _bpc_gridelement)
  (`self.Add` self _bpc_gridelement)
  (`/Game/Ships/ShipEditor/Grid/BP_DragDrop.Update Size` _returnvalue)
  (return _returnvalue))

(fn `Get Flat Index 2D`
  (params (Position :type "IntVector Structure"))
  (returns (Index :type Integer))
  (bind _resolution_x (break `IntVector` (`self.Resolution`)))
  (return (+ Position_X (* Position_Y _resolution_x))))

(fn `Get Modules Count at Position`
  (params (Position :type "IntVector Structure"))
  (returns (Count :type Integer))
  (locals (_c :type Integer))
  (for _array_element (`self.Elements`)
    (if (`/Game/Ships/ShipEditor/Grid/BPC_GridElement.Contains Position` _array_element Position)
      (`/Engine/EditorBlueprintResources/StandardMacros.IncrementInt` (`local._c`))))
  (return (`local._c`)))

(fn `Get Position From Index`
  (params (Index :type Integer))
  (returns (Position :type "IntVector Structure"))
  (bind _resolution_x (break `IntVector` (`self.Resolution`)))
  (return (make `IntVector` (mod Index _resolution_x) (/ Index _resolution_x))))

(fn `Get Ship Bounds`
  (returns (Center :type "Vector Structure") (Extent :type "Vector Structure"))
  (locals (Min :type "IntVector Structure") (Max :type "IntVector Structure"))
  (bind (_min_x _min_y _min_z) (break `IntVector` (`local.Min`)))
  (bind (_max_x _max_y _max_z) (break `IntVector` (`local.Max`)))
  (set `local.Min` (`self.Resolution`))
  (set `local.Max` (make `IntVector` 0))
  (for _array_element (`self.Elements`)
    (bind (_position_x _position_y _position_z) (break `IntVector` (`/Game/Ships/ShipEditor/Grid/BPC_GridElement.Position` _array_element)))
    (bind (_size_x _size_y _size_z) (break `IntVector` (`/Game/Ships/ShipEditor/Grid/BPC_GridElement.Size` _array_element)))
    (bind (_intvector_x _intvector_y _intvector_z) (break `IntVector` (make `IntVector` (+ _position_x _size_x -1) (+ _position_y _size_y -1) (+ _position_z _size_z -1))))
    (set `local.Max` (make `IntVector` (`KismetMathLibrary.Max` _intvector_x _max_x) (`KismetMathLibrary.Max` _intvector_y _max_y) (`KismetMathLibrary.Max` _intvector_z _max_z)))
    (bind (_position_x_2 _position_y_2 _position_z_2) (break `IntVector` (`/Game/Ships/ShipEditor/Grid/BPC_GridElement.Position` _array_element)))
    (set `local.Min` (make `IntVector` (`KismetMathLibrary.Min` _position_x_2 _min_x) (`KismetMathLibrary.Min` _position_y_2 _min_y) (`KismetMathLibrary.Min` _position_z_2 _min_z))))
  (return (`KismetMathLibrary.TransformLocation` (`self.GetTransform`) (* (+ (`KismetMathLibrary.Conv_IntVectorToVector` (`local.Max`)) (`KismetMathLibrary.Conv_IntVectorToVector` (`local.Min`))) (* (1.0 1.0 0.0) (`self.Cell Size`) 0.5))) (* (+ (- (`KismetMathLibrary.Conv_IntVectorToVector` (`local.Max`)) (`KismetMathLibrary.Conv_IntVectorToVector` (`local.Min`))) (1.0 1.0 1.0)) 0.5 (`self.Cell Size`))))

(fn `Get Ship Data`
  (returns (Data :type "/Game/Ships/ShipEditor/Structures/BPS_ShipData_World Structure"))
  (locals (Modules :type "Array of /Game/Ships/ShipEditor/Structures/BPS_ShipModuleData_World Structure") (`Box Grid Offset` :type "Vector Structure") (`Box Extent` :type "Vector Structure"))
  (bind _returnvalue (`self.GetTransform`))
  (bind _modulemap (`self.ModuleMap`))
  (bind (_center _extent) (`self.Get Ship Bounds`))
  (set `local.Box Extent` _extent)
  (set `local.Box Grid Offset` (* (`KismetMathLibrary.InverseTransformLocation` (`self.GetTransform`) (`SceneComponent.K2_GetComponentLocation` (`/Game/Ships/BP_Ship.BoxCollision` (`self.Ship`)))) -1.0))
  (bind _keys (`BlueprintMapLibrary.Map_Keys` _modulemap))
  (for _array_element _keys
    (bind _value (`BlueprintMapLibrary.Map_Find` _modulemap _array_element))
    (bind (_returnvalue_location _returnvalue_rotation) (`KismetMathLibrary.BreakTransform` (`self.GetTransform` _value)))
    (`KismetArrayLibrary.Array_Add` (`local.Modules`) (make `/Game/Ships/ShipEditor/Structures/BPS_ShipModuleData_World` (`/Game/Ships/Modules/Base/Blueprints/BP_ShipModule.Module Name` _value) (+ (`local.Box Grid Offset`) (`KismetMathLibrary.InverseTransformLocation` _returnvalue _returnvalue_location)) (`KismetMathLibrary.InverseTransformRotation` _returnvalue _returnvalue_rotation) (`/Game/Ships/ShipEditor/Grid/BPC_GridElement.Flipped` _array_element))))
  (return (make `/Game/Ships/ShipEditor/Structures/BPS_ShipData_World` (`local.Modules`) (`local.Box Grid Offset`) (`local.Box Extent`))))

(fn `Grid Position And Rotation To Transform`
  (params (Position :type "IntVector Structure") (Rotation :type Integer))
  (returns (`Relative Location` :type "Vector Structure") (`Relative Rotation` :type "Rotator Structure"))
  (return (* (`KismetMathLibrary.Conv_IntVectorToVector` Position) (`self.Cell Size`)) (`KismetMathLibrary.MakeRotator` 0.0 0.0 (`KismetMathLibrary.Conv_IntToDouble` (* Rotation 90)))))

(fn `Grid to Relative Location`
  (params (`Grid Position` :type "IntVector Structure"))
  (returns (`Relative Location` :type "Vector Structure"))
  (return (* (`KismetMathLibrary.Conv_IntVectorToVector` `Grid Position`) (`self.Cell Size`))))

(fn `Is Element Outside Grid`
  (params (Element :type "/Game/Ships/ShipEditor/Grid/BPC_GridElement Object Reference"))
  (returns (_ :type Boolean))
  (bind (_position_x _position_y) (break `IntVector` (`/Game/Ships/ShipEditor/Grid/BPC_GridElement.Position` Element)))
  (bind (_size_x _size_y) (break `IntVector` (`/Game/Ships/ShipEditor/Grid/BPC_GridElement.Size` Element)))
  (for _index (range _size_y)
    (for _index_2 (range _size_x)
      (bind (_intvector_x _intvector_y) (break `IntVector` (make `IntVector` _index_2 _index)))
      (bind __ (`self.Contains Position` (make `IntVector` (+ _intvector_x _position_x) (+ _intvector_y _position_y))))
      (if __
        (return false))))
  (return true))

(fn `Load Ship`
  (params (`Ship Data` :type "/Game/Ships/ShipEditor/Structures/BPS_ShipData_Grid Structure"))
  (bind (_grid _modules) (break `/Game/Ships/ShipEditor/Structures/BPS_ShipData_Grid` `Ship Data`))
  (bind (_resolution _cellsize) (break `/Game/Ships/ShipEditor/Structures/BPS_GridData` _grid))
  (`/Game/Ships/BP_Ship.Set Ship Enabled` (`self.Ship`) false)
  (set `self.Resolution` _resolution)
  (set `self.Cell Size` _cellsize)
  (for _array_element _modules
    (`self.Load Ship Module` _array_element)))

(fn `Load Ship Module`
  (params (`Module Data` :type "/Game/Ships/ShipEditor/Structures/BPS_ShipModuleData_Grid Structure"))
  (bind (_modulename _position _rotation) (break `/Game/Ships/ShipEditor/Structures/BPS_ShipModuleData_Grid` `Module Data`))
  (bind _module (`/Game/Ships/BP_Ship.Add New Module` (`self.Ship`) _modulename))
  (`self.Add Module To Grid` _module _position _rotation))

(fn `Module Transform To Grid Position And Rotation`
  (params (Module :type "/Game/Ships/Modules/Base/Blueprints/BP_ShipModule Object Reference"))
  (returns (Position :type "IntVector Structure") (Rotation :type Integer))
  (bind _returnvalue (`self.GetTransform`))
  (bind (_returnvalue_roll _returnvalue_pitch _returnvalue_yaw) (`KismetMathLibrary.BreakRotator` (`KismetMathLibrary.InverseTransformRotation` _returnvalue (`self.K2_GetActorRotation` Module))))
  (return (`self.Relative to Grid Location` (`KismetMathLibrary.InverseTransformLocation` _returnvalue (`self.K2_GetActorLocation` Module))) (`KismetMathLibrary.FTrunc` (/ _returnvalue_yaw 90.0))))

(fn `Relative to Grid Location`
  (params (`Relative Location` :type "Vector Structure"))
  (returns (`Grid Location` :type "IntVector Structure"))
  (return (`KismetMathLibrary.FTruncVector` (/ (+ `Relative Location` 1.0) (`self.Cell Size`)))))

(fn `Remove`
  (params (Element :type "/Game/Ships/ShipEditor/Grid/BPC_GridElement Object Reference"))
  (`KismetArrayLibrary.Array_RemoveItem` (`self.Elements`) Element)
  (`self.On Element Remove` Element))

(fn `Remove Ship Module`
  (params (`Grid Element` :type "/Game/Ships/ShipEditor/Grid/BPC_GridElement Object Reference"))
  (bind (_value _returnvalue) (`BlueprintMapLibrary.Map_Find` (`self.ModuleMap`) `Grid Element`))
  (if _returnvalue
    (`ActorComponent.K2_DestroyComponent` `Grid Element`)
    (`self.On Module Removed` (`/Game/Ships/Modules/Base/Blueprints/BP_ShipModule.Module Name` _value))
    (`self.K2_DestroyActor` (`ActorComponent.GetOwner` `Grid Element`))
    (`/Game/Ships/BP_Ship.Remove Module` (`self.Ship`) _value)
    (`BlueprintMapLibrary.Map_Remove` (`self.ModuleMap`) (`local.Grid Element`))))

(fn `Update Element`
  (params (Element :type "/Game/Ships/ShipEditor/Grid/BPC_GridElement Object Reference") (`Is Moving` :type Boolean))
  (bind __ (`self.Can Place Element` Element))
  (`/Game/Ships/ShipEditor/Grid/BP_DragDrop.Update Materials` (`/Game/Ships/ShipEditor/Grid/BPC_GridElement.Drag Drop` Element) `Is Moving` __))

(fn `Update Elements`
  (params (`Is Moving` :type Boolean))
  (for _array_element (`self.Elements`)
    (`self.Update Element` _array_element `Is Moving`)))

(fn `UserConstructionScript`)