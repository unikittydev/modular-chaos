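; Ship component that signals when the owning BP_Ship's shield is depleted.
; On BeginPlay it binds to the ship shield's HP-zero event and caches the shield.
; The first zero-HP event on a shield with nonzero max HP activates the component and plays a depletion sound at the ship's location.
; A Depleted flag blocks repeats and is never cleared here.
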(event `self.ReceiveBeginPlay`
  (bind _asbp_ship (cast `/Game/Ships/BP_Ship` (`self.GetOwner`)))
  (bind _ship_shield (`/Game/Ships/BP_Ship.Ship Shield` _asbp_ship))
  (add `/Game/DamageSystem/Blueprints/BPC_DamageableLayer.On HP Zero` _ship_shield (delegate `On HP Zero`))
  (set `self.Shield` _ship_shield))

(event `On HP Zero`
  (if (and (> (`/Game/DamageSystem/Blueprints/BPC_DamageableLayer.Max HP` (`self.Shield`)) 0) (not (`self.Depleted`)))
    (`self.Activate` false)
    (set `self.Depleted` true)
    (`GameplayStatics.PlaySoundAtLocation` "/Game/Audio/Cues/SC_ShieldDepletion.SC_ShieldDepletion" (`Actor.K2_GetActorLocation` (`self.GetOwner`)) (struct) 1.0 1.0 0.0 null null null null)))