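; Ship module that propels and steers its ship, with tuning loaded from DT_ShipThrusterData by module name.
; While enabled it accumulates ship move input, then each Tick applies acceleration-based force and torque to the ship's collision box and clears the input.
; Standard controls move ship-relative and bank the model on yaw; SimpleControls moves on world axes and turns toward the aim location.
; Niagara spawn rate follows forward and strafe input.
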(event `self.Initialize`
  (params (Ship :type "/Game/Ships/BP_Ship Object Reference") (`Module Name` :type Name))
  (bind _ship (`self.Ship`))
  (`parent.Initialize` Ship `Module Name`)
  (bind _returnvalue (`|GetDataTableRow` "/Game/Ships/Modules/Thruster/DT_ShipThrusterData.DT_ShipThrusterData" `Module Name`)
    (:`then`
      (bind (_forwardspeed _rotatespeed _maxrollangle _rollspeed) (break `/Game/Ships/Modules/Thruster/BPS_ShipThrusterData` _returnvalue))
      (set `self.Forward Speed` _forwardspeed)
      (set `self.Rotate Speed` _rotatespeed)
      (set `self.Max Roll Angle` _maxrollangle)
      (set `self.Roll Speed` _rollspeed)
      (set `self.Model Target` (`/Game/Ships/BP_Ship.Model` _ship))
      (set `self.Force Target` (`/Game/Ships/BP_Ship.BoxCollision` _ship))
      (set `self.Simple Controls` (`/Game/Ships/BP_Ship.Simple Controls` (`self.Ship`))))))

(event `self.ReceiveBeginPlay`
  (`parent.ReceiveBeginPlay`))

(event `self.On Enable`
  (`parent.On Enable`)
  (add `/Game/Ships/BP_Ship.On Ship Move` (`self.Ship`) (delegate `On Ship Move`))
  (if (`self.Simple Controls`)
    (add `/Game/Ships/BP_Ship.On Set Aim` (`self.Ship`) (delegate `On Set Aim`))))

(event `self.On Disable`
  (`parent.On Disable`)
  (remove `/Game/Ships/BP_Ship.On Ship Move` (`self.Ship`) (delegate `On Ship Move`))
  (if (`self.Simple Controls`)
    (remove `/Game/Ships/BP_Ship.On Set Aim` (`self.Ship`) (delegate `On Set Aim`))))

(event `On Ship Move`
  (params (Forward :type "Float (double-precision)") (Strafe :type "Float (double-precision)") (Yaw :type "Float (double-precision)"))
  ;[1 1 1] Input
  (`|ExecutionSequence`
    (:`then_0`
      (set `self.Forward Input` (+ Forward (`self.Forward Input`))))
    (:`then_1`
      (set `self.Strafe Input` (+ Strafe (`self.Strafe Input`))))
    (:`then_2`
      (set `self.Yaw Input` (+ Yaw (`self.Yaw Input`))))))

(event `On Set Aim`
  (params (Target :type "Vector Structure"))
  (set `self.Aim Location` Target))

(event `self.ReceiveTick`
  (params (DeltaSeconds :type "Float (single-precision)"))
  (bind _forward_speed (`self.Forward Speed`))
  (bind _forward_input (`self.Forward Input`))
  (bind _force_target (`self.Force Target`))
  (bind _returnvalue (`SceneComponent.GetForwardVector` (`self.Force Target`)))
  (bind _returnvalue_2 (* (`self.Yaw Input`) (`self.Rotate Speed`)))
  (bind _returnvalue_roll (`KismetMathLibrary.BreakRotator` (`KismetMathLibrary.TransformRotation` (`SceneComponent.GetRelativeTransform` (`self.Model Target`)))))
  (`parent.ReceiveTick` DeltaSeconds)
  (`|ExecutionSequence`
    (:`then_0`
      (if (not (`self.Simple Controls`))
        (`|ExecutionSequence`
          (:`then_0`
            (`PrimitiveComponent.AddForce` (`self.Force Target`) (`KismetMathLibrary.GreaterGreater_VectorRotator` (`KismetMathLibrary.MakeVector` (* _forward_input _forward_speed 100.0) (* (`self.Strafe Input`) _forward_speed 50.0)) (`SceneComponent.K2_GetComponentRotation` (`self.Force Target`))) "None" true))
          (:`then_1`
            (`PrimitiveComponent.AddTorqueInRadians` (`self.Force Target`) (`KismetMathLibrary.MakeVector` 0.0 0.0 (`KismetMathLibrary.SelectFloat` (* _returnvalue_2 -1.0) _returnvalue_2 (< (`KismetMathLibrary.Dot_VectorVector` (* _forward_input _returnvalue) _returnvalue) 0.0))) "None" true))
          (:`then_2`
            (`SceneComponent.K2_SetRelativeRotation` (`self.Model Target`) (`KismetMathLibrary.MakeRotator` (`KismetMathLibrary.Lerp` _returnvalue_roll (* (`self.Yaw Input`) (`self.Max Roll Angle`)) (* (`self.Roll Speed`) DeltaSeconds))) false false)))
        (else
          (`PrimitiveComponent.AddForce` _force_target (`KismetMathLibrary.MakeVector` (* (`self.Forward Input`) (`self.Forward Speed`) 100.0) (* (`self.Yaw Input`) (`self.Forward Speed`) 100.0)) "None" true)
          (`PrimitiveComponent.AddTorqueInRadians` (`self.Force Target`) (`KismetMathLibrary.MakeVector` 0.0 0.0 (* (`KismetMathLibrary.Dot_VectorVector` (`SceneComponent.GetForwardVector` _force_target) (`KismetMathLibrary.Cross_VectorVector` (`KismetMathLibrary.Normal` (- (`self.Aim Location`) (`SceneComponent.K2_GetComponentLocation` _force_target))) (`SceneComponent.GetUpVector` _force_target))) (`self.Rotate Speed`))) "None" true))))
    (:`then_1`
      ;[1 1 1] Particles
      (`NiagaraComponent.SetVariableFloat` (`self.NS`) "SpawnRate" (* (`KismetMathLibrary.FClamp` (+ (`KismetMathLibrary.Abs` (`self.Forward Input`)) (`KismetMathLibrary.Abs` (`self.Strafe Input`)))) (`self.Max Particles`))))
    (:`then_2`
      (set `self.Forward Input` 0.0)
      (set `self.Strafe Input` 0.0)
      (set `self.Yaw Input` 0.0))))

(event `self.On Reset`
  (`parent.On Reset`)
  (`NiagaraComponent.SetVariableFloat` (`self.NS`) "SpawnRate" 0.0)
  (set `self.Forward Input` 0.0)
  (set `self.Strafe Input` 0.0)
  (set `self.Yaw Input` 0.0))

(fn `Get Power Points`
  (returns (Points :type Integer))
  (return (+ (`parent.Get Power Points`) (`KismetMathLibrary.FTrunc` (+ (* (`self.Forward Speed`) (`self.ForwardPower`)) (* (`self.Rotate Speed`) (`self.RotatePower`)))))))

(fn `Initialize Mesh`
  (params (Flipped :type Boolean))
  (bind _staticmesh (`self.StaticMesh`))
  (`parent.Initialize Mesh` Flipped)
  (`SceneComponent.K2_SetRelativeLocation` (`self.NS`) (`KismetMathLibrary.InverseTransformLocation` (`SceneComponent.K2_GetComponentToWorld` _staticmesh) (`SceneComponent.GetSocketLocation` _staticmesh "NS")) false false))

(fn `UserConstructionScript`
  (`parent.UserConstructionScript`))