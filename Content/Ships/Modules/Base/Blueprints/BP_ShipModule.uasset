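; Base actor for a ship module, configured from a data table row that supplies its mesh (optionally flipped), level and default HP.
; Dynamic materials show a level-colored stripe and track the owning ship's location, hull HP percentage and shield state via health events and Tick.
; When the hull reaches zero, the module detaches, scatters its primitives with physics and radial force, then runs a material cleanup timeline before destroying itself.
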(event `Initialize`
  (params (Ship :type "/Game/Ships/BP_Ship Object Reference") (`Module Name` :type Name))
  (bind _output_get (set `self.Ship` Ship))
  (bind _ship_hull (`/Game/Ships/BP_Ship.Ship Hull` _output_get))
  (add `/Game/DamageSystem/Blueprints/BPC_DamageableLayer.On HP Zero` _ship_hull (delegate `On Ship Destroyed`))
  (add `/Game/DamageSystem/Blueprints/BPC_DamageableLayer.On HP Changed` (`/Game/Ships/BP_Ship.Ship Shield` _output_get) (delegate `Shield HP Changed`))
  (add `/Game/DamageSystem/Blueprints/BPC_DamageableLayer.On HP Changed` _ship_hull (delegate `HP Changed`))
  (bind _returnvalue (`|GetDataTableRow` "/Game/Ships/Modules/Base/DT_ShipModuleData.DT_ShipModuleData" `Module Name`)
    (:`then`
      (set `self.Default HP` (`.DefaultHP_17_2391D150447816685E5DF3A586986081` (break `/Game/Ships/Modules/Base/Structures/BPS_ShipModuleData` _returnvalue)))
      (set `self.Module Name` `Module Name`)
      (set `self.Module Data` _returnvalue)
      (if (`/Game/Ships/BP_Ship.Is Enabled` (`self.Ship`))
        (`self.On Enable`)
        (else
          (`self.On Disable`)))
      (`self.Shield HP Changed` 0))))

(event `On Ship Destroyed`
  (bind _returnvalue (`self.K2_GetComponentsByClass` "/Script/Engine.PrimitiveComponent"))
  (`self.K2_DetachFromActor` "KeepWorld" "KeepWorld" "KeepWorld")
  (`self.SetActorTickEnabled` false)
  (for _array_element _returnvalue
    (`PrimitiveComponent.SetCollisionEnabled` _array_element "PhysicsOnly")
    (`PrimitiveComponent.SetSimulatePhysics` _array_element true)
    (`PrimitiveComponent.AddRadialForce` _array_element (+ (`self.K2_GetActorLocation` (`self.Ship`)) (* (`KismetMathLibrary.RandomUnitVector`) (`KismetMathLibrary.Conv_DoubleToVector` 250.0))) 1000.0 5000.0 "RIF_Linear" true))
  (`TimelineComponent.SetPlayRate` (`self.Cleanup Timeline`) (/ 1.0 (`self.Cleanup Time`)))
  (bind (_direction _track) (`Timeline|Cleanup Timeline` :!via `PlayFromStart`)
    (:`Update`
      (for _array_element_2 (`self.Materials`)
        (`MaterialInstanceDynamic.SetScalarParameterValue` _array_element_2 "CleanupTime" _track)))
    (:`Finished`
      (for _array_element_3 _returnvalue
        (`ActorComponent.K2_DestroyComponent` _array_element_3))
      (`self.K2_DestroyActor`))))

(event `Shield HP Changed`
  (params (`HP Delta` :type Integer))
  (for _array_element (`self.Materials`)
    (`MaterialInstanceDynamic.SetScalarParameterValue` _array_element "HasShield" (`KismetMathLibrary.SelectFloat` 1.0 0.0 (> (`/Game/DamageSystem/Blueprints/BPC_DamageableLayer.Current HP` (`/Game/Ships/BP_Ship.Ship Shield` (`self.Ship`))) 0)))))

(event `HP Changed`
  (params (`HP Delta` :type Integer))
  (bind _ship_hull (`/Game/Ships/BP_Ship.Ship Hull` (`self.Ship`)))
  (for _array_element (`self.Materials`)
    (`MaterialInstanceDynamic.SetScalarParameterValue` _array_element "HP_Percent" (/ (`KismetMathLibrary.Conv_IntToDouble` (`/Game/DamageSystem/Blueprints/BPC_DamageableLayer.Current HP` _ship_hull)) (`/Game/DamageSystem/Blueprints/BPC_DamageableLayer.Max HP` _ship_hull)))))

(event `self.ReceiveTick`
  (params (DeltaSeconds :type "Float (single-precision)"))
  (for _array_element (`self.Materials`)
    (`MaterialInstanceDynamic.SetVectorParameterValue` _array_element "ShipLocation" (`KismetMathLibrary.Conv_VectorToLinearColor` (`self.K2_GetActorLocation` (`self.Ship`))))
    (`MaterialInstanceDynamic.SetScalarParameterValue` _array_element "HasShield" (`KismetMathLibrary.SelectFloat` 1.0 0.0 (> (`/Game/DamageSystem/Blueprints/BPC_DamageableLayer.Current HP` (`/Game/Ships/BP_Ship.Ship Shield` (`self.Ship`))) 0)))))

(fn `Create and Setup MID`
  (params (Mesh :type "StaticMeshComponent Object Reference"))
  (for _array_element (`self.Materials`)
    (if (== (`MaterialInstance.Parent` _array_element) (`local.Mesh`))
      (`KismetArrayLibrary.Array_RemoveItem` (`self.Materials`) _array_element)))
  (for (_array_element_2 _array_index) (`MeshComponent.GetMaterials` (`local.Mesh`))
    (bind _returnvalue (`KismetMaterialLibrary.CreateDynamicMaterialInstance` _array_element_2))
    (`PrimitiveComponent.SetMaterial` (`local.Mesh`) _array_index _returnvalue)
    (`KismetArrayLibrary.Array_Add` (`self.Materials`) _returnvalue)
    (`MaterialInstanceDynamic.SetVectorParameterValue` _returnvalue "StripeColor" (`self.Get Level Color`))))

(fn `Get Level Color`
  (returns (Color :type "LinearColor Structure"))
  (return (select `/Game/Ships/Modules/Base/Enums/BPE_ShipModule_Level` (`.Level_43_38DDD1674FEF22A5C15F1E92DD85D2D7` (break `/Game/Ships/Modules/Base/Structures/BPS_ShipModuleData` (`self.Module Data`))) :`NewEnumerator0` (struct :`R` 0.870588 :`G` 0.870588 :`B` 0.870588 :`A` 1.0) :`NewEnumerator1` (struct :`R` 0.871367 :`G` 0.745404 :`B` 0.026241 :`A` 1.0) :`NewEnumerator2` (struct :`R` 0.871367 :`G` 0.026241 :`B` 0.026241 :`A` 1.0) :!type "LinearColor Structure")))

(fn `Get Power Points`
  (returns (Points :type Integer))
  (return (`KismetMathLibrary.FTrunc` (* (`self.HPPower`) (`self.Default HP`)))))

(fn `Initialize Mesh`
  (params (Flipped :type Boolean))
  (bind (_classreference _size _defaulthp _powerpoints _basemesh _flippedmesh) (break `/Game/Ships/Modules/Base/Structures/BPS_ShipModuleData` (`self.Module Data`)))
  (set `self.Is Flipped` Flipped)
  (bind _returnvalue (`KismetSystemLibrary.LoadAsset_Blocking` (select `bool` (and Flipped (`KismetSystemLibrary.IsValidSoftObjectReference` _flippedmesh)) :`false` _basemesh :`true` _flippedmesh)))
  (bind _asstatic_mesh (cast `StaticMesh` _returnvalue))
  (if (!= _asstatic_mesh (`StaticMeshComponent.StaticMesh` (`self.StaticMesh`)))
    (`StaticMeshComponent.SetStaticMesh` (`self.StaticMesh`) _asstatic_mesh)
    (`self.Create and Setup MID` (`self.StaticMesh`))))

(fn `On Disable`
  (`self.SetActorTickEnabled` false))

(fn `On Enable`
  (`self.SetActorTickEnabled` true))

(fn `On Reset`)

(fn `UserConstructionScript`)