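; Blueprint function library that builds display stats for a ship module as parallel arrays of Russian parameter labels and text values.
; GetShipModuleInfo reads base health from DT_ShipModuleData, then picks a thruster, weapon, shield or squadron helper by class reference and appends its results.
; Each helper reads its type's data table by the same row name, with weapon and squadron helpers deriving some values, such as damage per cycle or second.
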(fn `Get Ship Module Info`
  (params (`Module Name` :type Name))
  (returns (Parameters :type "Array of Text") (Values :type "Array of Text"))
  (locals (`Thruster Ref` :type "/Game/Ships/Modules/Base/Blueprints/BP_ShipModule Soft Class Reference" :default "/Game/Ships/Modules/Thruster/BP_ShipThruster.BP_ShipThruster_C") (`Weapon Ref` :type "/Game/Ships/Modules/Base/Blueprints/BP_ShipModule Soft Class Reference" :default "/Game/Ships/Modules/Weapons/Blueprints/BP_ShipWeapon_Particle.BP_ShipWeapon_Particle_C") (`Shield Ref` :type "/Game/Ships/Modules/Base/Blueprints/BP_ShipModule Soft Class Reference" :default "/Game/Ships/Modules/Shield/Blueprints/BP_ShipShield.BP_ShipShield_C") (`Squadron Ref` :type "/Game/Ships/Modules/Base/Blueprints/BP_ShipModule Soft Class Reference" :default "/Game/Ships/Modules/Squadron/BP_ShipWeapon_Squadron.BP_ShipWeapon_Squadron_C") (bParams :type "Array of Text") (bValues :type "Array of Text"))
  (bind _returnvalue (`|GetDataTableRow` "/Game/Ships/Modules/Base/DT_ShipModuleData.DT_ShipModuleData" `Module Name`)
    (:`then`
      (set `local.bParams` (`|MakeArray` "Здоровье" :!type "Text"))
      (bind (_classreference _size _defaulthp) (break `/Game/Ships/Modules/Base/Structures/BPS_ShipModuleData` _returnvalue))
      (set `local.bValues` (`|MakeArray` (`KismetTextLibrary.Conv_IntToText` _defaulthp)))
      (if (== _classreference (`local.Thruster Ref`))
        (bind (_parameters _values) (`self.Get Ship Thruster Info` (`local.Module Name`)))
        (`KismetArrayLibrary.Array_Append` (`local.bParams`) _parameters)
        (`KismetArrayLibrary.Array_Append` (`local.bValues`) _values)
        (elif (== _classreference (`local.Weapon Ref`))
          (bind (_parameters_2 _values_2) (`self.Get Ship Weapon Info` (`local.Module Name`)))
          (`KismetArrayLibrary.Array_Append` (`local.bParams`) _parameters_2)
          (`KismetArrayLibrary.Array_Append` (`local.bValues`) _values_2)
          (elif (== _classreference (`local.Shield Ref`))
            (bind (_parameters_3 _values_3) (`self.Get Ship Shield Info` (`local.Module Name`)))
            (`KismetArrayLibrary.Array_Append` (`local.bParams`) _parameters_3)
            (`KismetArrayLibrary.Array_Append` (`local.bValues`) _values_3)
            (elif (== _classreference (`local.Squadron Ref`))
              (bind (_parameters_4 _values_4) (`self.Get Ship Squadron Info` (`local.Module Name`)))
              (`KismetArrayLibrary.Array_Append` (`local.bParams`) _parameters_4)
              (`KismetArrayLibrary.Array_Append` (`local.bValues`) _values_4)))))
      (return (`local.bParams`) (`local.bValues`)))))

(fn `Get Ship Shield Info`
  (params (`Module Name` :type Name))
  (returns (Parameters :type "Array of Text") (Values :type "Array of Text"))
  (bind _returnvalue (`|GetDataTableRow` "/Game/Ships/Modules/Shield/DT_ShipShieldData.DT_ShipShieldData" `Module Name`)
    (:`then`
      (bind (_shieldhp _rechargerate) (break `/Game/Ships/Modules/Shield/BPS_ShipShieldData` _returnvalue))
      (return (`|MakeArray` "Здоровье щита" "Скорость зарядки" :!type "Text") (`|MakeArray` (`KismetTextLibrary.Conv_IntToText` _shieldhp) (`KismetTextLibrary.Conv_IntToText` _rechargerate))))))

(fn `Get Ship Squadron Info`
  (params (`Module Name` :type Name))
  (returns (Parameters :type "Array of Text") (Values :type "Array of Text"))
  (bind _returnvalue (`|GetDataTableRow` "/Game/Ships/Modules/Squadron/DT_ShipSquadronData.DT_ShipSquadronData" `Module Name`)
    (:`then`
      (bind (_shuttlecount _flightduration _flightdelay _bulletspeed _flightradius _shuttlespeed _damage) (break `/Game/Ships/Modules/Squadron/Structures/BPS_Squadron_Functional` (`.Functional_2_D10660AF441613E17008649A3FB56729` (break `/Game/Ships/Modules/Squadron/Structures/BPS_Squadron` _returnvalue))))
      (return (`|MakeArray` "Урон в секунду" "Время полёта" "Время перезарядки" "Скорость снарядов" "Радиус стрельбы" :!type "Text") (`|MakeArray` (`KismetTextLibrary.Conv_IntToText` (* (`.DamagePoints_2_FDD4BB764CC37523C51825A835A7C714` (break `/Game/DamageSystem/Structures/BPS_Damage` _damage)) _shuttlecount 10)) (`KismetTextLibrary.Conv_DoubleToText` _flightduration "HalfToEven" false true 1 324 0 0) (`KismetTextLibrary.Conv_DoubleToText` _flightdelay "HalfToEven" false true 1 324 0 0) (`KismetTextLibrary.Conv_DoubleToText` _bulletspeed "HalfToEven" false true 1 324 0 0) (`KismetTextLibrary.Conv_DoubleToText` _flightradius "HalfToEven" false true 1 324 0 0))))))

(fn `Get Ship Thruster Info`
  (params (`Module Name` :type Name))
  (returns (Parameters :type "Array of Text") (Values :type "Array of Text"))
  (bind _returnvalue (`|GetDataTableRow` "/Game/Ships/Modules/Thruster/DT_ShipThrusterData.DT_ShipThrusterData" `Module Name`)
    (:`then`
      (bind (_forwardspeed _rotatespeed) (break `/Game/Ships/Modules/Thruster/BPS_ShipThrusterData` _returnvalue))
      (return (`|MakeArray` "Мощность" "Поворот" :!type "Text") (`|MakeArray` (`KismetTextLibrary.Conv_DoubleToText` _forwardspeed "HalfToEven" false true 1 324 0 0) (`KismetTextLibrary.Conv_DoubleToText` _rotatespeed "HalfToEven" false true 1 324 0 0))))))

(fn `Get Ship Weapon Info`
  (params (`Module Name` :type Name))
  (returns (Parameters :type "Array of Text") (Values :type "Array of Text"))
  (bind _returnvalue (`|GetDataTableRow` "/Game/Ships/Modules/Weapons/DT_ShipWeaponData.DT_ShipWeaponData" `Module Name`)
    (:`then`
      (bind (_particlecount _particlereload _magazinereload _projectilespeed _projectiledistance _randomangleoffset _coneangle _weapontype _damage) (break `/Game/Ships/Modules/Weapons/Structures/BPS_Weapon_Functional` (`.Functional_2_A277E6CF452FA85C2D4DA59396CD4F28` (break `/Game/Ships/Modules/Weapons/Structures/BPS_Weapon` _returnvalue))))
      (return (`|MakeArray` "Урон за цикл" "Снарядов за цикл" "Время перезарядки" "Скорость снарядов" "Дальность снарядов" :!type "Text") (`|MakeArray` (`KismetTextLibrary.Conv_IntToText` (* (`.DamagePoints_2_FDD4BB764CC37523C51825A835A7C714` (break `/Game/DamageSystem/Structures/BPS_Damage` _damage)) _particlecount)) (`KismetTextLibrary.Conv_IntToText` _particlecount) (`KismetTextLibrary.Conv_DoubleToText` (`KismetMathLibrary.SelectFloat` _particlereload _magazinereload (== 0.0 _magazinereload)) "HalfToEven" false true 1 324 0 2) (`KismetTextLibrary.Conv_DoubleToText` _projectilespeed "HalfToEven" false true 1 324 0 0) (`KismetTextLibrary.Conv_DoubleToText` _projectiledistance "HalfToEven" false true 1 324 0 0))))))