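; BP_ShipDrive is a ship module that turns the ship's physical movement into movement through celestial coordinate space.
; On initialization it caches the level's BP_JumpSystem and loads speed settings from DT_ShipDriveData by module name.
; Each tick it reads the collision box's velocity as a fraction of MaxVelocity, then advances the CelestialBody's local coordinates at AUSpeed and world coordinates at LightSpeed along that direction.
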(event `self.Initialize`
  (params (Ship :type "/Game/Ships/BP_Ship Object Reference") (`Module Name` :type Name))
  (`parent.Initialize` Ship `Module Name`)
  (bind _returnvalue (`GameplayStatics.GetActorOfClass` "/Game/CelestialSystem/Blueprints/Unused/BP_JumpSystem.BP_JumpSystem_C"))
  (set `self.JumpSystem` _returnvalue)
  (bind _returnvalue_2 (`|GetDataTableRow` "/Game/Ships/Modules/Drive/DT_ShipDriveData.DT_ShipDriveData" `Module Name`)
    (:`then`
      (bind (_auspeed _maxvelocity _lightspeed) (break `/Game/Ships/Modules/Drive/BPS_ShipDriveData` _returnvalue_2))
      (set `self.AU Speed` _auspeed)
      (set `self.Max Velocity` _maxvelocity)
      (set `self.Light Speed` _lightspeed))))

(event `self.ReceiveTick`
  (params (DeltaSeconds :type "Float (single-precision)"))
  (bind _celestial_body (`/Game/Ships/BP_Ship.Celestial Body` (`self.Ship`)))
  (bind _returnvalue (`PrimitiveComponent.GetPhysicsLinearVelocity` (`/Game/Ships/BP_Ship.BoxCollision` (`self.Ship`)) "None"))
  (bind _returnvalue_2 (/ (`KismetMathLibrary.VSize` _returnvalue) (`self.Max Velocity`)))
  (bind _returnvalue_3 (`KismetMathLibrary.Normal` _returnvalue 1e-05))
  (set `/Game/CelestialSystem/Blueprints/BPC_CelestialBody.Local Coordinates` (+ (`/Game/CelestialSystem/Blueprints/BPC_CelestialBody.Local Coordinates` _celestial_body) (* (* _returnvalue_2 DeltaSeconds (`self.AU Speed`)) _returnvalue_3)) _celestial_body)
  (set `/Game/CelestialSystem/Blueprints/BPC_CelestialBody.World Coordinates` (+ (`/Game/CelestialSystem/Blueprints/BPC_CelestialBody.World Coordinates` _celestial_body) (* _returnvalue_3 (* _returnvalue_2 DeltaSeconds (`self.Light Speed`)))) _celestial_body))

(fn `UserConstructionScript`
  (`parent.UserConstructionScript`))