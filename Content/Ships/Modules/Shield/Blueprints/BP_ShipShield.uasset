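; BP_ShipShield is a ship module that adds shield capacity and regeneration to the ship it is installed on.
; On Initialize it looks up its row in DT_ShipShieldData by module name, adds the shield HP and recharge rate to the ship's values, and fills the shield.
; On Destroyed it subtracts those bonuses and resets current shield HP to the new maximum.
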(event `self.Initialize`
  (params (Ship :type "/Game/Ships/BP_Ship Object Reference") (`Module Name` :type Name))
  (bind _ship (`self.Ship`))
  (bind _ship_shield (`/Game/Ships/BP_Ship.Ship Shield` _ship))
  (bind _shield_regen (`/Game/Ships/BP_Ship.Shield Regen` _ship))
  (`KismetSystemLibrary.PrintString` "before parent init")
  (`parent.Initialize` Ship `Module Name`)
  (`KismetSystemLibrary.PrintString` "after parent init")
  (bind _returnvalue (`|GetDataTableRow` "/Game/Ships/Modules/Shield/DT_ShipShieldData.DT_ShipShieldData" `Module Name`)
    (:`then`
      (bind _output_get (set `self.Data` _returnvalue))
      (bind (_shieldhp _rechargerate) (break `/Game/Ships/Modules/Shield/BPS_ShipShieldData` _output_get))
      (bind _output_get_2 (set `/Game/DamageSystem/Blueprints/BPC_DamageableLayer.Max HP` (+ _shieldhp (`/Game/DamageSystem/Blueprints/BPC_DamageableLayer.Max HP` _ship_shield)) _ship_shield))
      (set `/Game/DamageSystem/Blueprints/BPC_DamageableLayer.Current HP` _output_get_2 _ship_shield)
      (set `/Game/DamageSystem/Blueprints/BPC_Regeneration.Strength` (+ _rechargerate (`/Game/DamageSystem/Blueprints/BPC_Regeneration.Strength` _shield_regen)) _shield_regen)
      (`KismetSystemLibrary.PrintString` "shield setup"))
    (:`RowNotFound`
      (`KismetSystemLibrary.PrintString` (`KismetStringLibrary.Concat_StrStr` "shield not found " (`KismetStringLibrary.Conv_NameToString` `Module Name`))))))

(event `self.ReceiveDestroyed`
  (bind _ship (`self.Ship`))
  (bind (_shieldhp _rechargerate) (break `/Game/Ships/Modules/Shield/BPS_ShipShieldData` (`self.Data`)))
  (bind _ship_shield (`/Game/Ships/BP_Ship.Ship Shield` _ship))
  (bind _shield_regen (`/Game/Ships/BP_Ship.Shield Regen` _ship))
  (`parent.ReceiveDestroyed`)
  (bind _output_get (set `/Game/DamageSystem/Blueprints/BPC_DamageableLayer.Max HP` (- (`/Game/DamageSystem/Blueprints/BPC_DamageableLayer.Max HP` _ship_shield) _shieldhp) _ship_shield))
  (set `/Game/DamageSystem/Blueprints/BPC_DamageableLayer.Current HP` _output_get _ship_shield)
  (set `/Game/DamageSystem/Blueprints/BPC_Regeneration.Strength` (- (`/Game/DamageSystem/Blueprints/BPC_Regeneration.Strength` _shield_regen) _rechargerate) _shield_regen))

(fn `UserConstructionScript`
  (`parent.UserConstructionScript`))