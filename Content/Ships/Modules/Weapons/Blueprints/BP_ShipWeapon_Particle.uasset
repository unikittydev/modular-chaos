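; Ship weapon module that fires projectiles as Niagara particles from a yaw-limited, speed-limited turret.
; DT_ShipWeaponData configures the gun, effect, damage and timing, including Rate or Burst fire.
; Ship events drive aim and firing; Tick handles reload and triggers spawning and sound when a shot is ready.
; Exported particle data returns to the Blueprint, which either stops spawning or sphere-overlaps particle positions to damage other actors' BPC_DamageableManager.
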(event `self.Initialize`
  (params (Ship :type "/Game/Ships/BP_Ship Object Reference") (`Module Name` :type Name))
  (`parent.Initialize` Ship `Module Name`)
  (`self.Setup Particle System` `Module Name`))

(event `self.On Enable`
  (bind _ship (`self.Ship`))
  (`parent.On Enable`)
  (add `/Game/Ships/BP_Ship.On Set Aim` _ship (delegate `On Aim`))
  (add `/Game/Ships/BP_Ship.On Ship Fire Start` _ship (delegate `Start Fire`))
  (add `/Game/Ships/BP_Ship.On Ship Fire Stop` _ship (delegate `Stop Fire`))
  (add `/Game/Ships/BP_Ship.On Fire If In Range` _ship (delegate `Fire If In Range`)))

(event `self.On Disable`
  (bind _ship (`self.Ship`))
  (`parent.On Disable`)
  (remove `/Game/Ships/BP_Ship.On Set Aim` _ship (delegate `On Aim`))
  (remove `/Game/Ships/BP_Ship.On Ship Fire Start` _ship (delegate `Start Fire`))
  (remove `/Game/Ships/BP_Ship.On Ship Fire Stop` _ship (delegate `Stop Fire`))
  (remove `/Game/Ships/BP_Ship.On Fire If In Range` _ship (delegate `Fire If In Range`))
  (`self.Stop Fire`)
  (`NiagaraComponent.SetVariableBool` (`self.NS`) "SpawnProjectiles" false))

(event `On Aim`
  (params (Target :type "Vector Structure"))
  (set `self.Aim Location` Target))

(event `self.ReceiveTick`
  (params (DeltaSeconds :type "Float (single-precision)"))
  (`parent.ReceiveTick` DeltaSeconds)
  (`self.Aim` (`self.Aim Location`) DeltaSeconds)
  (`self.Try Reload` DeltaSeconds)
  (bind _can_fire (`self.Can Fire`))
  (if _can_fire
    (`NiagaraComponent.SetVariableBool` (`self.NS`) "SpawnProjectiles" true)
    (`self.Consume Particles`)
    (`GameplayStatics.PlaySoundAtLocation` (`.Sound_22_8809FD4F430321C8AF6E7B86FECD38D1` (break `/Game/Ships/Modules/Weapons/Structures/BPS_Weapon` (`self.Data`))) (`self.K2_GetActorLocation`) (struct) 1.0 1.0 0.0 null null null null)))

(event `self.On Reset`
  (`parent.On Reset`)
  (`self.Stop Fire`)
  (`self.Reset Aim`))

(event `Start Fire`
  (set `self.Is Firing` true))

(event `Stop Fire`
  (set `self.Is Firing` false))

(event `Fire If In Range`
  (bind __ (`self.Location in Fire Range` (`self.Aim Location`)))
  (if __
    (`self.Start Fire`)
    (else
      (`self.Stop Fire`))))

(event `self.ReceiveParticleData`
  (params (Data :type "Array of BasicParticleData Structure (by ref)") (NiagaraSystem :type "NiagaraSystem Object Reference") (SimulationPositionOffset :type "Vector Structure (by ref)"))
  (bind _data_functional (break `/Game/Ships/Modules/Weapons/Structures/BPS_Weapon` (`self.Data`)))
  (for _array_element Data
    (if (> (`.Size` (break `BasicParticleData` _array_element)) 0.5)
      (`NiagaraComponent.SetVariableBool` (`self.NS`) "SpawnProjectiles" false)
      (break)
      (else
        (bind (_outactors _returnvalue) (`KismetSystemLibrary.SphereOverlapActors` (break `BasicParticleData` _array_element) 10.0 (`|MakeArray` "ObjectTypeQuery2" "ObjectTypeQuery3" :!type "EObjectTypeQuery Enum")))
        (if _returnvalue
          (for _array_element_2 _outactors
            (if (!= _array_element_2 (`self.Ship`))
              (bind _returnvalue_2 (`self.GetComponentByClass` _array_element_2 "/Game/DamageSystem/Blueprints/BPC_DamageableManager.BPC_DamageableManager_C"))
              (`/Engine/EditorBlueprintResources/StandardMacros.IsValid` _returnvalue_2
                (:`Is Valid`
                  (`/Game/DamageSystem/Blueprints/BPC_DamageableManager.On Take Damage` _returnvalue_2 (`.Damage_28_62C9FD1C4D7C5AA204996FAEE7F58DDA` (break `/Game/Ships/Modules/Weapons/Structures/BPS_Weapon_Functional` _data_functional))))))))))))

(event `self.K2_OnReset`
  (bind _data_functional (break `/Game/Ships/Modules/Weapons/Structures/BPS_Weapon` (`self.Data`)))
  (set `self.Magazine Reload Counter` 0.0)
  (set `self.Particle Reload Counter` 0.0)
  (set `self.Particles In Magazine` (`.ParticleCount_5_4C5B2F744B5C04A28DB3CE9B6F313E69` (break `/Game/Ships/Modules/Weapons/Structures/BPS_Weapon_Functional` _data_functional))))

(fn `Aim`
  (params (`Target Location` :type "Vector Structure") (`Delta Seconds` :type "Float (double-precision)"))
  (bind _returnvalue (`KismetMathLibrary.MakeVector` `Target Location_X` `Target Location_Y`))
  (bind (_data_functional _data_appearance _data_gunmesh _data_weaponangle) (break `/Game/Ships/Modules/Weapons/Structures/BPS_Weapon` (`self.Data`)))
  (bind (_data_functional_2 _data_appearance_2 _data_gunmesh_2 _data_weaponangle_2 _data_aimspeed) (break `/Game/Ships/Modules/Weapons/Structures/BPS_Weapon` (`self.Data`)))
  (bind _tower (`self.Tower`))
  (bind _returnvalue_2 (* `Delta Seconds` _data_aimspeed))
  (bind (_relativerotation_roll _relativerotation_pitch _relativerotation_yaw) (`KismetMathLibrary.BreakRotator` (`SceneComponent.RelativeRotation` _tower)))
  (bind (_returnvalue_roll _returnvalue_pitch _returnvalue_yaw) (`KismetMathLibrary.BreakRotator` (`KismetMathLibrary.InverseTransformRotation` (`KismetMathLibrary.ComposeTransforms` (`self.GetTransform`) (`SceneComponent.GetRelativeTransform` (`/Game/Ships/BP_Ship.Model` (`self.Ship`)))) (`KismetMathLibrary.FindLookAtRotation` (`SceneComponent.K2_GetComponentLocation` _tower) _returnvalue))))
  (bind _returnvalue_3 (- _returnvalue_yaw _relativerotation_yaw))
  (bind _returnvalue_4 (`KismetMathLibrary.SelectFloat` (+ _returnvalue_3 360.0) _returnvalue_3 (< _returnvalue_3 -180.0)))
  (set `self.Target Ahead Weapon` (< (`KismetMathLibrary.Dot_VectorVector` (- (`SceneComponent.K2_GetComponentLocation` (`self.Tower`)) _returnvalue) (`SceneComponent.GetForwardVector` (`self.Tower`))) 0.0))
  (`SceneComponent.K2_SetRelativeRotation` (`self.Tower`) (`KismetMathLibrary.MakeRotator` 0.0 0.0 (`KismetMathLibrary.FClamp` (+ _relativerotation_yaw (`KismetMathLibrary.FClamp` (`KismetMathLibrary.SelectFloat` (- _returnvalue_4 360.0) _returnvalue_4 (> _returnvalue_4 180.0)) (- 0.0 _returnvalue_2) _returnvalue_2)) (* _data_weaponangle -0.5) (* _data_weaponangle 0.5))) false false))

(fn `Apply Sockets`
  (locals (`Old Tower Location` :type "Vector Structure"))
  (bind _gun (`self.Gun`))
  (bind _gun_2 (`self.Gun`))
  (`SceneComponent.K2_SetWorldLocationAndRotation` (`self.Tower`) (`SceneComponent.GetSocketLocation` (`self.StaticMesh`) "Gun") (`self.K2_GetActorRotation`) false true)
  (`SceneComponent.K2_SetRelativeLocation` (`self.Gun`) (- (0.0 0.0 0.0) (`KismetMathLibrary.InverseTransformLocation` (`SceneComponent.K2_GetComponentToWorld` _gun_2) (`SceneComponent.GetSocketLocation` _gun_2 "Gun"))) false false)
  ;[1 1 1] Adjust NS to socket
  (`SceneComponent.K2_SetWorldLocationAndRotation` (`self.NS`) (`SceneComponent.GetSocketLocation` _gun "NS") (`SceneComponent.K2_GetComponentRotation` _gun) false true))

(fn `Can Fire`
  (returns (`Can Fire` :type Boolean))
  (return (and (<= (`self.Particle Reload Counter`) 0.0) (> (`self.Particles In Magazine`) 0) (`self.Is Firing`))))

(fn `Consume Particles`
  (bind _data_functional (break `/Game/Ships/Modules/Weapons/Structures/BPS_Weapon` (`self.Data`)))
  (bind _data_functional_2 (break `/Game/Ships/Modules/Weapons/Structures/BPS_Weapon` (`self.Data`)))
  (bind (_particlecount _particlereload _magazinereload _projectilespeed _projectiledistance _randomangleoffset _coneangle _weapontype) (break `/Game/Ships/Modules/Weapons/Structures/BPS_Weapon_Functional` _data_functional))
  (bind (_particlecount_2 _particlereload_2 _magazinereload_2) (break `/Game/Ships/Modules/Weapons/Structures/BPS_Weapon_Functional` _data_functional_2))
  (bind _output_get (set `self.Particles In Magazine` (- (`self.Particles In Magazine`) (select `/Game/Ships/Modules/Weapons/Enums/BPE_WeaponType` _weapontype :`NewEnumerator0` 1 :`NewEnumerator1` _particlecount))))
  (set `self.Particle Reload Counter` _particlereload_2)
  (if (<= _output_get 0)
    (set `self.Magazine Reload Counter` _magazinereload_2))
  (return))

(fn `Get Power Points`
  (returns (Points :type Integer))
  (bind _data_functional (break `/Game/Ships/Modules/Weapons/Structures/BPS_Weapon` (`self.Data`)))
  (bind (_particlecount _particlereload _magazinereload _projectilespeed _projectiledistance _randomangleoffset _coneangle _weapontype _damage) (break `/Game/Ships/Modules/Weapons/Structures/BPS_Weapon_Functional` _data_functional))
  (return (+ (`parent.Get Power Points`) (`KismetMathLibrary.FTrunc` (/ (* _particlecount (`.DamagePoints_2_FDD4BB764CC37523C51825A835A7C714` (break `/Game/DamageSystem/Structures/BPS_Damage` _damage)) (`self.DamagePower`)) _particlereload)))))

(fn `Initialize Mesh`
  (params (Flipped :type Boolean))
  (`parent.Initialize Mesh` Flipped)
  (bind _returnvalue (`KismetSystemLibrary.LoadAsset_Blocking` (`.GunMesh_18_319454504297D64AA08502812954D867` (break `/Game/Ships/Modules/Weapons/Structures/BPS_Weapon` (`self.Data`)))))
  (bind _asstatic_mesh (cast `StaticMesh` _returnvalue))
  (`StaticMeshComponent.SetStaticMesh` (`self.Gun`) _asstatic_mesh)
  (`self.Create and Setup MID` (`self.Gun`))
  (`self.Apply Sockets`))

(fn `Location in Fire Range`
  (params (Location :type "Vector Structure"))
  (returns (_ :type Boolean))
  (bind _tower (`self.Tower`))
  (bind _data_functional (break `/Game/Ships/Modules/Weapons/Structures/BPS_Weapon` (`self.Data`)))
  (bind (_data_functional_2 _data_appearance _data_gunmesh _data_weaponangle) (break `/Game/Ships/Modules/Weapons/Structures/BPS_Weapon` (`self.Data`)))
  (bind (_returnvalue_x _returnvalue_y) (`KismetMathLibrary.BreakVector` (`SceneComponent.GetForwardVector` _tower)))
  (bind (_returnvalue_x_2 _returnvalue_y_2) (`KismetMathLibrary.BreakVector` (`SceneComponent.K2_GetComponentLocation` _tower)))
  (bind _returnvalue (- (`KismetMathLibrary.MakeVector` (.x Location) (.y Location)) (`KismetMathLibrary.MakeVector` _returnvalue_x_2 _returnvalue_y_2)))
  (return (and (< (`KismetMathLibrary.VSize` _returnvalue) (`.ProjectileDistance_14_14B0A19041DA40553ADC908D2DE9A35A` (break `/Game/Ships/Modules/Weapons/Structures/BPS_Weapon_Functional` _data_functional))) (< (`KismetMathLibrary.DegAcos` (`KismetMathLibrary.Dot_VectorVector` (`KismetMathLibrary.Normal` _returnvalue) (`KismetMathLibrary.Normal` (`KismetMathLibrary.MakeVector` _returnvalue_x _returnvalue_y)))) (* _data_weaponangle 0.5)))))

(fn `Reset Aim`
  (`SceneComponent.K2_SetRelativeRotation` :`self` (`self.Tower`)))

(fn `Setup Particle System`
  (params (`Module Name` :type Name))
  (bind (_data_functional _data_appearance) (break `/Game/Ships/Modules/Weapons/Structures/BPS_Weapon` (`self.Data`)))
  (bind (_data_functional_2 _data_appearance_2) (break `/Game/Ships/Modules/Weapons/Structures/BPS_Weapon` (`self.Data`)))
  (bind (_data_functional_3 _data_appearance_3) (break `/Game/Ships/Modules/Weapons/Structures/BPS_Weapon` (`self.Data`)))
  (bind _data_functional_4 (break `/Game/Ships/Modules/Weapons/Structures/BPS_Weapon` (`self.Data`)))
  (bind _data_functional_5 (break `/Game/Ships/Modules/Weapons/Structures/BPS_Weapon` (`self.Data`)))
  (bind _data_functional_6 (break `/Game/Ships/Modules/Weapons/Structures/BPS_Weapon` (`self.Data`)))
  (bind (_projectilecolor _trailcolor _deathcolor _projectilesize) (break `/Game/Ships/Modules/Weapons/Structures/BPS_Weapon_Appearance` _data_appearance))
  (bind (_projectilecolor_2 _trailcolor_2 _deathcolor_2 _projectilesize_2 _trailsize _deathsize _trailduration) (break `/Game/Ships/Modules/Weapons/Structures/BPS_Weapon_Appearance` _data_appearance_2))
  (bind (_projectilecolor_3 _trailcolor_3 _deathcolor_3 _projectilesize_3 _trailsize_2 _deathsize_2 _trailduration_2 _deathduration) (break `/Game/Ships/Modules/Weapons/Structures/BPS_Weapon_Appearance` _data_appearance_3))
  (bind (_particlecount _particlereload _magazinereload _projectilespeed _projectiledistance _randomangleoffset _coneangle _weapontype) (break `/Game/Ships/Modules/Weapons/Structures/BPS_Weapon_Functional` _data_functional_4))
  (bind (_particlecount_2 _particlereload_2 _magazinereload_2 _projectilespeed_2 _projectiledistance_2) (break `/Game/Ships/Modules/Weapons/Structures/BPS_Weapon_Functional` _data_functional_5))
  (bind (_particlecount_3 _particlereload_3 _magazinereload_3 _projectilespeed_3 _projectiledistance_3 _randomangleoffset_2 _coneangle_2) (break `/Game/Ships/Modules/Weapons/Structures/BPS_Weapon_Functional` _data_functional_6))
  (bind _returnvalue (`|GetDataTableRow` "/Game/Ships/Modules/Weapons/DT_ShipWeaponData.DT_ShipWeaponData" `Module Name`)
    (:`then`
      (bind (_functional _appearance _gunmesh _weaponangle _aimspeed _sound) (break `/Game/Ships/Modules/Weapons/Structures/BPS_Weapon` _returnvalue))
      (bind (_particlecount_4 _particlereload_4 _magazinereload_4 _projectilespeed_4 _projectiledistance_4 _randomangleoffset_3 _coneangle_3 _weapontype_2 _damage) (break `/Game/Ships/Modules/Weapons/Structures/BPS_Weapon_Functional` _functional))
      (set `self.Data` (select `bool` (== _magazinereload_4 0.0) :`false` _returnvalue :`true` (make `/Game/Ships/Modules/Weapons/Structures/BPS_Weapon` (make `/Game/Ships/Modules/Weapons/Structures/BPS_Weapon_Functional` 1 0.0 _particlereload_4 _projectilespeed_4 _projectiledistance_4 _randomangleoffset_3 _coneangle_3 _weapontype_2 _damage) _appearance _gunmesh _weaponangle _aimspeed _sound)))
      (`|ExecutionSequence`
        (:`then_0`
          ;[1 1 1] Particle Count
          (`NiagaraComponent.SetVariableInt` (`self.NS`) "ParticleCount" (select `/Game/Ships/Modules/Weapons/Enums/BPE_WeaponType` _weapontype :`NewEnumerator0` 1 :`NewEnumerator1` _particlecount))
          ;[1 1 1] Reach
          (`NiagaraComponent.SetVariableFloat` (`self.NS`) "ProjectileSpeed" _projectilespeed_2)
          ;[1 1 1] Angle
          (`NiagaraComponent.SetVariableFloat` (`self.NS`) "RandomAngleOffset" _randomangleoffset_2))
        (:`then_1`
          (`NiagaraComponent.SetVariableFloat` (`self.NS`) "ProjectileDistance" _projectiledistance_2)
          (`NiagaraComponent.SetVariableFloat` (`self.NS`) "ConeAngle" _coneangle_2))
        (:`then_2`
          (`|ExecutionSequence`
            (:`then_0`
              ;[1 1 1] Main Projectile
              (`NiagaraComponent.SetVariableLinearColor` (`self.NS`) "ProjectileColor" _projectilecolor)
              ;[1 1 1] Trail
              (`NiagaraComponent.SetVariableLinearColor` (`self.NS`) "TrailColor" _trailcolor_2)
              ;[1 1 1] Death
              (`NiagaraComponent.SetVariableLinearColor` (`self.NS`) "DeathColor" _deathcolor_3))
            (:`then_1`
              (`NiagaraComponent.SetVariableFloat` (`self.NS`) "ProjectileSize" _projectilesize)
              (`NiagaraComponent.SetVariableFloat` (`self.NS`) "TrailSize" _trailsize)
              (`NiagaraComponent.SetVariableFloat` (`self.NS`) "DeathSize" _deathsize_2))
            (:`then_2`
              (`NiagaraComponent.SetVariableFloat` (`self.NS`) "TrailDuration" _trailduration)
              (`NiagaraComponent.SetVariableFloat` (`self.NS`) "DeathDuration" _deathduration))
            (:`then_3`
              (`NiagaraComponent.SetVariableObject` (`self.NS`) "BPTarget" self)
              (`NiagaraComponent.SetVariableBool` (`self.NS`) "SpawnProjectiles" false)
              (`NiagaraComponent.SetVariableFloat` (`self.NS`) "ResetLoopDuration" 0.0))))))))

(fn `Try Reload`
  (params (`Delta Time` :type "Float (double-precision)"))
  (bind _data_functional (break `/Game/Ships/Modules/Weapons/Structures/BPS_Weapon` (`self.Data`)))
  (set `self.Particle Reload Counter` (- (`self.Particle Reload Counter`) `Delta Time`))
  (if (== (`self.Particles In Magazine`) 0)
    (bind _output_get (set `self.Magazine Reload Counter` (- (`self.Magazine Reload Counter`) `Delta Time`)))
    (if (<= _output_get 0.0)
      (set `self.Particles In Magazine` (`.ParticleCount_5_4C5B2F744B5C04A28DB3CE9B6F313E69` (break `/Game/Ships/Modules/Weapons/Structures/BPS_Weapon_Functional` _data_functional)))
      (return))
    (else
      (return))))

(fn `UserConstructionScript`
  (`parent.UserConstructionScript`))