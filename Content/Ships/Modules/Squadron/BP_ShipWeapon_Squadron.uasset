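; Squadron ship weapon module that simulates a swarm of attacking shuttles as a Niagara effect, configured by row from DT_ShipSquadronData.
; A sphere tracks nearby ships, and Tick picks a target from them to drive the effect's spawn flag and aim point.
; Niagara exports particle positions back to the Blueprint, where small sphere overlaps apply damage through BPC_DamageableManager.
; Fire handlers are empty, and power points scale with shuttle count, flight duration and damage.
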(event `self.Initialize`
  (params (Ship :type "/Game/Ships/BP_Ship Object Reference") (`Module Name` :type Name))
  (`parent.Initialize` Ship `Module Name`)
  (`self.Setup Particle System` `Module Name`))

(event `self.On Enable`
  (bind _ship (`self.Ship`))
  (`parent.On Enable`)
  (add `/Game/Ships/BP_Ship.On Set Aim` _ship (delegate `On Aim`))
  (add `/Game/Ships/BP_Ship.On Fire If In Range` _ship (delegate `On Fire If In Range`)))

(event `self.On Disable`
  (`parent.On Disable`)
  (remove `/Game/Ships/BP_Ship.On Set Aim` (`self.Ship`) (delegate `On Aim`)))

(event `On Aim`
  (params (Target :type "Vector Structure"))
  (set `self.Aim Location` Target)
  (`self.Aim`))

(event `On Fire If In Range`)

(event `Start Fire`)

(event `Stop Fire`)

(event `self.ReceiveParticleData`
  (params (Data :type "Array of BasicParticleData Structure (by ref)") (NiagaraSystem :type "NiagaraSystem Object Reference") (SimulationPositionOffset :type "Vector Structure (by ref)"))
  (bind _data_functional (break `/Game/Ships/Modules/Squadron/Structures/BPS_Squadron` (`self.Data`)))
  (for _array_element Data
    (bind (_outactors _returnvalue) (`KismetSystemLibrary.SphereOverlapActors` (break `BasicParticleData` _array_element) 10.0 (`|MakeArray` "ObjectTypeQuery2" "ObjectTypeQuery3" :!type "EObjectTypeQuery Enum")))
    (if _returnvalue
      (for _array_element_2 _outactors
        (bind _returnvalue_2 (`self.GetComponentByClass` _array_element_2 "/Game/DamageSystem/Blueprints/BPC_DamageableManager.BPC_DamageableManager_C"))
        (`/Engine/EditorBlueprintResources/StandardMacros.IsValid` _returnvalue_2
          (:`Is Valid`
            (`/Game/DamageSystem/Blueprints/BPC_DamageableManager.On Take Damage` _returnvalue_2 (`.Damage_16_55329CB547F36C9D5FB47695905A8692` (break `/Game/Ships/Modules/Squadron/Structures/BPS_Squadron_Functional` _data_functional)))))))))

(event `self.ReceiveTick`
  (params (DeltaSeconds :type "Float (single-precision)"))
  (bind _closest_actor (`self.Find Closest Actor`))
  (bind _returnvalue (and (`KismetSystemLibrary.IsValid` _closest_actor) (!= _closest_actor (`self.Ship`))))
  (`NiagaraComponent.SetVariableBool` (`self.NS`) "Spawn" _returnvalue)
  (if _returnvalue
    (`self.On Aim` (`self.K2_GetActorLocation` _closest_actor))))

(event `self.Sphere.OnComponentBeginOverlap`
  (params (OverlappedComponent :type "PrimitiveComponent Object Reference") (OtherActor :type "Actor Object Reference") (OtherComp :type "PrimitiveComponent Object Reference") (OtherBodyIndex :type Integer) (bFromSweep :type Boolean) (SweepResult :type "HitResult Structure (by ref)"))
  (bind _asbp_ship (cast `/Game/Ships/BP_Ship` OtherActor))
  (`KismetArrayLibrary.Array_Add` (`self.Ships`) _asbp_ship))

(event `self.Sphere.OnComponentEndOverlap`
  (params (OverlappedComponent :type "PrimitiveComponent Object Reference") (OtherActor :type "Actor Object Reference") (OtherComp :type "PrimitiveComponent Object Reference") (OtherBodyIndex :type Integer))
  (bind _asbp_ship (cast `/Game/Ships/BP_Ship` OtherActor))
  (`KismetArrayLibrary.Array_RemoveItem` (`self.Ships`) _asbp_ship))

(fn `Aim`
  (`NiagaraComponent.SetVariableVec3` (`self.NS`) "Target" (`self.Aim Location`)))

(fn `Find Closest Actor`
  (returns (`Closest Actor` :type "Actor Object Reference"))
  (locals (`Min Index` :type Integer :default 0) (Distance :type "Float (double-precision)" :default 99999999.0))
  (bind _returnvalue (`KismetMathLibrary.Vector_DistanceSquared` (`self.K2_GetActorLocation` (`self.Ship`)) (`self.K2_GetActorLocation` (`|GetArrayItem` (`self.Ships`) (`local.Min Index`)))))
  (for (_array_element _array_index) (`self.Ships`)
    (if (!= (`GameplayStatics.GetObjectClass` _array_element) (`GameplayStatics.GetObjectClass` (`self.Ship`)))
      (if (< _returnvalue (`local.Distance`))
        (set `local.Min Index` _array_index)
        (set `local.Distance` _returnvalue))))
  (return (`|GetArrayItem` (`self.Ships`) (`local.Min Index`))))

(fn `Get Power Points`
  (returns (Points :type Integer))
  (bind _data_functional (break `/Game/Ships/Modules/Squadron/Structures/BPS_Squadron` (`self.Data`)))
  (bind (_shuttlecount _flightduration _flightdelay _bulletspeed _flightradius _shuttlespeed _damage) (break `/Game/Ships/Modules/Squadron/Structures/BPS_Squadron_Functional` _data_functional))
  (return (+ (`parent.Get Power Points`) (`KismetMathLibrary.FTrunc` (* _shuttlecount _flightduration (`.DamagePoints_2_FDD4BB764CC37523C51825A835A7C714` (break `/Game/DamageSystem/Structures/BPS_Damage` _damage)) (`self.DamagePower`))))))

(fn `Location In Range`
  (params (Location :type "Vector Structure"))
  (returns (_ :type Boolean))
  (bind _data_functional (break `/Game/Ships/Modules/Squadron/Structures/BPS_Squadron` (`self.Data`)))
  (bind (_shuttlecount _flightduration _flightdelay _bulletspeed _flightradius) (break `/Game/Ships/Modules/Squadron/Structures/BPS_Squadron_Functional` _data_functional))
  (bind (_returnvalue_x _returnvalue_y) (`KismetMathLibrary.BreakVector` (`SceneComponent.K2_GetComponentLocation` (`self.DefaultSceneRoot`))))
  (return (< (`KismetMathLibrary.Vector_DistanceSquared` (`KismetMathLibrary.MakeVector` Location_X Location_Y) (`KismetMathLibrary.MakeVector` _returnvalue_x _returnvalue_y)) (* _flightradius _flightradius))))

(fn `Setup Particle System`
  (params (`Module Name` :type Name))
  (bind (_data_functional _data_appearance) (break `/Game/Ships/Modules/Squadron/Structures/BPS_Squadron` (`self.Data`)))
  (bind _data_functional_2 (break `/Game/Ships/Modules/Squadron/Structures/BPS_Squadron` (`self.Data`)))
  (bind _data_functional_3 (break `/Game/Ships/Modules/Squadron/Structures/BPS_Squadron` (`self.Data`)))
  (bind _data_functional_4 (break `/Game/Ships/Modules/Squadron/Structures/BPS_Squadron` (`self.Data`)))
  (bind _data_functional_5 (break `/Game/Ships/Modules/Squadron/Structures/BPS_Squadron` (`self.Data`)))
  (bind (_data_functional_6 _data_appearance_2) (break `/Game/Ships/Modules/Squadron/Structures/BPS_Squadron` (`self.Data`)))
  (bind (_data_functional_7 _data_appearance_3) (break `/Game/Ships/Modules/Squadron/Structures/BPS_Squadron` (`self.Data`)))
  (bind (_shuttlecount _flightduration _flightdelay) (break `/Game/Ships/Modules/Squadron/Structures/BPS_Squadron_Functional` _data_functional_3))
  (bind (_shuttlecount_2 _flightduration_2 _flightdelay_2 _bulletspeed _flightradius) (break `/Game/Ships/Modules/Squadron/Structures/BPS_Squadron_Functional` _data_functional_4))
  (bind (_shuttlecolor _trailcolor _bulletcolor _shuttlesize _trailsize _bulletsize) (break `/Game/Ships/Modules/Squadron/Structures/BPS_Squadron_Appearance` _data_appearance))
  (bind (_shuttlecolor_2 _trailcolor_2 _bulletcolor_2 _shuttlesize_2) (break `/Game/Ships/Modules/Squadron/Structures/BPS_Squadron_Appearance` _data_appearance_2))
  (bind (_shuttlecolor_3 _trailcolor_3 _bulletcolor_3 _shuttlesize_3 _trailsize_2 _bulletsize_2 _trailduration) (break `/Game/Ships/Modules/Squadron/Structures/BPS_Squadron_Appearance` _data_appearance_3))
  (bind _returnvalue (`|GetDataTableRow` "/Game/Ships/Modules/Squadron/DT_ShipSquadronData.DT_ShipSquadronData" `Module Name`)
    (:`then`
      (set `self.Data` _returnvalue)
      (`|ExecutionSequence`
        (:`then_0`
          ;[1 1 1] Particle Count
          (`NiagaraComponent.SetVariableInt` (`self.NS`) "ShuttleCount" (`.ShuttleCount_2_AB5A4BDF46671B583E3FC891BCBB1587` (break `/Game/Ships/Modules/Squadron/Structures/BPS_Squadron_Functional` _data_functional_2)))
          ;[1 1 1] Loop
          (`NiagaraComponent.SetVariableFloat` (`self.NS`) "FlightDuration" _flightduration)
          ;[1 1 1] Reach
          (`NiagaraComponent.SetVariableFloat` (`self.NS`) "BulletSpeed" _bulletspeed)
          ;[1 1 1] Shuttle Speed
          (`NiagaraComponent.SetVariableFloat` (`self.NS`) "ShuttleSpeed" (`.ShuttleSpeed_13_3C55CB5B4B3BCC955EF3249E66D8F40B` (break `/Game/Ships/Modules/Squadron/Structures/BPS_Squadron_Functional` _data_functional_5))))
        (:`then_1`
          (`NiagaraComponent.SetVariableFloat` (`self.NS`) "FlightDelay" _flightdelay)
          (`NiagaraComponent.SetVariableFloat` (`self.NS`) "FlightRadius" _flightradius))
        (:`then_2`
          (`|ExecutionSequence`
            (:`then_0`
              ;[1 1 1] Shuttle
              (`NiagaraComponent.SetVariableLinearColor` (`self.NS`) "ShuttleColor" _shuttlecolor_2)
              ;[1 1 1] Trail
              (`NiagaraComponent.SetVariableLinearColor` (`self.NS`) "TrailColor" _trailcolor_3)
              ;[1 1 1] Bullets
              (`NiagaraComponent.SetVariableLinearColor` (`self.NS`) "BulletColor" _bulletcolor))
            (:`then_1`
              (`NiagaraComponent.SetVariableFloat` (`self.NS`) "ShuttleSize" _shuttlesize_2)
              (`NiagaraComponent.SetVariableFloat` (`self.NS`) "TrailSize" _trailsize_2)
              (`NiagaraComponent.SetVariableFloat` (`self.NS`) "BulletSize" _bulletsize))
            (:`then_2`
              (`NiagaraComponent.SetVariableFloat` (`self.NS`) "TrailDuration" _trailduration))
            (:`then_3`
              (`NiagaraComponent.SetVariableObject` (`self.NS`) "BPTarget" self)
              (`NiagaraComponent.SetVariableVec3` (`self.NS`) "Target" (`self.Aim Location`)))))))))

(fn `UserConstructionScript`
  (`parent.UserConstructionScript`))