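; BPC_DamageParticleIndicator is a particle component on BP_Ship that signals hull damage through its emission amount.
; On BeginPlay it binds to the ShipHull's HP events and sets the EmitCount particle parameter to zero.
; HP changes scale emission linearly as the HP fraction drops below SmokeThreshold, with no clamp on negative results above it.
; Reaching zero HP sets emission back to zero.
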(event `self.ReceiveBeginPlay`
  (bind _asbp_ship (cast `/Game/Ships/BP_Ship` (`self.GetOwner`)))
  (bind _output_get (set `self.Ship` _asbp_ship))
  (bind _ship_hull (`/Game/Ships/BP_Ship.Ship Hull` _output_get))
  (add `/Game/DamageSystem/Blueprints/BPC_DamageableLayer.On HP Changed` _ship_hull (delegate `On HP Changed`))
  (add `/Game/DamageSystem/Blueprints/BPC_DamageableLayer.On HP Zero` _ship_hull (delegate `On HP Zero`))
  (`self.SetVariableFloat` "EmitCount"))

(event `On HP Changed`
  (params (`HP Delta` :type Integer))
  (bind _ship_hull (`/Game/Ships/BP_Ship.Ship Hull` (`self.Ship`)))
  (`self.SetVariableFloat` "EmitCount" (* (- 1.0 (/ (/ (`KismetMathLibrary.Conv_IntToDouble` (`/Game/DamageSystem/Blueprints/BPC_DamageableLayer.Current HP` _ship_hull)) (`/Game/DamageSystem/Blueprints/BPC_DamageableLayer.Max HP` _ship_hull)) (`self.Smoke Threshold`))) (`self.EmitCount`))))

(event `On HP Zero`
  (`self.SetVariableFloat` "EmitCount"))