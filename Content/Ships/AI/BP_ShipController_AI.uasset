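; AI controller Blueprint for enemy ships that starts their behavior tree when play begins.
; It loads the ship blackboard and sets Target to the player ship found in the level.
; After a one-tick delay it reads the controlled ship's max fire range into WeaponRange, then runs BT_Ship.
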(event `self.ReceiveBeginPlay`
  (bind _blackboardcomponent (`self.UseBlackboard` "/Game/Ships/AI/BB_Ship.BB_Ship"))
  (bind _returnvalue (`GameplayStatics.GetActorOfClass` "/Game/Ships/Player/BP_Ship_Player.BP_Ship_Player_C"))
  (`BlackboardComponent.SetValueAsObject` _blackboardcomponent "Target" _returnvalue)
  (`KismetSystemLibrary.DelayUntilNextTick`)
  (bind _asbp_ship_ai (cast `/Game/Ships/AI/BP_Ship_AI` (`self.K2_GetPawn` self)))
  (bind _max_range (`/Game/Ships/BP_Ship.Get Max Fire Range` _asbp_ship_ai))
  (`BlackboardComponent.SetValueAsFloat` _blackboardcomponent "WeaponRange" _max_range)
  (`self.RunBehaviorTree` "/Game/Ships/AI/BT_Ship.BT_Ship"))

(fn `UserConstructionScript`)