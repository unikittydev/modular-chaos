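; Ship component that plays an impact sound whenever its owning BP_Ship loses HP.
; On BeginPlay it casts the owner to BP_Ship and binds to the HP changed event of that ship's damageable manager.
; A negative HP delta plays the configured sound at the owner's location.
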(event `self.ReceiveBeginPlay`
  (bind _asbp_ship (cast `/Game/Ships/BP_Ship` (`self.GetOwner`)))
  (add `/Game/DamageSystem/Blueprints/BPC_DamageableManager.On HP Changed` (`/Game/Ships/BP_Ship.BPC_DamageableManager` _asbp_ship) (delegate `HP Changed`)))

(event `HP Changed`
  (params (`HP Delta` :type Integer))
  (if (< `HP Delta` 0)
    (`GameplayStatics.PlaySoundAtLocation` (`self.Sound`) (`Actor.K2_GetActorLocation` (`self.GetOwner`)) (struct) 1.0 1.0 0.0 null null null null)))