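; Inventory component for the player ship that stores owned items as a list of names, with add, remove, get and set functions.
; Adding or removing an item fires a matching notification event.
; A cheat mode, applied on BeginPlay, replaces the list with every row name from the ship module data table and makes add and remove calls do nothing.
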(event `self.ReceiveBeginPlay`
  (`self.Set Cheat Inventory` (`self.Cheat Inventory`)))

(fn `Add Item`
  (params (`Item Name` :type Name))
  (if (not (`self.Cheat Inventory`))
    (`KismetArrayLibrary.Array_Add` (`self.Items`) `Item Name`)
    (`self.Item Added` `Item Name`)))

(fn `Get All Items`
  (returns (Items :type "Array of Name"))
  (return (`self.Items`)))

(fn `Remove Item`
  (params (`Item Name` :type Name))
  (bind _items (`self.Items`))
  (if (not (`self.Cheat Inventory`))
    (`KismetArrayLibrary.Array_Remove` _items (`KismetArrayLibrary.Array_Find` _items `Item Name`))
    (`self.Item Removed` `Item Name`)
    (return)))

(fn `Set Cheat Inventory`
  (params (Value :type Boolean))
  (bind _output_get (set `self.Cheat Inventory` Value))
  (if _output_get
    (`KismetArrayLibrary.Array_Clear` (`self.Items`))
    (bind _outrownames (`DataTableFunctionLibrary.GetDataTableRowNames` "/Game/Ships/Modules/Base/DT_ShipModuleData.DT_ShipModuleData"))
    (`KismetArrayLibrary.Array_Append` (`self.Items`) _outrownames)))

(fn `Set Items`
  (params (Items :type "Array of Name"))
  (bind _items (`self.Items`))
  (`KismetArrayLibrary.Array_Clear` _items)
  (`KismetArrayLibrary.Array_Append` _items Items))