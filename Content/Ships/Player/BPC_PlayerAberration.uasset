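; Player ship component that turns hull damage into screen feedback through aberration and desaturation post-processing.
; On begin play it binds to the owning ship's hull HP changes, finds the PP_Aberration-tagged volume and swaps its first post-process material for a dynamic instance.
; Each HP change rebuilds the volume's settings, scaling intensity from the HP ratio against a threshold, and feeds that ratio to the material's Percentage parameter.
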(event `self.ReceiveBeginPlay`
  (bind _asbp_ship (cast `/Game/Ships/BP_Ship` (`self.GetOwner`)))
  (bind _output_get (set `self.Ship` _asbp_ship))
  (add `/Game/DamageSystem/Blueprints/BPC_DamageableLayer.On HP Changed` (`/Game/Ships/BP_Ship.Ship Hull` _output_get) (delegate `HP Changed`))
  (bind _outactors (`GameplayStatics.GetAllActorsOfClassWithTag` "/Script/Engine.PostProcessVolume" "PP_Aberration"))
  (bind _output_get_2 (set `self.PP Volume` (`|GetArrayItem` _outactors)))
  (bind _array (break `WeightedBlendables` (`.WeightedBlendables` (break `PostProcessSettings` (`PostProcessVolume.Settings` _output_get_2)))))
  (bind (_weight _object) (break `WeightedBlendable` (`|GetArrayItem` _array)))
  (bind _asmaterial (cast `Material` _object))
  (bind _returnvalue (`KismetMaterialLibrary.CreateDynamicMaterialInstance` _asmaterial))
  (bind _output_get_3 (set `self.Desaturation PPM` _returnvalue))
  (`KismetArrayLibrary.Array_Set` _array 0 (make `WeightedBlendable` _weight _output_get_3)))

(event `HP Changed`
  (params (`HP Delta` :type Integer))
  (bind _ship_hull (`/Game/Ships/BP_Ship.Ship Hull` (`self.Ship`)))
  (bind _returnvalue (/ (`KismetMathLibrary.Conv_IntToDouble` (`/Game/DamageSystem/Blueprints/BPC_DamageableLayer.Current HP` _ship_hull)) (`/Game/DamageSystem/Blueprints/BPC_DamageableLayer.Max HP` _ship_hull)))
  (set `PostProcessVolume.Settings` (make `PostProcessSettings` :`SceneFringeIntensity` (* (- 1.0 (/ _returnvalue (`self.Aberration Threshold`))) (`self.Max Aberration`)) :`WeightedBlendables` (make `WeightedBlendables` (`|MakeArray` (make `WeightedBlendable` 1.0 (`self.Desaturation PPM`))))) (`self.PP Volume`))
  (`MaterialInstanceDynamic.SetScalarParameterValue` (`self.Desaturation PPM`) "Percentage" _returnvalue))