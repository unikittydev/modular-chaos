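; BPC_LoseHandler is a component on the player ship that handles losing when the hull is destroyed.
; On BeginPlay it binds to the owning BP_Ship_Player's hull HP-zero event.
; When that fires, it prints the level and wave reached from BP_LevelManager and plays the WBP_LoseOverlay turn-on animation.
; After the animation ends, it restores cursor and UI-only input and opens the menu level.
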(event `self.ReceiveBeginPlay`
  (bind _asbp_ship_player (cast `/Game/Ships/Player/BP_Ship_Player` (`self.GetOwner`)))
  (add `/Game/DamageSystem/Blueprints/BPC_DamageableLayer.On HP Zero` (`/Game/Ships/BP_Ship.Ship Hull` _asbp_ship_player) (delegate `On Ship Destroyed`)))

(event `On Ship Destroyed`
  (bind _returnvalue (`GameplayStatics.GetPlayerController` 0))
  (bind _returnvalue_2 (`GameplayStatics.GetActorOfClass` "/Game/Progression/BP_LevelManager.BP_LevelManager_C"))
  (`KismetSystemLibrary.PrintString` (`KismetStringLibrary.Concat_StrStr` "Died at " "L" (`KismetStringLibrary.Conv_IntToString` (`/Game/Progression/BP_LevelManager.Current Level Index` _returnvalue_2)) "W" (`KismetStringLibrary.Conv_IntToString` (`/Game/Progression/BP_LevelManager.Current Wave Index` _returnvalue_2))) true true (struct :`R` 1.0 :`B` 0.008842 :`A` 1.0) 15.0)
  (bind _returnvalue_3 (`|CreateWidget` "/Game/Ships/Player/UI/WBP_LoseOverlay.WBP_LoseOverlay_C"))
  (`UserWidget.AddToViewport` _returnvalue_3 0)
  (bind _turnon (`/Game/Ships/Player/UI/WBP_LoseOverlay.TurnOn` _returnvalue_3))
  (`UserWidget.PlayAnimation` _returnvalue_3 _turnon 0.0 1 "Forward" 1.0 false)
  (`KismetSystemLibrary.Delay` (`WidgetAnimation.GetEndTime` _turnon))
  (set `PlayerController.bShowMouseCursor` true _returnvalue)
  (`WidgetBlueprintLibrary.SetInputMode_UIOnlyEx` _returnvalue null)
  (`GameplayStatics.OpenLevelBySoftObjectPtr` "/Game/L_Menu.L_Menu"))