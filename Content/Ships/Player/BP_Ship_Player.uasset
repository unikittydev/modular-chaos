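; Player-controlled ship Blueprint that extends a parent ship with input, HUD, crosshair and save loading.
; Enhanced Input actions broadcast move and fire dispatchers, with a mode toggle switching horizontal input between yaw and strafe.
; Mouse aim is projected onto the Z=0 game plane, driving a clamped, lerped spring-arm camera offset.
; It registers its body with the celestial system and switches to UI-only input at zero hull HP.
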(event `self.ReceiveBeginPlay`
  (`parent.ReceiveBeginPlay`)
  (`|ExecutionSequence`
    (:`then_0`
      ;[1 1 1] Input Mapping
      (bind _asbp_ship_controller (cast `/Game/Ships/Player/BP_ShipController` (`self.GetController`)))
      (bind _returnvalue (pcsubsystem `EnhancedInputLocalPlayerSubsystem` _asbp_ship_controller))
      (`EnhancedInputSubsystemInterface.AddMappingContext` _returnvalue "/Game/Input/IMC_Camera.IMC_Camera" 0 (struct))
      (`EnhancedInputSubsystemInterface.AddMappingContext` _returnvalue "/Game/Input/IMC_Ship_Thrusters.IMC_Ship_Thrusters" 0 (struct))
      (`EnhancedInputSubsystemInterface.AddMappingContext` _returnvalue "/Game/Input/IMC_Ship_Weapon.IMC_Ship_Weapon" 0 (struct)))
    (:`then_1`
      ;[1 1 1] Setup Celestial System
      (bind _returnvalue_2 (`GameplayStatics.GetActorOfClass` "/Game/CelestialSystem/Blueprints/BP_CelestialSystem.BP_CelestialSystem_C"))
      (`/Engine/EditorBlueprintResources/StandardMacros.IsValid` _returnvalue_2
        (:`Is Valid`
          (`/Game/CelestialSystem/Blueprints/BP_CelestialSystem.Set Target Body` _returnvalue_2 (`self.Celestial Body`)))))
    (:`then_2`
      (add `/Game/DamageSystem/Blueprints/BPC_DamageableLayer.On HP Zero` (`self.Ship Hull`) (delegate `self.On HP Zero`))
      (`self.Set Ship Enabled` true))))

(event `self.On HP Zero`
  (`parent.On HP Zero`)
  (`WidgetBlueprintLibrary.SetInputMode_UIOnlyEx` (`GameplayStatics.GetPlayerController` 0) (`self.UI`) "DoNotLock" true))

(event `self.ReceiveDestroyed`
  (bind _returnvalue (`GameplayStatics.GetActorOfClass` "/Game/CelestialSystem/Blueprints/BP_CelestialSystem.BP_CelestialSystem_C"))
  (`/Game/CelestialSystem/Blueprints/BP_CelestialSystem.Remove Target Body` _returnvalue))

(event `self.ReceiveTick`
  (params (DeltaSeconds :type "Float (single-precision)"))
  (`self.Adjust Camera Offset` (`self.Aim Location`) DeltaSeconds))

(event `EnhancedInput|/Game/Input/Actions/IA_Fire`
  (params (ActionValue :type Boolean) (ElapsedSeconds :type "Float (double-precision)") (TriggeredSeconds :type "Float (double-precision)") (InputAction :type "InputAction Object Reference" :default "/Game/Input/Actions/IA_Fire.IA_Fire"))
  (:`Started`
    (`self.On Ship Fire Start`))
  (:`Canceled`
    (`self.On Ship Fire Stop`)))

(event `EnhancedInput|/Game/Input/Actions/IA_MoveShip`
  (params (ActionValue :type "Vector2D Structure") (ElapsedSeconds :type "Float (double-precision)") (TriggeredSeconds :type "Float (double-precision)") (InputAction :type "InputAction Object Reference" :default "/Game/Input/Actions/IA_MoveShip.IA_MoveShip"))
  (:`Triggered`
    (`self.On Ship Move` ActionValue_Y (`KismetMathLibrary.SelectFloat` ActionValue_X 0.0 (`self.Strafe Mode`)) (`KismetMathLibrary.SelectFloat` 0.0 ActionValue_X (`self.Strafe Mode`)))))

(event `EnhancedInput|/Game/Input/Actions/IA_ShipMoveMode`
  (params (ActionValue :type Boolean) (ElapsedSeconds :type "Float (double-precision)") (TriggeredSeconds :type "Float (double-precision)") (InputAction :type "InputAction Object Reference" :default "/Game/Input/Actions/IA_ShipMoveMode.IA_ShipMoveMode"))
  (:`Started`
    (bind _output_get (set `self.Strafe Mode` true))
    (`self.On Ship Move Mode Changed` _output_get))
  (:`Completed`
    (bind _output_get_2 (set `self.Strafe Mode` false))
    (`self.On Ship Move Mode Changed` _output_get_2)))

(event `InputVectorAxis|Mouse2D`
  (params (AxisValue :type "Vector Structure"))
  (if (`self.IsActorTickEnabled` (`self.GetController`))
    (bind _aim_location (`self.Get Aim Location`))
    (bind _output_get (set `self.Aim Location` _aim_location))
    (`self.On Set Aim` _output_get)))

(fn `Add UI`
  (bind _returnvalue (`|GenericCreateObject` (`GameplayStatics.GetPlayerController` 0) "/Game/Ships/Player/UI/WBP_Player.WBP_Player_C" self))
  (bind _output_get (set `self.UI` _returnvalue))
  (`UserWidget.AddToViewport` _output_get 0))

(fn `Adjust Camera Offset`
  (params (`Aim Location` :type "Vector Structure") (`Delta Seconds` :type "Float (double-precision)"))
  (bind _springarm (`self.SpringArm`))
  (bind _returnvalue (`SceneComponent.K2_GetComponentLocation` (`self.SpringArm`)))
  (bind (_returnvalue_x _returnvalue_y) (`KismetMathLibrary.BreakVector` (`SceneComponent.K2_GetComponentLocation` _springarm)))
  (bind (_socketoffset_x _socketoffset_y) (`KismetMathLibrary.BreakVector` (`SpringArmComponent.SocketOffset` _springarm)))
  (bind (_socketoffset_x_2 _socketoffset_y_2 _socketoffset_z) (`KismetMathLibrary.BreakVector` (`SpringArmComponent.SocketOffset` (`self.SpringArm`))))
  (bind (_returnvalue_x_2 _returnvalue_y_2) (`KismetMathLibrary.BreakVector` (+ (`KismetMathLibrary.ClampVectorSize` (- (`KismetMathLibrary.MakeVector` (.x `Aim Location`) (.y `Aim Location`)) (+ (`KismetMathLibrary.MakeVector` _returnvalue_x _returnvalue_y) (`KismetMathLibrary.MakeVector` _socketoffset_x _socketoffset_y))) 0.0 (`self.Max Camera Offset Length`)) _returnvalue)))
  (bind (_returnvalue_x_3 _returnvalue_y_3) (`KismetMathLibrary.BreakVector` (- (`KismetMathLibrary.MakeVector` _returnvalue_x_2 _returnvalue_y_2) _returnvalue)))
  (set `SpringArmComponent.SocketOffset` (`KismetMathLibrary.VLerp` (`SpringArmComponent.SocketOffset` (`self.SpringArm`)) (`KismetMathLibrary.MakeVector` _returnvalue_x_3 _returnvalue_y_3 _socketoffset_z) (* (`self.Camera Lerp Speed`) `Delta Seconds`)) (`self.SpringArm`)))

(fn `Get Aim Location`
  (returns (`Aim Location` :type "Vector Structure"))
  (bind _asplayer_controller (cast `PlayerController` (`self.GetController`)))
  (bind _location (`/Game/Blueprints/BPL_ScreenUtils.Project Mouse Location on Game Plane` _asplayer_controller))
  (return _location))

(fn `Reset Camera Offset`
  (bind (_socketoffset_x _socketoffset_y _socketoffset_z) (`KismetMathLibrary.BreakVector` (`SpringArmComponent.SocketOffset` (`self.SpringArm`))))
  (set `SpringArmComponent.SocketOffset` (`KismetMathLibrary.MakeVector` 0.0 0.0 _socketoffset_z) (`self.SpringArm`)))

(fn `Set Ship Enabled`
  (params (Enable :type Boolean))
  (`parent.Set Ship Enabled` Enable)
  (if (`local.Enable`)
    (bind _returnvalue (`|SpawnActorFromClass` "/Game/Ships/Modules/Weapons/Blueprints/BP_ShipCross.BP_ShipCross_C" (`KismetMathLibrary.MakeTransform` (0.0 0.0 0.0)) "AlwaysSpawn" "MultiplyWithRoot" null self null))
    (set `self.ShipCross` _returnvalue)
    (`self.Add UI`)
    (else
      (`self.K2_DestroyActor` (`self.ShipCross`))
      (`Widget.RemoveFromParent` (`self.UI`))
      (`self.Reset Camera Offset`))))

(fn `Set Ship Reset`
  (params (Reset :type Boolean))
  (`parent.Set Ship Reset` Reset)
  (if true
    (`self.Reset Camera Offset`)))

(fn `Try Load Ship`
  (bind _returnvalue (`GameplayStatics.GetActorOfClass` "/Game/Progression/BP_SaveHandler.BP_SaveHandler_C"))
  (`/Engine/EditorBlueprintResources/StandardMacros.IsValid` _returnvalue
    (:`Is Valid`
      (`self.Load Ship From Data` (`/Game/Progression/BP_SaveGame_Player.Ship` (`/Game/Progression/BP_SaveHandler.Save` _returnvalue))))
    (:`Is Not Valid`
      (`self.Load Ship Data`))))

(fn `UserConstructionScript`
  (`parent.UserConstructionScript`))