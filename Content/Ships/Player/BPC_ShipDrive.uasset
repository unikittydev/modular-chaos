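; BPC_ShipDrive is a drive component for the player ship, currently inactive beyond setup.
; On BeginPlay it casts its owner to BP_Ship_Player and caches it along with the level's BP_JumpSystem actor.
; Tick is empty.
; Disconnected logic would advance the ship's CelestialBody local and world coordinates along physics velocity, scaled by speed relative to MaxVelocity, using AUSpeed and LightSpeed respectively.
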(event `self.ReceiveBeginPlay`
  (bind _asbp_ship_player (cast `/Game/Ships/Player/BP_Ship_Player` (`self.GetOwner`)))
  (set `self.Ship` _asbp_ship_player)
  (bind _returnvalue (`GameplayStatics.GetActorOfClass` "/Game/CelestialSystem/Blueprints/Unused/BP_JumpSystem.BP_JumpSystem_C"))
  (set `self.JumpSystem` _returnvalue))

(event `self.ReceiveTick`
  (params (DeltaSeconds :type "Float (single-precision)")))