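; BPC_PlayerFOV is a component for the player ship that changes the camera's field of view with the ship's speed.
; On BeginPlay it casts its owner to BP_Ship_Player and caches it.
; Each tick it divides the BoxCollision physics velocity magnitude by MaxFOVVelocity, clamps that to 0–1, and uses it to linearly blend the camera FOV from FromFOV to ToFOV, with no extra smoothing.
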(event `self.ReceiveBeginPlay`
  (bind _asbp_ship_player (cast `/Game/Ships/Player/BP_Ship_Player` (`self.GetOwner`)))
  (set `self.Ship` _asbp_ship_player))

(event `self.ReceiveTick`
  (params (DeltaSeconds :type "Float (single-precision)"))
  (bind _returnvalue (`PrimitiveComponent.GetPhysicsLinearVelocity` (`/Game/Ships/BP_Ship.BoxCollision` (`self.Ship`)) "None"))
  (`CameraComponent.SetFieldOfView` (`/Game/Ships/Player/BP_Ship_Player.Camera` (`self.Ship`)) (`KismetMathLibrary.Lerp` (`self.From FOV`) (`self.To FOV`) (`KismetMathLibrary.FClamp` (/ (`KismetMathLibrary.VSize` _returnvalue) (`self.Max FOV Velocity`))))))