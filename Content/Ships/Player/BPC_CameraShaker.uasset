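; Player ship component that shakes the player camera on damage, item pickup and shock wave hits.
; On BeginPlay it binds to hull and shield HP changes, shock wave and item collection events on its owning BP_Ship_Player.
; Each event passes its own intensity and duration to ShakeCamera, with HP changes counting only when negative.
; ShakeCamera starts a scaled shake, then uses a retriggerable delay to softly stop the latest instance.
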(event `self.ReceiveBeginPlay`
  (bind _ship (`self.Ship`))
  (bind _asbp_ship_player (cast `/Game/Ships/Player/BP_Ship_Player` (`self.GetOwner`)))
  (bind _output_get (set `self.Ship` _asbp_ship_player))
  (add `/Game/DamageSystem/Blueprints/BPC_DamageableLayer.On HP Changed` (`/Game/Ships/BP_Ship.Ship Hull` _output_get) (delegate `On HP Changed`))
  (add `/Game/DamageSystem/Blueprints/BPC_DamageableLayer.On HP Changed` (`/Game/Ships/BP_Ship.Ship Shield` _output_get) (delegate `On HP Changed`))
  (add `/Game/Ships/BP_Ship.On Get Ship In Shock Wave` _ship (delegate `On Get Ship In Shock Wave`))
  (add `/Game/Ships/Player/BP_Ship_Player.On Item Collected` _ship (delegate `Item Collected`)))

(event `On HP Changed`
  (params (`HP Delta` :type Integer))
  (if (< `HP Delta` 0)
    (`self.Shake Camera` (`self.Damage Shake Intensity`) (`self.Damage Shake Duration`))))

(event `Item Collected`
  (`self.Shake Camera` (`self.Collect Item Shake Intensity`) (`self.Collect Item Shake Duration`)))

(event `On Get Ship In Shock Wave`
  (`self.Shake Camera` (`self.Destroy Shake Intensity`) (`self.Destroy Shake Duration`)))

(event `Shake Camera`
  (params (Intensity :type "Float (double-precision)") (Duration :type "Float (double-precision)"))
  (bind _returnvalue (`GameplayStatics.GetPlayerCameraManager` 0))
  (bind _returnvalue_2 (`PlayerCameraManager.StartCameraShakeFromSource` :`self` _returnvalue :`ShakeClass` "/Game/Ships/Player/PlayerCameraShake.PlayerCameraShake_C" :`Scale` Intensity))
  (`KismetSystemLibrary.RetriggerableDelay` Duration)
  (`PlayerCameraManager.StopCameraShake` _returnvalue _returnvalue_2 false))