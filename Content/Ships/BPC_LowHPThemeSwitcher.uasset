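; Ship component that switches the level's music theme to a chiptune variant when the owning ship's hull HP runs low.
; On BeginPlay it finds the BP_ThemeSystem actor and binds to the owner BP_Ship hull's HP change event.
; Each change compares the HP ratio to a threshold, and a Chiptuned flag ensures SwitchTheme fires only on crossings, reverting when HP recovers.
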(event `self.ReceiveBeginPlay`
  (bind _returnvalue (`GameplayStatics.GetActorOfClass` "/Game/ThemeSystem/Blueprints/BP_ThemeSystem.BP_ThemeSystem_C"))
  (set `self.Theme System` _returnvalue)
  (bind _asbp_ship (cast `/Game/Ships/BP_Ship` (`self.GetOwner`)))
  (bind _output_get (set `self.Ship` _asbp_ship))
  (add `/Game/DamageSystem/Blueprints/BPC_DamageableLayer.On HP Changed` (`/Game/Ships/BP_Ship.Ship Hull` _output_get) (delegate `HP Changed`)))

(event `HP Changed`
  (params (`HP Delta` :type Integer))
  (bind _hp_percent_threshold (`self.HP Percent Threshold`))
  (bind _ship_hull (`/Game/Ships/BP_Ship.Ship Hull` (`self.Ship`)))
  (bind _returnvalue (/ (`KismetMathLibrary.Conv_IntToDouble` (`/Game/DamageSystem/Blueprints/BPC_DamageableLayer.Current HP` _ship_hull)) (`/Game/DamageSystem/Blueprints/BPC_DamageableLayer.Max HP` _ship_hull)))
  (if (`self.Chiptuned`)
    (if (> _returnvalue _hp_percent_threshold)
      (`/Game/ThemeSystem/Blueprints/BP_ThemeSystem.Switch Theme` (`self.Theme System`) false)
      (set `self.Chiptuned` false))
    (elif (< _returnvalue _hp_percent_threshold)
      (`/Game/ThemeSystem/Blueprints/BP_ThemeSystem.Switch Theme` (`self.Theme System`) true)
      (set `self.Chiptuned` true))))