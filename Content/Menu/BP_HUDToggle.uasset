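; BP_HUDToggle is an actor that toggles a clean, HUD-free view when Tab is pressed.
; On BeginPlay it caches the BP_Ship_Player found in the level.
; A FlipFlop alternates between hiding and showing all top-level user widgets, along with the ship and its ShipCross actor.
; The ship visibility calls sit inside the widget loop, so they repeat per widget and only run when a widget exists.
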(event `self.ReceiveBeginPlay`
  (bind _returnvalue (`GameplayStatics.GetActorOfClass` "/Game/Ships/Player/BP_Ship_Player.BP_Ship_Player_C"))
  (set `self.Ship` _returnvalue))

(event `Key|Tab`
  (params (Key :type "Key Structure"))
  (bind _ship (`self.Ship`))
  (bind _ship_2 (`self.Ship`))
  (:`Pressed`
    (`/Engine/EditorBlueprintResources/StandardMacros.FlipFlop`
      (:`A`
        (bind _foundwidgets (`WidgetBlueprintLibrary.GetAllWidgetsOfClass` "/Script/UMG.UserWidget"))
        (for _array_element _foundwidgets
          (`Widget.SetVisibility` _array_element "Hidden")
          (`self.SetActorHiddenInGame` _ship_2 true)
          (`self.SetActorHiddenInGame` (`/Game/Ships/Player/BP_Ship_Player.ShipCross` _ship_2) true)))
      (:`B`
        (bind _foundwidgets_2 (`WidgetBlueprintLibrary.GetAllWidgetsOfClass` "/Script/UMG.UserWidget"))
        (for _array_element_2 _foundwidgets_2
          (`Widget.SetVisibility` _array_element_2 "Visible")
          (`self.SetActorHiddenInGame` _ship false)
          (`self.SetActorHiddenInGame` (`/Game/Ships/Player/BP_Ship_Player.ShipCross` _ship) false))))))

(fn `UserConstructionScript`)