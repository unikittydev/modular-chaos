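; Pause handler Blueprint that opens and closes the game's pause menu.
; Tick polls for an Escape press, then pauses the game, creates a WBP_PauseMenu with a reference back to itself, and switches to UI-only input with the cursor shown.
; Resume unpauses, removes the menu, restores game-only input and returns the cursor to its saved pre-pause visibility.
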(event `self.ReceiveTick`
  (params (DeltaSeconds :type "Float (single-precision)"))
  (if (`PlayerController.WasInputKeyJustPressed` (`GameplayStatics.GetPlayerController` 0) "Escape")
    (`self.Pause`)))

(event `Pause`
  (bind _returnvalue (`GameplayStatics.GetPlayerController` 0))
  (`GameplayStatics.SetGamePaused` true)
  (bind _returnvalue_2 (`|CreateWidget` "/Game/Menu/WBP_PauseMenu.WBP_PauseMenu_C" null self))
  (bind _output_get (set `self.Pause Panel` _returnvalue_2))
  (`UserWidget.AddToViewport` _output_get 0)
  (`WidgetBlueprintLibrary.SetInputMode_UIOnlyEx` _returnvalue _output_get)
  (set `self.Mouse Cursor Before Pause` (`PlayerController.bShowMouseCursor` _returnvalue))
  (set `PlayerController.bShowMouseCursor` true _returnvalue))

(event `Resume`
  (bind _returnvalue (`GameplayStatics.GetPlayerController` 0))
  (`GameplayStatics.SetGamePaused` false)
  (`Widget.RemoveFromParent` (`self.Pause Panel`))
  (`WidgetBlueprintLibrary.SetInputMode_GameOnly` _returnvalue)
  (set `PlayerController.bShowMouseCursor` (`self.Mouse Cursor Before Pause`) _returnvalue))

(fn `UserConstructionScript`)