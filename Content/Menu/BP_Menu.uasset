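; BP_Menu is a Blueprint that opens the main menu when play begins.
; It creates WBP_MainMenu, adds it to the viewport, switches input to UI-only and shows the mouse cursor.
; An optional ClearSave flag then deletes the tutorial, completion, player and settings save slots.
; A disconnected test graph that saves and loads a BP_SaveTest object never runs.
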(event `self.ReceiveBeginPlay`
  (bind _returnvalue (`GameplayStatics.GetPlayerController` 0))
  (bind _returnvalue_2 (`|CreateWidget` "/Game/Menu/WBP_MainMenu.WBP_MainMenu_C" (`GameplayStatics.GetPlayerController` 0)))
  (`UserWidget.AddToViewport` _returnvalue_2 0)
  (`WidgetBlueprintLibrary.SetInputMode_UIOnlyEx` _returnvalue _returnvalue_2)
  (set `PlayerController.bShowMouseCursor` true _returnvalue)
  (if (`self.Clear Save`)
    (`GameplayStatics.DeleteGameInSlot` "tutorial")
    (`GameplayStatics.DeleteGameInSlot` "completion")
    (`GameplayStatics.DeleteGameInSlot` "player")
    (`GameplayStatics.DeleteGameInSlot` "settings")))

(fn `UserConstructionScript`)