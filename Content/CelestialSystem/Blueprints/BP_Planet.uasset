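; BP_Planet is a planet actor in the celestial system whose look is driven by a dynamic material on its sphere.
; When Randomize is set, BeginPlay creates that material and randomizes sky, ground and cloud colors by random hue, plus a coordinate offset for variation.
; UpdateSunInfo passes sun location, planet location and sun temperature into the material.
; FadeIn and FadeOut animate a DitherMask parameter over a given time, with optional destruction after fading out.
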(event `self.ReceiveBeginPlay`
  (if (`self.Randomize`)
    (`self.Create Dynamic Material`)
    (`self.Randomize Body`)))

(event `Randomize Body`
  (`MaterialInstanceDynamic.SetVectorParameterValue` (`self.Material`) "DaySkyColor" (`self.Random Color` 0.3 0.4))
  (`MaterialInstanceDynamic.SetVectorParameterValue` (`self.Material`) "GrassColor" (`self.Random Color` 1.0 0.25))
  (`MaterialInstanceDynamic.SetVectorParameterValue` (`self.Material`) "SandColor" (`self.Random Color` 0.5 1.0))
  (`MaterialInstanceDynamic.SetVectorParameterValue` (`self.Material`) "SunsetSkyColor" (`self.Random Color` 1.0 1.0))
  (`MaterialInstanceDynamic.SetVectorParameterValue` (`self.Material`) "CloudColor" (select `bool` (`KismetMathLibrary.RandomBool`) :`false` (`KismetMathLibrary.LinearColor_White`) :`true` (`self.Random Color` 0.8 0.2)))
  (`MaterialInstanceDynamic.SetVectorParameterValue` (`self.Material`) "CoordinateOffset" (`KismetMathLibrary.Conv_VectorToLinearColor` (* (`KismetMathLibrary.RandomUnitVector`) 5.0))))

(event `Fade In`
  (params (Time :type "Float (double-precision)"))
  (`TimelineComponent.SetPlayRate` (`self.Fade In Timeline`) (/ 1.0 Time))
  (bind (_direction _track) (`Timeline|Fade In Timeline` :!via `PlayFromStart`)
    (:`Update`
      (`MaterialInstanceDynamic.SetScalarParameterValue` (`self.Material`) "DitherMask" (`KismetMathLibrary.Lerp` -1.0 2.0 _track)))))

(event `Fade Out`
  (params (Time :type "Float (double-precision)") (Destroy :type Boolean :default true))
  (`TimelineComponent.SetPlayRate` (`self.Fade Out Timeline`) (/ 1.0 Time))
  (bind (_direction _track) (`Timeline|Fade Out Timeline` :!via `PlayFromStart`)
    (:`Update`
      (`MaterialInstanceDynamic.SetScalarParameterValue` (`self.Material`) "DitherMask" (`KismetMathLibrary.Lerp` 2.0 -1.0 _track)))
    (:`Finished`
      (if Destroy
        (`self.K2_DestroyActor`)))))

(fn `Create Dynamic Material`
  (bind _returnvalue (`KismetMaterialLibrary.CreateDynamicMaterialInstance` (`PrimitiveComponent.GetMaterial` (`self.Sphere`) 0)))
  (`PrimitiveComponent.SetMaterial` (`self.Sphere`) 0 _returnvalue)
  (set `self.Material` _returnvalue)
  (return))

(fn `Random Color`
  (params (S :type "Float (double-precision)") (V :type "Float (double-precision)"))
  (returns (Color :type "LinearColor Structure"))
  (return (`KismetMathLibrary.HSVToRGBLinear` (make `LinearColor` (`KismetMathLibrary.RandomFloatInRange` 0.0 360.0) S V 1.0))))

(fn `Update Sun Info`
  (params (`Sun Temperature` :type "Float (double-precision)"))
  (bind _material (`self.Material`))
  (`MaterialInstanceDynamic.SetVectorParameterValue` _material "SunLocation" (`KismetMathLibrary.Conv_VectorToLinearColor` (`/Game/CelestialSystem/Blueprints/BP_CelestialSystem.Sun Location` (`/Game/CelestialSystem/Blueprints/BPC_CelestialBody.Celestial System` (`self.Body`)))))
  (`MaterialInstanceDynamic.SetVectorParameterValue` _material "SelfLocation" (`KismetMathLibrary.Conv_VectorToLinearColor` (`/Game/CelestialSystem/Blueprints/BPC_CelestialBody.World Coordinates` (`self.Body`))))
  (`MaterialInstanceDynamic.SetScalarParameterValue` _material "SunTemperature" `Sun Temperature`))

(fn `UserConstructionScript`)