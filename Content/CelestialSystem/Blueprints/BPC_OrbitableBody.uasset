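; Orbitable body component that computes a circular orbit around a parent body in the celestial system.
; On BeginPlay, an unset Parent is taken from the Body of the owner's attach-parent BP_Planet, and tick is then enabled only if one is found.
; Each tick sets LocalCoordinates to the parent's LocalCoordinates plus a Radius-scaled XY offset, with the angle from game time divided by YearDuration and tau.
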(event `self.ReceiveBeginPlay`
  (`parent.ReceiveBeginPlay`)
  (`/Engine/EditorBlueprintResources/StandardMacros.IsValid` (`self.Parent`)
    (:`Is Not Valid`
      (bind _asbp_planet (cast `/Game/CelestialSystem/Blueprints/BP_Planet` (`Actor.GetAttachParentActor` (`self.GetOwner`)))
        (:`then`
          (set `self.Parent` (`/Game/CelestialSystem/Blueprints/BP_Planet.Body` _asbp_planet)))
        (:`CastFailed`
          _))
      (`self.SetComponentTickEnabled` (`KismetSystemLibrary.IsValid` (`self.Parent`))))))

(event `self.ReceiveTick`
  (params (DeltaSeconds :type "Float (single-precision)"))
  (bind _returnvalue (/ (`KismetSystemLibrary.GetGameTimeInSeconds`) (`self.Year Duration`) (`KismetMathLibrary.GetTAU`) 1.0 1.0))
  (set `self.Local Coordinates` (+ (`/Game/CelestialSystem/Blueprints/BPC_CelestialBody.Local Coordinates` (`self.Parent`)) (* (`KismetMathLibrary.MakeVector` (`KismetMathLibrary.Cos` _returnvalue) (`KismetMathLibrary.Sin` _returnvalue)) (`self.Radius`)))))