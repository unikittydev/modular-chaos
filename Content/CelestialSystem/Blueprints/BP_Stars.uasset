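; BP_Stars drives a star sky particle system that follows the player's camera.
; Each tick it passes the first player's camera location to NEStarSkySystem as CameraPosition.
; It also sets SpawnRate to the distance the camera moved since the last tick times VelocityFactor, so faster movement spawns more particles.
; The distance is not divided by delta time, so the rate varies with frame rate.
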(event `self.ReceiveTick`
  (params (DeltaSeconds :type "Float (single-precision)"))
  (bind _returnvalue (`PlayerCameraManager.GetCameraLocation` (`PlayerController.PlayerCameraManager` (`GameplayStatics.GetPlayerController` 0))))
  (`NiagaraComponent.SetVariablePosition` (`self.NE_StarSky_System`) "CameraPosition" _returnvalue)
  (`NiagaraComponent.SetVariableFloat` (`self.NE_StarSky_System`) "SpawnRate" (* (`KismetMathLibrary.VSize` (- _returnvalue (`self.OldPosition`))) (`self.VelocityFactor`)))
  (`NiagaraComponent.SetVariableFloat` (`self.NE_StarSky_System`) "SpawnRate" (* (`KismetMathLibrary.VSize` (- _returnvalue (`self.OldPosition`))) (`self.VelocityFactor`)))
  (set `self.OldPosition` (`PlayerCameraManager.GetCameraLocation` (`PlayerController.PlayerCameraManager` (`GameplayStatics.GetPlayerController` 0)))))

(fn `UserConstructionScript`)