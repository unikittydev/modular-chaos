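; Generates random space environments of sky colors, side lights, a star and planets, and transitions between them on demand.
; Each environment randomizes colors in HSV, draws the planet count from a curve and scatters bodies below a target location.
; A change fades out old bodies and fades in new ones, while a timeline blends skybox material and light colors through HSV.
; New star positions feed the celestial system, and planets receive the star's temperature.
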(event `Initialize`
  (bind _asmaterial_instance_dynamic (cast `MaterialInstanceDynamic` (`PrimitiveComponent.GetMaterial` (`StaticMeshActor.StaticMeshComponent` (`self.Skybox`)) 0)))
  (set `self.Sky Material` _asmaterial_instance_dynamic)
  (bind _environment (`self.Create Random Environment` (0.0 0.0 0.0)))
  (bind _output_get (set `self.Current Environment` _environment))
  (`self.Set Environment Values` _output_get)
  (bind (_primaryskycolor _secondaryskycolor _sidecolor1 _sidecolor2 _starlocation _planetlocations) (break `/Game/CelestialSystem/Blueprints/BPS_Environment` _output_get))
  (`self.Spawn Celestials` _starlocation _planetlocations))

(event `Change Environment`
  (params (Rate :type "Float (double-precision)") (`Target Location` :type "Vector Structure"))
  (`TimelineComponent.SetPlayRate` (`self.Environment Lerp`) Rate)
  (bind _environment (`self.Create Random Environment` `Target Location`))
  (for _array_element (`self.Current Bodies`)
    (`/Game/CelestialSystem/Blueprints/BP_Planet.Fade Out` _array_element (`self.Fade In Out Time`) true))
  (`KismetArrayLibrary.Array_Clear` (`self.Current Bodies`))
  (bind (_primaryskycolor _secondaryskycolor _sidecolor1 _sidecolor2 _starlocation _planetlocations) (break `/Game/CelestialSystem/Blueprints/BPS_Environment` _environment))
  (`self.Spawn Celestials` _starlocation _planetlocations)
  (bind (_direction _track) (`Timeline|Environment Lerp` :!via `PlayFromStart`)
    (:`Update`
      (`self.Set Environment Values` (`self.Lerp Environment` (`self.Current Environment`) _environment _track)))
    (:`Finished`
      (set `self.Current Environment` _environment))))

(event `Set Environment Values`
  (params (Environment :type "/Game/CelestialSystem/Blueprints/BPS_Environment Structure"))
  (bind (_primaryskycolor _secondaryskycolor _sidecolor1 _sidecolor2) (break `/Game/CelestialSystem/Blueprints/BPS_Environment` Environment))
  (bind _sky_material (`self.Sky Material`))
  (`MaterialInstanceDynamic.SetVectorParameterValue` _sky_material "PrimaryColor" _primaryskycolor)
  (`MaterialInstanceDynamic.SetVectorParameterValue` _sky_material "SecondaryColor" _secondaryskycolor)
  (`LightComponent.SetLightColor` (`Light.LightComponent` (`self.Side Light 1`)) _sidecolor1 true)
  (`LightComponent.SetLightColor` (`Light.LightComponent` (`self.Side Light 2`)) _sidecolor2 true))

(fn `Complementary Color`
  (params (`In Color` :type "LinearColor Structure"))
  (returns (`Comp Color` :type "LinearColor Structure"))
  (bind (_h _s _v _a) (`KismetMathLibrary.RGBToHSV` `In Color`))
  (return (`KismetMathLibrary.HSVToRGB` (mod (+ _h 180.0) 360.0) _s _v _a)))

(fn `Create Random Environment`
  (params (`Target Location` :type "Vector Structure"))
  (returns (Environment :type "/Game/CelestialSystem/Blueprints/BPS_Environment Structure"))
  (locals (`Planet Locations` :type "Array of Vector Structure") (`Planet Count` :type Integer))
  (bind _color (`self.Random Color`))
  (bind _comp_color (`self.Complementary Color` _color))
  (bind _output_get (set `local.Planet Count` (`self.Get Planet Count`)))
  (for _ (range 1 (+ _output_get 1))
    (`KismetArrayLibrary.Array_Add` (`local.Planet Locations`) (`self.Get Body Location` (`local.Target Location`) (`self.Min Planet Distance`) (`self.Max Planet Distance`))))
  (return (make `/Game/CelestialSystem/Blueprints/BPS_Environment` (* _color (`KismetMathLibrary.HSVToRGBLinear` (make `LinearColor` 0.0 0.0 (`KismetMathLibrary.RandomFloatInRange` (`self.Primary S Min`) (`self.Primary S Max`)) 1.0))) (* _comp_color (`KismetMathLibrary.HSVToRGBLinear` (make `LinearColor` 0.0 0.0 (`KismetMathLibrary.RandomFloatInRange` (`self.Secondary S Min`) (`self.Secondary S Max`)) 1.0))) _color _comp_color (`self.Get Body Location` (`local.Target Location`) (`self.Min Star Distance`) (`self.Max Star Distance`)) (`local.Planet Locations`))))

(fn `Get Body Location`
  (params (`Target Location` :type "Vector Structure") (Min :type "Float (double-precision)") (Max :type "Float (double-precision)"))
  (returns (`Body Location` :type "Vector Structure"))
  (bind (_returnvalue_x _returnvalue_y _returnvalue_z) (`KismetMathLibrary.BreakVector` (`KismetMathLibrary.RandomUnitVector`)))
  (return (+ `Target Location` (* (`KismetMathLibrary.RandomFloatInRange` Min Max) (`KismetMathLibrary.MakeVector` _returnvalue_x _returnvalue_y (- 0.0 (`KismetMathLibrary.Abs` _returnvalue_z)))))))

(fn `Get Planet Count`
  (returns (Count :type Integer))
  (return (`KismetMathLibrary.FTrunc` (`CurveFloat.GetFloatValue` (`self.Num Planets`) (`KismetMathLibrary.RandomFloat`)))))

(fn `Lerp Environment`
  (params (From :type "/Game/CelestialSystem/Blueprints/BPS_Environment Structure") (To :type "/Game/CelestialSystem/Blueprints/BPS_Environment Structure") (Time :type "Float (double-precision)"))
  (returns (Out :type "/Game/CelestialSystem/Blueprints/BPS_Environment Structure"))
  (bind (_primaryskycolor _secondaryskycolor _sidecolor1 _sidecolor2) (break `/Game/CelestialSystem/Blueprints/BPS_Environment` From))
  (bind (_primaryskycolor_2 _secondaryskycolor_2 _sidecolor1_2 _sidecolor2_2) (break `/Game/CelestialSystem/Blueprints/BPS_Environment` To))
  (return (make `/Game/CelestialSystem/Blueprints/BPS_Environment` (`KismetMathLibrary.LinearColorLerpUsingHSV` _primaryskycolor _primaryskycolor_2 (`local.Time`)) (`KismetMathLibrary.LinearColorLerpUsingHSV` _secondaryskycolor _secondaryskycolor_2 (`local.Time`)) (`KismetMathLibrary.LinearColorLerpUsingHSV` _sidecolor1 _sidecolor1_2 (`local.Time`)) (`KismetMathLibrary.LinearColorLerpUsingHSV` _sidecolor2 _sidecolor2_2 (`local.Time`)))))

(fn `Random Color`
  (returns (Color :type "LinearColor Structure"))
  (return (`KismetMathLibrary.HSVToRGB` (`KismetMathLibrary.RandomFloatInRange` 0.0 360.0) 1.0 1.0)))

(fn `Spawn Celestials`
  (params (`Star Location` :type "Vector Structure") (`Planet Locations` :type "Array of Vector Structure"))
  (`|ExecutionSequence`
    (:`then_0`
      (bind _returnvalue (`|SpawnActorFromClass` "/Game/CelestialSystem/Blueprints/BP_Star.BP_Star_C" (`KismetMathLibrary.MakeTransform` (0.0 0.0 0.0)) "Undefined" "MultiplyWithRoot" null true null))
      (bind _output_get (set `/Game/CelestialSystem/Blueprints/BPC_CelestialBody.World Coordinates` `Star Location` (`/Game/CelestialSystem/Blueprints/BP_Planet.Body` _returnvalue)))
      (set `/Game/CelestialSystem/Blueprints/BP_CelestialSystem.Sun Location` _output_get (`self.Celestial System`))
      (`/Game/CelestialSystem/Blueprints/BP_Planet.Fade In` _returnvalue (`self.Fade In Out Time`))
      (`KismetArrayLibrary.Array_Add` (`self.Current Bodies`) _returnvalue))
    (:`then_1`
      (for _array_element `Planet Locations`
        (bind _returnvalue_2 (`|SpawnActorFromClass` "/Game/CelestialSystem/Blueprints/BP_Planet.BP_Planet_C" (`KismetMathLibrary.MakeTransform` (0.0 0.0 0.0)) "Undefined" "MultiplyWithRoot" null true null))
        (set `/Game/CelestialSystem/Blueprints/BPC_CelestialBody.World Coordinates` _array_element (`/Game/CelestialSystem/Blueprints/BP_Planet.Body` _returnvalue_2))
        (`/Game/CelestialSystem/Blueprints/BP_Planet.Update Sun Info` _returnvalue_2 (`/Game/CelestialSystem/Blueprints/BP_Star.Temperature` _returnvalue))
        (`/Game/CelestialSystem/Blueprints/BP_Planet.Fade In` _returnvalue_2 (`self.Fade In Out Time`))
        (`KismetArrayLibrary.Array_Add` (`self.Current Bodies`) _returnvalue_2)))))

(fn `UserConstructionScript`)