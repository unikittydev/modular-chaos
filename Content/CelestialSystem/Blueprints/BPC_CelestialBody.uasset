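; BPC_CelestialBody registers itself as a celestial body with the level's BP_CelestialSystem.
; On BeginPlay it uses the assigned CelestialSystem or falls back to finding one in the world, then adds itself if AddToSystem is set.
; On EndPlay it removes itself from that system.
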(event `self.ReceiveBeginPlay`
  (`/Engine/EditorBlueprintResources/StandardMacros.IsValid` (`self.Celestial System`)
    (:`Is Valid`
      _)
    (:`Is Not Valid`
      (bind _returnvalue (`GameplayStatics.GetActorOfClass` "/Game/CelestialSystem/Blueprints/BP_CelestialSystem.BP_CelestialSystem_C"))
      (`/Engine/EditorBlueprintResources/StandardMacros.IsValid` _returnvalue
        (:`Is Valid`
          (set `self.Celestial System` _returnvalue)))))
  (if (`self.Add to system`)
    (`/Game/CelestialSystem/Blueprints/BP_CelestialSystem.Add Celestial Body` (`self.Celestial System`) self)))

(event `self.ReceiveEndPlay`
  (params (EndPlayReason :type "EEndPlayReason Enum" :default "Destroyed"))
  (`/Engine/EditorBlueprintResources/StandardMacros.IsValid` (`self.Celestial System`)
    (:`Is Valid`
      (`/Game/CelestialSystem/Blueprints/BP_CelestialSystem.Remove Celestial Body` (`self.Celestial System`) self))))