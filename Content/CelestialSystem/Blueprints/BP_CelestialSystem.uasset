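; BP_CelestialSystem simulates the player ship's travel through space and runs its jumps between coordinates.
; Each tick it places registered bodies around the camera from their scaled world-coordinate offset to the target body.
; SpaceBar triggers a random jump or one to a spawned ship-editor activator, with a hint overlay replacing the ship UI.
; A distance-scaled Timeline lerps the target's coordinates, shifting the skybox material while EnvironmentSystem changes the environment.
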(event `self.ReceiveBeginPlay`
  (set `self.Camera` (`GameplayStatics.GetPlayerCameraManager` 0))
  (`self.Get Sky MID`)
  (`/Game/CelestialSystem/Blueprints/BP_EnvironmentLerp.Initialize` (`self.Environment System`))
  (bind _asbp_ship (cast `/Game/Ships/BP_Ship` (`Controller.K2_GetPawn` (`GameplayStatics.GetPlayerController` 0))))
  (add `/Game/Ships/BP_Ship.On Set Enabled` _asbp_ship (delegate `On Set Ship Enabled`)))

(event `On Set Ship Enabled`
  (params (Enabled :type Boolean))
  (`/Engine/EditorBlueprintResources/StandardMacros.IsValid` (`self.Jump Overlay`)
    (:`Is Valid`
      (if Enabled
        (if (`self.Can Jump`)
          (set `Widget.Visibility` "Visible" (`/Game/Ships/Player/UI/WBP_JumpAvailable.JumpHint` (`self.Jump Overlay`))))
        (else
          (set `Widget.Visibility` "Hidden" (`/Game/Ships/Player/UI/WBP_JumpAvailable.JumpHint` (`self.Jump Overlay`))))))))

(event `self.ReceiveTick`
  (params (DeltaSeconds :type "Float (single-precision)"))
  (`/Engine/EditorBlueprintResources/StandardMacros.IsValid` (`self.Target Body`)
    (:`Is Valid`
      (for _array_element (`self.Bodies`)
        (`self.K2_SetActorLocation` (`ActorComponent.GetOwner` _array_element) (+ (* (- (`/Game/CelestialSystem/Blueprints/BPC_CelestialBody.World Coordinates` _array_element) (`/Game/CelestialSystem/Blueprints/BPC_CelestialBody.World Coordinates` (`self.Target Body`))) (`self.Celestials World Coordinates Factor`)) (`SceneComponent.K2_GetComponentLocation` (`PlayerCameraManager.TransformComponent` (`self.Camera`)))) false false)))))

(event `Key|SpaceBar`
  (params (Key :type "Key Structure"))
  (:`Pressed`
    (bind _asbp_ship (cast `/Game/Ships/BP_Ship` (`ActorComponent.GetOwner` (`self.Target Body`))))
    (if (and (`self.Can Jump`) (not (`self.Is Jumping`)) (`/Game/Ships/BP_Ship.Is Enabled` _asbp_ship))
      (if (`self.Next Jump Is Editor`)
        (bind _ship_editor_activator (`self.Jump to Ship Editor`))
        (set `self.Ship Editor` _ship_editor_activator)
        (else
          (bind _world_location (`self.Get Random Jump Location From Min Time` 5.0))
          (`self.Jump` _world_location))))))

(event `Jump`
  (params (`Target World Coordinates` :type "Vector Structure"))
  (bind (_returnvalue_x _returnvalue_y _returnvalue_z) (`KismetMathLibrary.BreakVector` (`KismetMathLibrary.NegateVector` (`/Game/CelestialSystem/Blueprints/BPC_CelestialBody.World Coordinates` (`self.Target Body`)))))
  (bind _returnvalue (- `Target World Coordinates` (`/Game/CelestialSystem/Blueprints/BPC_CelestialBody.World Coordinates` (`self.Target Body`))))
  (bind (_returnvalue_x_2 _returnvalue_y_2) (`KismetMathLibrary.BreakVector` (* _returnvalue (`self.Celestials World Coordinates Factor`))))
  (bind _returnvalue_2 (/ (`KismetMathLibrary.VSize` _returnvalue) (`self.Jump Speed`)))
  (bind _returnvalue_3 (/ 1.0 _returnvalue_2))
  (if (not (`KismetSystemLibrary.IsValid` (`self.Jump Overlay`)))
    (`self.Show Jump Overlay` false)
    (else
      (`Widget.SetVisibility` (`/Game/Ships/Player/UI/WBP_JumpAvailable.JumpHint` (`self.Jump Overlay`)) "Hidden")))
  (set `self.Is Jumping` true)
  (bind _asbp_ship_player (cast `/Game/Ships/Player/BP_Ship_Player` (`ActorComponent.GetOwner` (`self.Target Body`))))
  (`/Game/Ships/BP_Ship.Jump` _asbp_ship_player (+ (`SceneComponent.K2_GetComponentLocation` (`/Game/Ships/BP_Ship.BoxCollision` _asbp_ship_player)) (`KismetMathLibrary.MakeVector` _returnvalue_x_2 _returnvalue_y_2)) _returnvalue_2)
  (`KismetSystemLibrary.Delay` (+ (`/Game/Ships/BP_Ship.Stop Time` _asbp_ship_player) (`/Game/Ships/BP_Ship.Look At Time` _asbp_ship_player))) ; Compensate for ship stopping and rotation
  (set `self.Initial World Coordinates` (`/Game/CelestialSystem/Blueprints/BPC_CelestialBody.World Coordinates` (`self.Target Body`)))
  (`TimelineComponent.SetPlayRate` (`self.Timeline`) _returnvalue_3)
  (`/Game/CelestialSystem/Blueprints/BP_EnvironmentLerp.Change Environment` (`self.Environment System`) _returnvalue_3 `Target World Coordinates`)
  (bind (_direction _track) (`Timeline|Timeline` :!via `PlayFromStart`)
    (:`Update`
      (set `/Game/CelestialSystem/Blueprints/BPC_CelestialBody.World Coordinates` (`KismetMathLibrary.VLerp` (`self.Initial World Coordinates`) `Target World Coordinates` _track) (`self.Target Body`))
      (`MaterialInstanceDynamic.SetVectorParameterValue` (`self.Skybox Material`) "ShipCoordinateOffset" (make `LinearColor` _returnvalue_x _returnvalue_y _returnvalue_z 1.0)))
    (:`Finished`
      (set `self.Is Jumping` false)
      (`self.On Jump End`)
      (`Widget.SetVisibility` (`/Game/Ships/Player/UI/WBP_JumpAvailable.JumpHint` (`self.Jump Overlay`)) "Visible"))))

(event `Set Can Jump`
  (params (Value :type Boolean))
  (bind _output_get (set `self.Can Jump` Value))
  (if _output_get
    (`self.Show Jump Overlay` true)
    (else
      (`self.Hide Jump Overlay`))))

(event `Show Jump Overlay`
  (params (`Show Text` :type Boolean))
  (bind _asbp_ship_player (cast `/Game/Ships/Player/BP_Ship_Player` (`ActorComponent.GetOwner` (`self.Target Body`))))
  (bind _returnvalue (`|CreateWidget` "/Game/Ships/Player/UI/WBP_JumpAvailable.WBP_JumpAvailable_C"))
  (`UserWidget.AddToViewport` _returnvalue 0)
  (bind _output_get (set `self.Jump Overlay` _returnvalue))
  (`UserWidget.PlayAnimation` _output_get (select `bool` `Show Text` :`false` (`/Game/Ships/Player/UI/WBP_JumpAvailable.ShowFrameOnly` _output_get) :`true` (`/Game/Ships/Player/UI/WBP_JumpAvailable.ShowFrame` _output_get)) 0.0 1 "Forward" 1.0 false)
  (`Widget.SetVisibility` (`/Game/Ships/Player/BP_Ship_Player.UI` _asbp_ship_player) "Hidden")
  (`Widget.SetVisibility` (`/Game/Ships/Player/UI/WBP_JumpAvailable.JumpHint` (`self.Jump Overlay`)) (select `bool` `Show Text` :`false` "Collapsed" :`true` "Visible" :!type "ESlateVisibility Enum")))

(event `Hide Jump Overlay`
  (bind _jump_overlay (`self.Jump Overlay`))
  (bind _hideframe (`/Game/Ships/Player/UI/WBP_JumpAvailable.HideFrame` _jump_overlay))
  (bind _asbp_ship_player (cast `/Game/Ships/Player/BP_Ship_Player` (`ActorComponent.GetOwner` (`self.Target Body`))))
  (`UserWidget.PlayAnimation` _jump_overlay _hideframe 0.0 1 "Forward" 1.0 false)
  (`KismetSystemLibrary.Delay` (`WidgetAnimation.GetEndTime` _hideframe))
  (`Widget.RemoveFromParent` (`self.Jump Overlay`))
  (`Widget.SetVisibility` (`/Game/Ships/Player/BP_Ship_Player.UI` _asbp_ship_player) "Visible")
  (set `self.Jump Overlay` null))

(fn `Add Celestial Body`
  (params (Body :type "/Game/CelestialSystem/Blueprints/BPC_CelestialBody Object Reference"))
  (`KismetArrayLibrary.Array_Add` (`self.Bodies`) Body))

(fn `Get Random Jump Location From Min Time`
  (params (`Min Jump Time` :type "Float (double-precision)"))
  (returns (`World Location` :type "Vector Structure"))
  (locals (`Target Location` :type "Vector Structure" :default (0.0 0.0 0.0)))
  (set `local.Target Location` (* (`KismetMathLibrary.RandomUnitVector`) (`KismetMathLibrary.RandomFloatInRange` 0.0 (`self.Jump Radius`))))
  (while (< (`KismetMathLibrary.Vector_Distance` (`/Game/CelestialSystem/Blueprints/BPC_CelestialBody.World Coordinates` (`self.Target Body`)) (`local.Target Location`)) (* `Min Jump Time` (`self.Jump Speed`)))
    (set `local.Target Location` (* (`KismetMathLibrary.RandomUnitVector`) (`KismetMathLibrary.RandomFloatInRange` 0.0 (`self.Jump Radius`)))))
  (return (`local.Target Location`)))

(fn `Get Random Jump Location Of Length`
  (params (`Jump Length` :type "Float (double-precision)"))
  (returns (`World Location` :type "Vector Structure"))
  (locals (`Target Location` :type "Vector Structure"))
  (set `local.Target Location` (* (`KismetMathLibrary.RandomUnitVector`) (`KismetMathLibrary.RandomFloatInRange` 0.0 (`self.Jump Radius`))))
  (while (< (`KismetMathLibrary.Vector_Distance` (`/Game/CelestialSystem/Blueprints/BPC_CelestialBody.World Coordinates` (`self.Target Body`)) (`local.Target Location`)) (`local.Jump Length`))
    (set `local.Target Location` (* (`KismetMathLibrary.RandomUnitVector`) (`self.Jump Radius`))))
  (return (+ (* (`KismetMathLibrary.Normal` (- (`local.Target Location`) (`/Game/CelestialSystem/Blueprints/BPC_CelestialBody.World Coordinates` (`self.Target Body`)))) (`local.Jump Length`)) (`/Game/CelestialSystem/Blueprints/BPC_CelestialBody.World Coordinates` (`self.Target Body`)))))

(fn `Get Sky MID`
  (returns (Material :type "MaterialInstanceDynamic Object Reference"))
  (`/Engine/EditorBlueprintResources/StandardMacros.IsValid` (`self.Skybox Material`)
    (:`Is Valid`
      (return (`self.Skybox Material`)))
    (:`Is Not Valid`
      (bind _returnvalue (`KismetMaterialLibrary.CreateDynamicMaterialInstance` (`PrimitiveComponent.GetMaterial` (`StaticMeshActor.StaticMeshComponent` (`self.Skybox`)) 0)))
      (bind _output_get (set `self.Skybox Material` _returnvalue))
      (`PrimitiveComponent.SetMaterial` (`StaticMeshActor.StaticMeshComponent` (`self.Skybox`)) 0 _output_get)
      (return _output_get))))

(fn `Jump to Ship Editor`
  (returns (`Ship Editor Activator` :type "Actor Object Reference"))
  (set `self.Next Jump Is Editor` false)
  (bind _world_location (`self.Get Random Jump Location From Min Time` 5.0))
  (bind _asbp_ship (cast `/Game/Ships/BP_Ship` (`ActorComponent.GetOwner` (`self.Target Body`))))
  (bind (_returnvalue_x _returnvalue_y) (`KismetMathLibrary.BreakVector` (- _world_location (`/Game/CelestialSystem/Blueprints/BPC_CelestialBody.World Coordinates` (`self.Target Body`)))))
  (bind _returnvalue (`KismetMathLibrary.MakeVector` _returnvalue_x _returnvalue_y))
  (bind _returnvalue_2 (`|SpawnActorFromClass` "/Game/Ships/ShipEditor/Grid/BP_ShipEditorActivator.BP_ShipEditorActivator_C" (`KismetMathLibrary.MakeTransform` (`KismetMathLibrary.MakeVector` (.x (+ (+ (`SceneComponent.K2_GetComponentLocation` (`/Game/Ships/BP_Ship.BoxCollision` _asbp_ship)) (* _returnvalue (`self.Celestials World Coordinates Factor`))) (* (`KismetMathLibrary.Normal` _returnvalue) 700.0))) (.y (+ (+ (`SceneComponent.K2_GetComponentLocation` (`/Game/Ships/BP_Ship.BoxCollision` _asbp_ship)) (* _returnvalue (`self.Celestials World Coordinates Factor`))) (* (`KismetMathLibrary.Normal` _returnvalue) 700.0))) -100.0)) "AlwaysSpawn" "MultiplyWithRoot" null false null))
  (`self.Jump` _world_location)
  (return _returnvalue_2))

(fn `Remove Celestial Body`
  (params (Body :type "/Game/CelestialSystem/Blueprints/BPC_CelestialBody Object Reference"))
  (`KismetArrayLibrary.Array_RemoveItem` (`self.Bodies`) Body))

(fn `Remove Target Body`
  (`self.Set Target Body` null))

(fn `Set Target Body`
  (params (Body :type "/Game/CelestialSystem/Blueprints/BPC_CelestialBody Object Reference"))
  (set `self.Target Body` Body))

(fn `UserConstructionScript`)