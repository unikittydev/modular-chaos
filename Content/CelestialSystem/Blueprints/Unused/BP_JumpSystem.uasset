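; Prototype jump system that moves the celestial system's target body to new world coordinates over a set time, shifting the sky to match.
; BeginPlay puts a dynamic material on the Sky mesh and finds BP_CelestialSystem.
; Tick feeds the negated target coordinates into the material's ShipCoordinateOffset and triggers a random test jump on Space Bar.
; Jump scales a timeline's play rate by duration to lerp the coordinates.
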(event `self.ReceiveBeginPlay`
  (bind _returnvalue (`KismetMaterialLibrary.CreateDynamicMaterialInstance` (`PrimitiveComponent.GetMaterial` (`StaticMeshActor.StaticMeshComponent` (`self.Sky`)) 0)))
  (bind _output_get (set `self.Material` _returnvalue))
  (`PrimitiveComponent.SetMaterial` (`StaticMeshActor.StaticMeshComponent` (`self.Sky`)) 0 _output_get)
  (bind _returnvalue_2 (`GameplayStatics.GetActorOfClass` "/Game/CelestialSystem/Blueprints/BP_CelestialSystem.BP_CelestialSystem_C"))
  (set `self.Celestial System` _returnvalue_2))

(event `self.ReceiveTick`
  (params (DeltaSeconds :type "Float (single-precision)"))
  (bind (_returnvalue_x _returnvalue_y _returnvalue_z) (`KismetMathLibrary.BreakVector` (`KismetMathLibrary.NegateVector` (`/Game/CelestialSystem/Blueprints/BPC_CelestialBody.World Coordinates` (`/Game/CelestialSystem/Blueprints/BP_CelestialSystem.Target Body` (`self.Celestial System`))))))
  (`MaterialInstanceDynamic.SetVectorParameterValue` (`self.Material`) "ShipCoordinateOffset" (make `LinearColor` _returnvalue_x _returnvalue_y _returnvalue_z 1.0))
  (if (`PlayerController.WasInputKeyJustPressed` (`GameplayStatics.GetPlayerController` 0) "SpaceBar")
    (`self.Jump` (* (`KismetMathLibrary.RandomUnitVector`) (`self.test radius`)) (`self.test time`))))

(event `Jump`
  (params (`Target World Coordinates` :type "Vector Structure") (Time :type "Float (double-precision)"))
  (set `self.Initial World Coordinates` (`/Game/CelestialSystem/Blueprints/BPC_CelestialBody.World Coordinates` (`/Game/CelestialSystem/Blueprints/BP_CelestialSystem.Target Body` (`self.Celestial System`))))
  (`TimelineComponent.SetPlayRate` (`self.Jump Timeline`) (/ 1.0 Time))
  (bind (_direction _track) (`Timeline|Jump Timeline` :!via `PlayFromStart`)
    (:`Update`
      (set `/Game/CelestialSystem/Blueprints/BPC_CelestialBody.World Coordinates` (`KismetMathLibrary.VLerp` (`self.Initial World Coordinates`) `Target World Coordinates` _track) (`/Game/CelestialSystem/Blueprints/BP_CelestialSystem.Target Body` (`self.Celestial System`))))))

(fn `UserConstructionScript`)