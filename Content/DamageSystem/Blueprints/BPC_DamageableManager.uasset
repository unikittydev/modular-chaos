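; BPC_DamageableManager is a damage system component that distributes incoming damage and healing across a stack of layers.
; Damage passes through the layers in order with its damage type, each returning the leftover points for the next.
; Healing cascades the same way in reverse layer order.
; Both paths report the net applied amount through CallOnHPChanged, negative for damage and positive for healing.
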(event `On Take Damage`
  (params (Damage :type "/Game/DamageSystem/Structures/BPS_Damage Structure"))
  (`self.Take Damage` Damage))

(event `On Take Heal`
  (params (Heal :type Integer))
  (`self.Take Heal` Heal))

(fn `Take Damage`
  (params (Damage :type "/Game/DamageSystem/Structures/BPS_Damage Structure"))
  (locals (`Damage left` :type Integer))
  (bind (_damage_damagepoints _damage_damagetype) (break `/Game/DamageSystem/Structures/BPS_Damage` (`local.Damage`)))
  (bind _damage_damagepoints_2 (break `/Game/DamageSystem/Structures/BPS_Damage` (`local.Damage`)))
  (set `local.Damage left` Damage_DamagePoints_2_FDD4BB764CC37523C51825A835A7C714)
  (for _array_element (`self.Layers`)
    (bind _passed_damage (`/Game/DamageSystem/Blueprints/BPC_DamageableLayer.Take Damage` _array_element (make `/Game/DamageSystem/Structures/BPS_Damage` (`local.Damage left`) _damage_damagetype)))
    (set `local.Damage left` _passed_damage))
  (`self.On HP Changed` (- (`local.Damage left`) _damage_damagepoints_2)))

(fn `Take Heal`
  (params (Heal :type Integer))
  (locals (`Heal Left` :type Integer))
  (set `local.Heal Left` Heal)
  (bind (_arrayindex _arrayelement) (`/Engine/EditorBlueprintResources/StandardMacros.ReverseForEachLoop` (`self.Layers`))
    (:`LoopBody`
      (bind _heal_passed (`/Game/DamageSystem/Blueprints/BPC_DamageableLayer.Take Heal` _arrayelement (`local.Heal Left`)))
      (set `local.Heal Left` _heal_passed))
    (:`Completed`
      (`self.On HP Changed` (- (`local.Heal`) (`local.Heal Left`))))))