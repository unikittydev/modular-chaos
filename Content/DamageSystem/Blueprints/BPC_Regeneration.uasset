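; Regeneration component in the damage system that heals a target once a delay has passed without HP loss.
; Init binds to the Manager's HP changes, so any zero or negative delta resets the delay counter.
; Tick applies Strength per second as truncated heals, using an Error accumulator for fractional remainders.
; Unless RegenerateAfterDepleted is set, the target reaching zero HP disables ticking, stopping regeneration.
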(event `Init`
  (add `/Game/DamageSystem/Blueprints/BPC_DamageableManager.On HP Changed` (`self.Manager`) (delegate `On HP Changed`))
  (if (not (`self.Regenerate After Depleted`))
    (add `/Game/DamageSystem/Blueprints/BPC_DamageableLayer.On HP Zero` (`self.Regen Rarget`) (delegate `On Target HP Zero`))))

(event `On HP Changed`
  (params (`HP Delta` :type Integer))
  (if (<= `HP Delta` 0)
    (set `self.Counter` 0.0)))

(event `On Target HP Zero`
  (`self.SetComponentTickEnabled` false))

(event `self.ReceiveTick`
  (params (DeltaSeconds :type "Float (single-precision)"))
  (bind _returnvalue (+ (* DeltaSeconds (`self.Strength`)) (`self.Error`)))
  (`/Engine/EditorBlueprintResources/StandardMacros.IsValid` (`self.Regen Rarget`)
    (:`Is Valid`
      (bind _output_get (set `self.Counter` (+ DeltaSeconds (`self.Counter`))))
      (if (>= _output_get (`self.Delay`))
        (set `self.Error` (`KismetMathLibrary.Fraction` (+ (`self.Error`) (`KismetMathLibrary.Fraction` _returnvalue))))
        (`/Game/DamageSystem/Blueprints/BPC_DamageableLayer.Take Heal` (`self.Regen Rarget`) (`KismetMathLibrary.FTrunc` _returnvalue))))))