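; Component that acts as one damageable HP layer in the damage system, handling damage and healing.
; TakeDamage reduces incoming points by the resistance looked up for the damage type, truncates the result and caps it at current HP.
; TakeHeal restores HP up to the maximum and returns the unused healing.
; Both broadcast HP changes; at zero HP, damage also fires OnHPZero and returns raw points minus damage taken.
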(fn `Take Damage`
  (params (Damage :type "/Game/DamageSystem/Structures/BPS_Damage Structure"))
  (returns (`Passed Damage` :type Integer))
  (locals (`Damage Taken` :type Integer))
  (bind _damage_damagepoints (break `/Game/DamageSystem/Structures/BPS_Damage` (`local.Damage`)))
  (bind (_value _returnvalue) (`BlueprintMapLibrary.Map_Find` (`self.Resistance`) Damage_DamageType_7_AD178A1B4AE5F0CEA8E0F28B6B386776))
  (set `local.Damage Taken` (`KismetMathLibrary.Min` (`KismetMathLibrary.FTrunc` (* Damage_DamagePoints_2_FDD4BB764CC37523C51825A835A7C714 (- 1.0 (`KismetMathLibrary.SelectFloat` _value 0.0 _returnvalue)))) (`self.Current HP`)))
  (set `self.Current HP` (- (`self.Current HP`) (`local.Damage Taken`)))
  (bind _result (`/Engine/EditorBlueprintResources/StandardMacros.NegateInt` (`local.Damage Taken`))
    (:`  `
      (`self.On HP Changed` _result)
      (if (== (`self.Current HP`) 0)
        (`self.On HP Zero`)
        (return (- _damage_damagepoints (`local.Damage Taken`)))))))

(fn `Take Heal`
  (params (Heal :type Integer))
  (returns (`Heal Passed` :type Integer))
  (locals (`Heal Taken` :type Integer))
  (bind _output_get (set `local.Heal Taken` (`KismetMathLibrary.Min` Heal (- (`self.Max HP`) (`self.Current HP`)))))
  (set `self.Current HP` (+ _output_get (`self.Current HP`)))
  (`self.On HP Changed` (`local.Heal Taken`))
  (return (- (`local.Heal`) (`local.Heal Taken`))))