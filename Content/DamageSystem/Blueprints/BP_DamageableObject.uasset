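; BP_DamageableObject is a damageable world object that hurts ships it hits and takes damage itself.
; Construction registers its Hull as a layer in the damageable manager component, and the actor destroys itself when Hull HP reaches zero.
; On a hit with a BP_Ship, it sends typed random damage to both managers.
; The roll is RandomInteger(MaxDamage) plus (MaxDamage − MinDamage), so it is not bounded by Min and Max.
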(event `self.ReceiveBeginPlay`
  (add `/Game/DamageSystem/Blueprints/BPC_DamageableLayer.On HP Zero` (`self.Hull`) (delegate `On Destroyed`)))

(event `On Destroyed`
  (`self.K2_DestroyActor`))

(event `self.ReceiveHit`
  (params (MyComp :type "PrimitiveComponent Object Reference") (Other :type "Actor Object Reference") (OtherComp :type "PrimitiveComponent Object Reference") (bSelfMoved :type Boolean) (HitLocation :type "Vector Structure") (HitNormal :type "Vector Structure") (NormalImpulse :type "Vector Structure") (Hit :type "HitResult Structure (by ref)"))
  (bind _damage_type (`self.Damage Type`))
  (bind _returnvalue (+ (`KismetMathLibrary.RandomInteger` (`self.Max Damage`)) (- (`self.Max Damage`) (`self.Min Damage`))))
  (bind _asbp_ship (cast `/Game/Ships/BP_Ship` Other))
  (`/Game/DamageSystem/Blueprints/BPC_DamageableManager.On Take Damage` (`/Game/Ships/BP_Ship.BPC_DamageableManager` _asbp_ship) (make `/Game/DamageSystem/Structures/BPS_Damage` _returnvalue _damage_type))
  (`/Game/DamageSystem/Blueprints/BPC_DamageableManager.On Take Damage` (`self.BPC_DamageableManager`) (make `/Game/DamageSystem/Structures/BPS_Damage` _returnvalue _damage_type)))

(fn `UserConstructionScript`
  (`KismetArrayLibrary.Array_Add` (`/Game/DamageSystem/Blueprints/BPC_DamageableManager.Layers` (`self.BPC_DamageableManager`)) (`self.Hull`)))